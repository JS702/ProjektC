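; ExplosionSpot is a placeable actor that sets off a single explosion effect at its location at a random moment after play begins.
; BeginPlay calls Explode, which waits a random whole number of seconds under three minutes, then spawns an enlarged, auto-release pooled emitter and plays a sound.
; GetRandomExplosion picks between the standard and big particle systems with a coin flip.
; It applies no damage and does not repeat.
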(event Custom|Explode
  (bind _returnvalue (Transformation|GetActorLocation))
  (Utilities|FlowControl|Delay (Math|Conversions|ToFloat(Integer) (Math|Random|RandomInteger 180)))
  (bind _newparam (CallFunction|GetRandomExplosion))
  (Effects|SpawnEmitteratLocation _newparam _returnvalue "0, 0, 0" "2.000000,2.000000,2.000000" true "AutoRelease")
  (Audio|PlaySoundatLocation "/Game/StarterContent/Audio/Explosion01.Explosion01" _returnvalue "0, 0, 0" 1.0 1.0 0.0 0 0 0 0))

(event EventBeginPlay
  (CallFunction|Explode))

(fn ConstructionScript)

(fn GetRandomExplosion
  (if (Math|Random|RandomBool)
    (return "/Game/StarterContent/Particles/P_Explosion.P_Explosion")
    (else
      (return "/Game/Realistic_Starter_VFX_Pack_Vol2/Particles/Explosion/P_Explosion_Big_A.P_Explosion_Big_A"))))