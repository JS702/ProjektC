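; Enemy sniper for a VR shooter that moves to a random free SniperPosi, crouches into prone and fires on the player.
; A timed attack loop plays montages and reloads when empty, with a weighted random roll choosing an accurate, cover-checked damaging shot or an offset miss.
; Point damage triggers hit reactions or death, with headshots killing instantly.
; Death frees the position, notifies GameManager_BP, plays a directional montage, freezes and destroys the actor.
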(event Custom|Attack
  ;[1 1 1] Attack
  (if (Variables|Default|GetisAlive)
    (if (> (Variables|Default|Getammunition) 0)
      (Variables|Default|SetisAttacking true)
      (Audio|PlaySoundatLocation "/Game/Sounds/Voicelines/Open_Fire/ShootigCue.ShootigCue" (Transformation|GetActorLocation) "0, 0, 0" 1.0 1.0 0.0 0 0 0 0)
      (Animation|PlayAnimMontage "/Game/Animation/Animations/Sniper/Prone_Firing_Rifle_Montage.Prone_Firing_Rifle_Montage" 1.0 "None")
      (CallFunction|Shoot)
      (Variables|Default|Setammunition (- (Variables|Default|Getammunition) 1))
      (Variables|Default|SetisAttacking false)
      (Utilities|FlowControl|Delay 5.0)
      (CallFunction|Attack)
      (else
        (CallFunction|Reload)))))

(event Custom|Reload
  ;[1 1 1] Reload
  (if (Variables|Default|GetisAlive)
    (Audio|PlaySoundatLocation "/Game/Sounds/Weapons/Enemy_Reloads/Gewehr98_fullReload.Gewehr98_fullReload" (Transformation|GetActorLocation) "0, 0, 0" 1.0 1.0 0.0 0 0 0 0)
    (bind _returnvalue (Animation|PlayAnimMontage "/Game/Animation/Animations/Sniper/Prone_Reloading_Montage.Prone_Reloading_Montage" 1.0 "None"))
    (Utilities|FlowControl|Delay _returnvalue)
    (Variables|Default|Setammunition 9)
    (CallFunction|Attack)))

(event Custom|Die
  (params (A :type Vector) (Headshot :type Boolean))
  ;[1 1 1] Die
  (CallFunction|FreeSniperLocation)
  (Variables|Default|SetisAlive false)
  (bind _returnvalue (Actor|GetActorOfClass "/Game/Blueprints/GameManager_BP.GameManager_BP_C"))
  (Default|SniperKillled _returnvalue)
  (if Headshot
    (bind _montage (CallFunction|GetHeadshotMontage A))
    (bind _returnvalue_2 (Animation|PlayAnimMontage _montage 1.0 "None"))
    (Utilities|FlowControl|Delay (* _returnvalue_2 0.75))
    (else
      (bind _montage_2 (CallFunction|GetDeathMontage A))
      (bind _returnvalue_3 (Animation|PlayAnimMontage _montage_2 1.0 "None"))
      (Utilities|FlowControl|Delay (* _returnvalue_3 0.75))))
  (Variables|Default|SetCustomTimeDilation 0.0)
  (Utilities|FlowControl|Delay 2.0)
  (Actor|DestroyActor))

(event EventBeginPlay
  (bind _asvrpawn (Utilities|Casting|CastToVRPawn (Game|Player|GetPlayerPawn 0)))
  (Variables|Default|Setplayer _asvrpawn)
  (bind _output (CallFunction|FindSniperLocation :!label _label))
  (bind _output_get (Variables|Default|SetsniperPosi _output))
  (AI|AIMoveTo self "0, 0, 0" _output_get 5.0 true
    (:OnSuccess
      (Character|Crouch)
      (CallFunction|LookatPlayer)
      (CallFunction|Attack))
    (:OnFail
      (goto _label))))

(event EventTick
  (params (DeltaSeconds :type Float%20%28single-precision%29))
  (if (Variables|Default|GetisAttacking)
    (CallFunction|LookatPlayer)))

(event Game|Damage|EventPointDamage
  (params (Damage :type Float%20%28single-precision%29) (DamageType :type Damage%20Type%20Object%20Reference) (HitLocation :type Vector :default "0, 0, 0") (HitNormal :type Vector :default "0, 0, 0") (HitComponent :type Primitive%20Component%20Object%20Reference) (BoneName :type Name :default "None") (ShotFromDirection :type Vector :default "0, 0, 0") (InstigatedBy :type Controller%20Object%20Reference) (DamageCauser :type Actor%20Object%20Reference) (HitInfo :type Hit%20Result%20Structure%20%28by%20ref%29))
  (bind _returnvalue (== BoneName "Head"))
  ;[1 1 1] Take Damage
  (if (Variables|Default|GetisAlive)
    (Pawn|Components|CharacterMovement|DisableMovement (Variables|Character|GetCharacterMovement))
    (bind _output_get (Variables|Default|SetcurrentHealth (- (Variables|Default|GetcurrentHealth) Damage)))
    (Default|BloodEffect (Variables|Default|GetAC_Blood_Effect) HitLocation HitNormal)
    (if _returnvalue
      (CallFunction|Die ShotFromDirection _returnvalue :!label _label)
      (elif (<= _output_get 0.0)
        (goto _label)
        (else
          (Audio|PlaySoundatLocation "/Game/Sounds/Voicelines/Got_Hit/GotHitCue.GotHitCue" (Transformation|GetActorLocation) "0, 0, 0" 1.0 1.0 0.0 0 0 0 0)
          (bind _montage (CallFunction|GetHitReaction))
          (bind _returnvalue_2 (Animation|PlayAnimMontage _montage 1.0 "None"))
          (Utilities|FlowControl|Delay _returnvalue_2)
          (Pawn|Components|CharacterMovement|SetMovementMode (Variables|Character|GetCharacterMovement) "MOVE_Walking" 0))))))

(fn ConstructionScript)

(fn LookatPlayer
  (Transformation|SetActorRotation (Math|Rotator|MakeRotator 0.0 0.0 (.yaw (Math|Rotator|FindLookatRotation (Transformation|GetActorLocation) (Transformation|GetActorLocation (Variables|Default|Getplayer))))) true))

(fn FreeSniperLocation
  (bind _sniperposi (Variables|Default|GetsniperPosi))
  (Utilities|IsValid _sniperposi
    (:Is%20Valid
      (Variables|/Script/Engine.Actor|SetTags _sniperposi (Utilities|Array|MakeArray "Free")))))

(fn GetDeathMontage
  (params (HitDirection :type Vector))
  (bind _returnvalue (Transformation|GetActorTransform))
  (bind _returnvalue_2 (Math|Rotator|FindRelativeLookatRotation _returnvalue HitDirection))
  (bind _yaw (Math|Rotator|BreakRotator _returnvalue_2))
  (if (AI|Components|NavMovement|IsCrouching (Variables|Character|GetCharacterMovement))
    (return "/Game/Animation/Animations/Sniper/Prone_Death_Montage.Prone_Death_Montage")
    (elif (< (Math|Float|Absolute(Float) _yaw) 45.0)
      (return "/Game/Animation/Animations/Sniper/Death_Montage.Death_Montage")
      (elif (> (Math|Float|Absolute(Float) _yaw) 135.0)
        (return "/Game/Animation/Animations/Sniper/Death_From_The_Back_Montage.Death_From_The_Back_Montage")
        (elif (< _yaw 0.0)
          (return "/Game/Animation/Animations/Sniper/Death_From_Left_Montage.Death_From_Left_Montage")
          (else
            (return "/Game/Animation/Animations/Sniper/Death_From_Right_Montage.Death_From_Right_Montage")))))))

(fn GetHeadshotMontage
  (params (TargetLocation :type Vector%20%28by%20ref%29))
  (if (AI|Components|NavMovement|IsCrouching (Variables|Character|GetCharacterMovement))
    (return "/Game/Animation/Animations/Sniper/Prone_Death_Montage.Prone_Death_Montage")
    (elif (> (Math|Float|Absolute(Float) (.Yaw (Math|Rotator|BreakRotator (Math|Rotator|FindRelativeLookatRotation (Transformation|GetActorTransform) TargetLocation)))) 135.0)
      (return "/Game/Animation/Animations/Sniper/Death_From_Front_Headshot_Montage.Death_From_Front_Headshot_Montage")
      (else
        (return "/Game/Animation/Animations/Sniper/Death_From_Back_Headshot_Montage.Death_From_Back_Headshot_Montage")))))

(fn GetHitReaction
  (if (AI|Components|NavMovement|IsCrouching (Variables|Character|GetCharacterMovement))
    (return "/Game/Animation/Animations/Sniper/Rifle_Prone_Hit_Reaction_Montage.Rifle_Prone_Hit_Reaction_Montage")
    (else
      (return "/Game/Animation/Animations/Sniper/hit_reaction_Montage1.hit_reaction_Montage1"))))

(fn Shoot
  (bind _returnvalue (Math|Random|RandomFloatinRange 25.0 1e+02))
  (bind _player (Variables|Default|Getplayer))
  (bind _returnvalue_2 (Transformation|GetActorLocation _player))
  (bind (_x _y _z) (Math|Vector|BreakVector _returnvalue_2))
  (Components|Activation|Activate (Variables|Default|GetMuzzleFlash) false)
  (if (Math|Random|RandomBoolwithWeight 0.2)
    (bind (_outhit _returnvalue_3) (Collision|LineTraceByChannel (Transformation|GetWorldLocation (Variables|Default|GetArrow1)) (Math|Vector|MakeVector _x _y (+ _z 9e+01)) "TraceTypeQuery2" false 0 "None" true "(R=0.423529,G=0.400000,B=0.400000,A=1.000000)" "(R=0.546875,G=0.527345,B=0.516198,A=1.000000)"))
    (Audio|PlaySoundatLocation "/Game/Sounds/Weapons/Gewehr98/Gewehr98_shot.Gewehr98_shot" (Transformation|GetActorLocation) "0, 0, 0" 1.0 1.0 0.0 0 0 0 0)
    (if _returnvalue_3
      (Effects|SpawnEmitteratLocation "/Game/InfinityBladeEffects/Effects/FX_Monsters/FX_Monster_Troll/death/P_TrollDeathImpact.P_TrollDeathImpact" (.ImpactPoint (Collision|BreakHitResult _outhit)) (Math|Rotator|MakeRotfromX (.Normal (Collision|BreakHitResult _outhit))) "0.150000,0.150000,0.150000" true "AutoRelease")
      (else
        (Game|Damage|ApplyDamage (Variables|Default|Getplayer) 3e+01 0 0)))
    (else
      (bind _outhit_2 (Collision|LineTraceByChannel (Transformation|GetWorldLocation (Variables|Default|GetArrow1)) (Math|Vector|MakeVector (+ _x _returnvalue) (+ _y _returnvalue) (+ _z _returnvalue)) "TraceTypeQuery2" false 0 "None" true "(R=0.423529,G=0.400000,B=0.400000,A=1.000000)" "(R=0.423529,G=0.400000,B=0.400000,A=1.000000)"))
      (Audio|PlaySoundatLocation "/Game/Sounds/Weapons/Gewehr98/Gewehr98_shot.Gewehr98_shot" (Transformation|GetActorLocation) "0, 0, 0" 1.0 1.0 0.0 0 0 0 0)
      (Effects|SpawnEmitteratLocation "/Game/InfinityBladeEffects/Effects/FX_Monsters/FX_Monster_Troll/death/P_TrollDeathImpact.P_TrollDeathImpact" (.ImpactPoint (Collision|BreakHitResult _outhit_2)) (Math|Rotator|MakeRotfromX (.Normal (Collision|BreakHitResult _outhit_2))) "0.500000,0.500000,0.500000" true "AutoRelease"))))

(fn FindSniperLocation
  (bind _outactors (Actor|GetAllActorsOfClasswithTag "/Game/Blueprints/SniperPosi.SniperPosi_C" "Free"))
  (Variables|/Script/Engine.Actor|SetTags (Utilities|Array|Get(acopy) _outactors (Math|Random|RandomInteger (Utilities|Array|Length _outactors))) (Utilities|Array|MakeArray "Occupied"))
  (return (Utilities|Array|Get(acopy) _outactors (Math|Random|RandomInteger (Utilities|Array|Length _outactors)))))