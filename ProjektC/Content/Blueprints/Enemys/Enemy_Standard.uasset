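; Standard rifle enemy AI that moves between cover, attacks the player and reports its death to GameManager_BP.
; A delayed event loop picks random or nearer-to-player cover via Free/Occupied tags, then relocates, shoots or throws grenades; reloading is stubbed off.
; When the nearest-cover search finds none, it charges into a repeating melee chase.
; Point damage plays hit reactions; headshots kill instantly, with death montages chosen by stance and hit direction.
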(event Custom|MoveToCover
  ;[1 1 1] Move to Nearest Cover
  (if (Variables|Default|GetisAlive)
    (bind _cover (CallFunction|FindCover))
    (if (Variables|Default|GetrunToPlayer)
      (CallFunction|FreeCover)
      (CallFunction|MovetoPlayer)
      (else
        (AI|AIMoveTo self "0, 0, 0" _cover 5.0 true
          (:then
            (CallFunction|FreeCover)
            (bind _output_get (Variables|Default|Setcover _cover))
            (Variables|/Script/Engine.Actor|SetTags _output_get (Utilities|Array|MakeArray "Occupied")))
          (:OnSuccess
            (Character|Crouch)
            (CallFunction|LookatPlayer)
            (CallFunction|ChooseNextAction))
          (:OnFail
            (CallFunction|FreeCover)
            (CallFunction|MovetoCover)))))))

(event Custom|ChooseNextAction
  ;[1 1 1] Choose Next Action
  (if (Variables|Default|GetisAlive)
    (Utilities|FlowControl|Delay 2.0)
    (if false ; If Weapon has no ammo Left
      (CallFunction|Reload)
      (elif (Math|Random|RandomBool)
        (CallFunction|MovetoCover)
        (else
          (CallFunction|Attack))))))

(event Custom|Attack
  (bind _weapon (Variables|Default|GetWeapon))
  ;[1 1 1] Attack
  (if (Variables|Default|GetisAlive)
    (Variables|Default|SetisAttacking true)
    (if (!= (Math|Random|RandomInteger 9) 0)
      (bind _returnvalue (Animation|PlayAnimMontage "/Game/Animation/Animations/Standart/Shoot_Rifle_Montage.Shoot_Rifle_Montage" 1.0 "None"))
      (Utilities|FlowControl|Delay _returnvalue)
      (else
        (Rendering|SetVisibility _weapon false false)
        (bind _returnvalue_2 (Animation|PlayAnimMontage "/Game/Animation/Animations/Standart/toss_grenade_Montage.toss_grenade_Montage" 1.0 "None"))
        (Utilities|FlowControl|Delay (* _returnvalue_2 0.57))
        (Game|SpawnActorfromClass "/Game/Blueprints/Weapons/Grenade.Grenade_C" (Math|Transform|MakeTransform (Transformation|GetSocketLocation (Variables|Character|GetMesh) "RightHand") (Math|Conversions|RotationFromXVector (Transformation|GetActorForwardVector)) "1.000000,1.000000,1.000000") "AdjustIfPossibleButAlwaysSpawn" 0 0)
        (Utilities|FlowControl|Delay (* _returnvalue_2 0.43))
        (Rendering|SetVisibility _weapon true false)))
    (Variables|Default|SetisAttacking false)
    (CallFunction|ChooseNextAction)))

(event Custom|Reload
  ;[1 1 1] Reload
  (if (Variables|Default|GetisAlive)
    (if (AI|Components|NavMovement|IsCrouching (Variables|Character|GetCharacterMovement))
      (bind _returnvalue (Animation|PlayAnimMontage "/Game/Animation/Animations/Standart/ReloadCrouched_Montage.ReloadCrouched_Montage" 1.0 "None"))
      (Utilities|FlowControl|Delay _returnvalue)
      (else
        (bind _returnvalue_2 (Animation|PlayAnimMontage "/Game/Animation/Animations/Standart/reloading_Montage.reloading_Montage" 1.0 "None"))
        (Utilities|FlowControl|Delay _returnvalue_2)))
    (CallFunction|ChooseNextAction)))

(event Custom|MoveToPlayer
  ;[1 1 1] Move to Player
  (if (Variables|Default|GetisAlive)
    (AI|AIMoveTo self "0, 0, 0" (Game|Player|GetPlayerPawn 0) 125.0 true
      (:OnSuccess
        (CallFunction|LookatPlayer)
        (bind _returnvalue (Animation|PlayAnimMontage "/Game/Animation/Animations/Standart/Rifle_Punch_Montage.Rifle_Punch_Montage" 1.0 "None"))
        (Utilities|FlowControl|Delay _returnvalue)
        (CallFunction|MovetoPlayer :!label _label))
      (:OnFail
        (if (Variables|Default|GetisAlive)
          (goto _label))))))

(event Custom|Die
  (params (A :type Vector) (Headshot :type Boolean))
  ;[1 1 1] Die
  (Variables|Default|SetisAlive false)
  (bind _returnvalue (Actor|GetActorOfClass "/Game/Blueprints/GameManager_BP.GameManager_BP_C"))
  (Default|EnemyKilled _returnvalue)
  (if Headshot
    (bind _montage (CallFunction|GetHeadshotMontage A))
    (bind _returnvalue_2 (Animation|PlayAnimMontage _montage 1.0 "None"))
    (Utilities|FlowControl|Delay (* _returnvalue_2 0.75))
    (else
      (bind _montage_2 (CallFunction|GetDeathMontage A))
      (bind _returnvalue_3 (Animation|PlayAnimMontage _montage_2 1.0 "None"))
      (Utilities|FlowControl|Delay (* _returnvalue_3 0.75))))
  (Variables|Default|SetCustomTimeDilation 0.0)
  (Utilities|FlowControl|Delay 2.0)
  (Actor|DestroyActor))

(event EventBeginPlay
  (bind _outactors (Actor|GetAllActorsOfClasswithTag "/Game/Blueprints/Cover.Cover_C" "Far"))
  (Variables|Default|Setcover (Utilities|Array|Get(acopy) _outactors))
  (CallFunction|MovetoCover))

(event EventTick
  (params (DeltaSeconds :type Float%20%28single-precision%29))
  (if (Variables|Default|GetisAttacking)
    (CallFunction|LookatPlayer)))

(event Game|Damage|EventPointDamage
  (params (Damage :type Float%20%28single-precision%29) (DamageType :type Damage%20Type%20Object%20Reference) (HitLocation :type Vector :default "0, 0, 0") (HitNormal :type Vector :default "0, 0, 0") (HitComponent :type Primitive%20Component%20Object%20Reference) (BoneName :type Name :default "None") (ShotFromDirection :type Vector :default "0, 0, 0") (InstigatedBy :type Controller%20Object%20Reference) (DamageCauser :type Actor%20Object%20Reference) (HitInfo :type Hit%20Result%20Structure%20%28by%20ref%29))
  (bind _returnvalue (== BoneName "Head"))
  ;[1 1 1] Take Damage
  (if (Variables|Default|GetisAlive)
    (Pawn|Components|CharacterMovement|DisableMovement (Variables|Character|GetCharacterMovement))
    (bind _output_get (Variables|Default|SetcurrentHealth (- (Variables|Default|GetcurrentHealth) Damage)))
    (Audio|SpawnSoundAttached 0 (Variables|Collision|GetCapsuleComponent) "None" "0, 0, 0" "0, 0, 0" "KeepRelativeOffset" false 1.0 1.0 0.0 0 0)
    (Default|BloodEffect (Variables|Default|GetAC_Blood_Effect) HitLocation HitNormal)
    (if _returnvalue
      (CallFunction|Die ShotFromDirection _returnvalue :!label _label)
      (elif (<= _output_get 0.0)
        (goto _label)
        (else
          (bind _montage (CallFunction|GetHitReaction))
          (bind _returnvalue_2 (Animation|PlayAnimMontage _montage 1.0 "None"))
          (Utilities|FlowControl|Delay _returnvalue_2)
          (Pawn|Components|CharacterMovement|SetMovementMode (Variables|Character|GetCharacterMovement) "MOVE_Walking" 0))))))

(fn ConstructionScript)

(fn LookatPlayer
  (Transformation|SetActorRotation (Math|Rotator|MakeRotator 0.0 0.0 (.yaw (Math|Rotator|FindLookatRotation (Transformation|GetActorLocation) (Transformation|GetActorLocation (Game|Player|GetPlayerPawn 0)))))))

(fn FindNearestCover
  (bind _returnvalue (Game|Player|GetPlayerPawn 0))
  (Variables|Default|SetrunToPlayer true)
  (LocalVariables|SetnearestCover (Variables|Default|Getcover))
  (bind _outactors (Actor|GetAllActorsOfClasswithTag "/Game/Blueprints/Cover.Cover_C" "Free"))
  (for _array_element _outactors
    (if (Math|Boolean|ANDBoolean (> (Transformation|GetDistanceTo (LocalVariables|GetnearestCover)) (Transformation|GetDistanceTo _array_element)) (> (Transformation|GetDistanceTo _array_element) 5e+02) (< (Transformation|GetDistanceTo _array_element _returnvalue) (Transformation|GetDistanceTo (LocalVariables|GetnearestCover) _returnvalue)))
      (LocalVariables|SetnearestCover _array_element)
      (Variables|Default|SetrunToPlayer false)))
  (return (LocalVariables|GetnearestCover)))

(fn FreeCover
  (bind _cover (Variables|Default|Getcover))
  (Utilities|IsValid _cover
    (:Is%20Valid
      (Variables|/Script/Engine.Actor|SetTags _cover (Utilities|Array|MakeArray "Free")))))

(fn FindRandomCover
  (bind _outactors (Actor|GetAllActorsOfClasswithTag "/Game/Blueprints/Cover.Cover_C" "Free" :!label _label))
  (if (> (Transformation|GetDistanceTo (Utilities|Array|Get(acopy) _outactors (Math|Random|RandomInteger (Utilities|Array|Length _outactors)))) 5e+02)
    (return (Utilities|Array|Get(acopy) _outactors (Math|Random|RandomInteger (Utilities|Array|Length _outactors))))
    (else
      (goto _label))))

(fn FindCover
  (if (Math|Random|RandomBoolwithWeight 0.5)
    (bind _cover (CallFunction|FindNearestCover))
    (return _cover)
    (else
      (bind _output (CallFunction|FindRandomCover))
      (return _output))))

(fn GetDeathMontage
  (params (HitDirection :type Vector))
  (bind _returnvalue (Transformation|GetActorTransform))
  (bind _returnvalue_2 (Math|Rotator|FindRelativeLookatRotation _returnvalue HitDirection))
  (bind _yaw (Math|Rotator|BreakRotator _returnvalue_2))
  (if (AI|Components|NavMovement|IsCrouching (Variables|Character|GetCharacterMovement))
    (return "/Game/Animation/Animations/Standart/Crouch_Death_Montage.Crouch_Death_Montage")
    (elif (< (Math|Float|Absolute(Float) _yaw) 45.0)
      (return "/Game/Animation/Animations/Standart/Death_Montage.Death_Montage")
      (elif (> (Math|Float|Absolute(Float) _yaw) 135.0)
        (return "/Game/Animation/Animations/Standart/Death_From_The_Back_Montage.Death_From_The_Back_Montage")
        (elif (< _yaw 0.0)
          (return "/Game/Animation/Animations/Standart/Death_From_Left_Montage.Death_From_Left_Montage")
          (else
            (return "/Game/Animation/Animations/Standart/Death_From_Right_Montage.Death_From_Right_Montage")))))))

(fn GetHeadshotMontage
  (params (TargetLocation :type Vector%20%28by%20ref%29))
  (if (AI|Components|NavMovement|IsCrouching (Variables|Character|GetCharacterMovement))
    (return "/Game/Animation/Animations/Standart/Death_Crouching_Headshot_Front_Montage.Death_Crouching_Headshot_Front_Montage")
    (elif (> (Math|Float|Absolute(Float) (.Yaw (Math|Rotator|BreakRotator (Math|Rotator|FindRelativeLookatRotation (Transformation|GetActorTransform) TargetLocation)))) 135.0)
      (return "/Game/Animation/Animations/Standart/Death_From_Front_Headshot_Montage.Death_From_Front_Headshot_Montage")
      (else
        (return "/Game/Animation/Animations/Standart/Death_From_Front_Headshot_Montage.Death_From_Front_Headshot_Montage")))))

(fn GetHitReaction
  (if (AI|Components|NavMovement|IsCrouching (Variables|Character|GetCharacterMovement))
    (return "/Game/Animation/Animations/Standart/Hit_Reaction_Crouched_Montage.Hit_Reaction_Crouched_Montage")
    (else
      (return "/Game/Animation/Animations/Standart/Hit_Reaction_Montage.Hit_Reaction_Montage"))))