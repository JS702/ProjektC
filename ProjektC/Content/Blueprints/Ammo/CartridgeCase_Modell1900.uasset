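; Ejected-casing actor for the Modell1900 cartridge that cleans itself up after spawning.
; On BeginPlay it waits ten seconds, then a timed Delay loop steps a Scale variable down and applies it uniformly to the case component's world scale.
; Once Scale reaches the minimum threshold, the actor destroys itself, so the case shrinks away before removal.
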(event EventBeginPlay
  (Utilities|FlowControl|Delay 1e+01)
  (bind _output_get (Variables|Default|Setscale (- (Variables|Default|Getscale) 0.1) :!label _label))
  (if (> _output_get 0.1)
    (Transformation|SetWorldScale3D (Variables|Default|Getmodell1900_cartridgeCase) (Math|Vector|MakeVector (Variables|Default|Getscale) (Variables|Default|Getscale) (Variables|Default|Getscale)))
    (Utilities|FlowControl|Delay 0.1)
    (goto _label)
    (else
      (Actor|DestroyActor))))

(fn ConstructionScript)