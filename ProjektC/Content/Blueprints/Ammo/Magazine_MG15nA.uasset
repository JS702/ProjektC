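; Magazine_MG15nA is a grabbable magazine for the MG15nA weapon, built for motion-controller interaction.
; On Grab, it attaches its root to the motion controller, keeping world transform, only if the controller lies within the GripCollision sphere radius.
; On Release, it detaches the root while keeping its world transform.
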(event EventGrab
  (params (MotionController :type Motion%20Controller%20Component%20Object%20Reference))
  (bind _gripcollision (Variables|Default|GetGripCollision))
  (if (<= (Math|Vector|Distance(Vector) (Transformation|GetWorldLocation MotionController) (Transformation|GetWorldLocation _gripcollision)) (Variables|/Script/Engine.SphereComponent|GetSphereRadius _gripcollision))
    (Transformation|AttachComponentToComponent (Variables|Default|GetDefaultSceneRoot) MotionController "None" "KeepWorld" "KeepWorld" "KeepWorld" true)))

(event EventRelease
  (params (MotionController :type Motion%20Controller%20Component%20Object%20Reference))
  (Transformation|DetachFromComponent (Variables|Default|GetDefaultSceneRoot) "KeepWorld" "KeepWorld" "KeepWorld" true))

(fn ConstructionScript)