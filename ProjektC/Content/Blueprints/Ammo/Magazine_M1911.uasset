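; VR-grabbable M1911 pistol magazine that the player picks up and releases with either hand.
; BeginPlay caches the pawn's tagged hand meshes and their mannequin XR anim instances.
; Grab checks the controller is inside the grip sphere, picks the hand by controller name, sets its pose and snaps the root to its magazine socket, resetting scale only for the left.
; Release detaches it in place.
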(event EventRelease
  (params (MotionController :type Motion%20Controller%20Component%20Object%20Reference))
  (Transformation|DetachFromComponent (Variables|Default|GetDefaultSceneRoot) "KeepWorld" "KeepWorld" "KeepWorld" true))

(event EventGrab
  (params (MotionController :type Motion%20Controller%20Component%20Object%20Reference))
  (bind _gripcollision (Variables|Default|GetGripCollision))
  (if (<= (Math|Vector|Distance(Vector) (Transformation|GetWorldLocation MotionController) (Transformation|GetWorldLocation _gripcollision)) (Variables|/Script/Engine.SphereComponent|GetSphereRadius _gripcollision))
    (if (Utilities|Enum|Equal(Enum) (Utilities|GetObjectName MotionController) "MotionControllerRight")
      (Variables|/Game/Characters/MannequinsXR/Meshes/SK_MannequinsXR_AnimBlueprint.SK_MannequinsXR_AnimBlueprint_C|SetBlendSpaceEnum (Variables|Default|GetRightHandAnim) "NewEnumerator5")
      (Transformation|AttachComponentToComponent (Variables|Default|GetDefaultSceneRoot) (Variables|Default|GetRightHand) "M1911MagazineSocket" "SnapToTarget" "SnapToTarget" "SnapToTarget" true)
      (else
        (Variables|/Game/Characters/MannequinsXR/Meshes/SK_MannequinsXR_AnimBlueprint.SK_MannequinsXR_AnimBlueprint_C|SetBlendSpaceEnum (Variables|Default|GetLeftHandAnim) "NewEnumerator5")
        (Transformation|AttachComponentToComponent (Variables|Default|GetDefaultSceneRoot) (Variables|Default|GetLeftHand) "M1911MagazineSocket" "SnapToTarget" "SnapToTarget" "SnapToTarget" true)
        (Transformation|SetWorldScale3D (Variables|Default|GetDefaultSceneRoot) "1.000000,1.000000,1.000000")))))

(event EventBeginPlay
  (bind _returnvalue (Game|Player|GetPlayerPawn 0))
  (bind _output_get (Variables|Default|SetLeftHand (Utilities|Array|Get(acopy) (Actor|GetComponentsbyTag _returnvalue "/Script/Engine.SkeletalMeshComponent" "HandLeft"))))
  (bind _output_get_2 (Variables|Default|SetRightHand (Utilities|Array|Get(acopy) (Actor|GetComponentsbyTag _returnvalue "/Script/Engine.SkeletalMeshComponent" "HandRight"))))
  (bind _assk_mannequins_xr_anim_blueprint (Utilities|Casting|CastToSK_MannequinsXR_AnimBlueprint (Components|SkeletalMesh|GetAnimInstance _output_get)))
  (Variables|Default|SetLeftHandAnim _assk_mannequins_xr_anim_blueprint)
  (bind _assk_mannequins_xr_anim_blueprint_2 (Utilities|Casting|CastToSK_MannequinsXR_AnimBlueprint (Components|SkeletalMesh|GetAnimInstance _output_get_2)))
  (Variables|Default|SetRightHandAnim _assk_mannequins_xr_anim_blueprint_2))

(fn ConstructionScript)