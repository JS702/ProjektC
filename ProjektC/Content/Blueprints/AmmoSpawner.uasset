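; VR ammo spawner that produces a Bullet in the player's hand when grabbed.
; BeginPlay caches the pawn's tagged hand meshes and their XR mannequin anim blueprints.
; Grab checks that the motion controller is within the sphere radius, spawns a bullet at the cube, sets that hand's pose and snaps the bullet to its three-finger socket, choosing the hand by controller name.
; Release detaches the last spawned bullet, keeping its world transform.
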(event EventBeginPlay
  (bind _returnvalue (Game|Player|GetPlayerPawn 0))
  (bind _output_get (Variables|Default|SetLeftHand (Utilities|Array|Get(acopy) (Actor|GetComponentsbyTag _returnvalue "/Script/Engine.SkeletalMeshComponent" "HandLeft"))))
  (bind _output_get_2 (Variables|Default|SetRightHand (Utilities|Array|Get(acopy) (Actor|GetComponentsbyTag _returnvalue "/Script/Engine.SkeletalMeshComponent" "HandRight"))))
  (bind _assk_mannequins_xr_anim_blueprint (Utilities|Casting|CastToSK_MannequinsXR_AnimBlueprint (Components|SkeletalMesh|GetAnimInstance _output_get)))
  (Variables|Default|SetLeftHandAnim _assk_mannequins_xr_anim_blueprint)
  (bind _assk_mannequins_xr_anim_blueprint_2 (Utilities|Casting|CastToSK_MannequinsXR_AnimBlueprint (Components|SkeletalMesh|GetAnimInstance _output_get_2)))
  (Variables|Default|SetRightHandAnim _assk_mannequins_xr_anim_blueprint_2))

(event EventGrab
  (params (MotionController :type Motion%20Controller%20Component%20Object%20Reference))
  (bind _cube (Variables|Default|Getcube))
  (bind _sphere (Variables|Default|GetSphere))
  (bind _returnvalue (Transformation|GetWorldTransform _cube))
  (if (<= (Math|Vector|Distance(Vector) (Transformation|GetWorldLocation MotionController) (Transformation|GetWorldLocation _sphere)) (Variables|/Script/Engine.SphereComponent|GetSphereRadius _sphere))
    (bind _returnvalue_2 (Game|SpawnActorfromClass "/Game/Blueprints/Ammo/Bullet.Bullet_C" (Math|Transform|MakeTransform (.location _returnvalue) (.rotation _returnvalue) "1.000000,1.000000,1.000000") "Undefined" 0 0))
    (bind _output_get (Variables|Default|SetspawnedBullet _returnvalue_2))
    (Variables|/Game/Blueprints/Ammo/Bullet.Bullet_C|SetjustSpawned _output_get false)
    (if (Utilities|Enum|Equal(Enum) (Utilities|GetObjectName MotionController) "MotionControllerRight")
      (Variables|/Game/Characters/MannequinsXR/Meshes/SK_MannequinsXR_AnimBlueprint.SK_MannequinsXR_AnimBlueprint_C|SetBlendSpaceEnum (Variables|Default|GetRightHandAnim) "NewEnumerator4")
      (Transformation|AttachComponentToComponent _output_get (Variables|Default|GetRightHand) "threeFingerSocket" "SnapToTarget" "SnapToTarget" "SnapToTarget" true)
      (else
        (Variables|/Game/Characters/MannequinsXR/Meshes/SK_MannequinsXR_AnimBlueprint.SK_MannequinsXR_AnimBlueprint_C|SetBlendSpaceEnum (Variables|Default|GetLeftHandAnim) "NewEnumerator4")
        (Transformation|AttachComponentToComponent _output_get (Variables|Default|GetLeftHand) "threeFingerSocket" "SnapToTarget" "SnapToTarget" "SnapToTarget" true)))))

(event EventRelease
  (params (MotionController :type Motion%20Controller%20Component%20Object%20Reference))
  (bind _spawnedbullet (Variables|Default|GetspawnedBullet)
    (:then
      (Transformation|DetachFromComponent (Variables|/Script/Engine.Actor|GetRootComponent _spawnedbullet) "KeepWorld" "KeepWorld" "KeepWorld" true))
    (:else)))

(fn ConstructionScript)