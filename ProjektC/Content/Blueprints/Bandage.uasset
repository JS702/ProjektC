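; VR bandage pickup that restores the player to full health when held with both hands until a countdown completes, then destroys itself.
; Overlap flags gate grabs, which notify the Body actor on first pickup, attach to the first controller and swap in the bandage's hand meshes.
; A second grip starts timers and sound while Tick aims the bandage between controllers.
; Releasing either hand cancels healing, handing over attachment or restoring physics.
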(event OnComponentBeginOverlap(gripCollision)
  (params (OverlappedComponent :type Primitive%20Component%20Object%20Reference) (OtherActor :type Actor%20Object%20Reference) (OtherComp :type Primitive%20Component%20Object%20Reference) (OtherBodyIndex :type Integer) (bFromSweep :type Boolean) (SweepResult :type Hit%20Result%20Structure%20%28by%20ref%29))
  (bind _returnvalue (Utilities|GetObjectName OtherComp))
  (if (Utilities|Enum|Equal(Enum) _returnvalue "HandCollisionLeft")
    (Variables|Default|SetgrabbableLeft true)
    (elif (Utilities|Enum|Equal(Enum) _returnvalue "HandCollisionRight")
      (Variables|Default|SetgrabbableRight true))))

(event OnComponentEndOverlap(gripCollision)
  (params (OverlappedComponent :type Primitive%20Component%20Object%20Reference) (OtherActor :type Actor%20Object%20Reference) (OtherComp :type Primitive%20Component%20Object%20Reference) (OtherBodyIndex :type Integer))
  (bind _returnvalue (Utilities|GetObjectName OtherComp))
  (if (Utilities|Enum|Equal(Enum) _returnvalue "HandCollisionLeft")
    (Variables|Default|SetgrabbableLeft false)
    (elif (Utilities|Enum|Equal(Enum) _returnvalue "HandCollisionRight")
      (Variables|Default|SetgrabbableRight false))))

(event EventTick
  (params (DeltaSeconds :type Float%20%28single-precision%29))
  (bind _maingripcontroller (Variables|Default|GetMainGripController))
  (bind _secondarygripcontroller (Variables|Default|GetSecondaryGripController))
  (bind _returnvalue (Transformation|GetWorldLocation _maingripcontroller))
  (bind _returnvalue_2 (Transformation|GetWorldLocation _secondarygripcontroller))
  (bind _returnvalue_3 (Math|Rotator|FindLookatRotation _returnvalue _returnvalue_2))
  (if (and (Utilities|IsValid (Variables|Default|GetMainGripController)) (Utilities|IsValid (Variables|Default|GetSecondaryGripController))) ; Checks if the player grabbed with both hands
    ;[1 1 1] Two handed grab rotating
    (Transformation|SetWorldRotation (Variables|Default|Getbandage) (Math|Rotator|MakeRotator (.roll (Transformation|GetWorldRotation _maingripcontroller)) (.pitch _returnvalue_3) (.yaw _returnvalue_3)) false false)))

(event EventGrab
  (params (MotionController :type Motion%20Controller%20Component%20Object%20Reference))
  (if (or (and (Utilities|Enum|Equal(Enum) (Utilities|GetObjectName MotionController) "MotionControllerRight") (Variables|Default|GetgrabbableRight)) (and (Utilities|Enum|Equal(Enum) (Utilities|GetObjectName MotionController) "MotionControllerLeft") (Variables|Default|GetgrabbableLeft)))
    (if (Variables|Default|GetspawnedOnBody)
      (Default|BandageGrabbed (Variables|Default|Getbody))
      (Variables|Default|SetspawnedOnBody false))
    (if (Variables|Default|GetphysicsEnabled)
      (Physics|SetSimulatePhysics (Variables|Default|Getbandage) false)
      (Variables|Default|SetphysicsEnabled false))
    (if (not (Variables|Default|GetisAttachedToOneHand))
      (bind _output_get (Variables|Default|SetmainGripController MotionController))
      (bind _returnvalue (Transformation|AttachComponentToComponent (Variables|Default|Getbandage) _output_get "None" "SnapToTarget" "SnapToTarget" "KeepWorld" true))
      (Variables|Default|SetisAttachedToOneHand _returnvalue)
      (else
        (Variables|Default|SetsecondaryGripController MotionController)))
    (if (Utilities|Enum|Equal(Enum) (Utilities|GetObjectName MotionController) "MotionControllerRight")
      (Development|SetHiddeninGame (Variables|Default|GetplayerHandRight) true false)
      (Development|SetHiddeninGame (Variables|Default|GethandRight) false false)
      (else
        (Development|SetHiddeninGame (Variables|Default|GetplayerHandLeft) true false)
        (Development|SetHiddeninGame (Variables|Default|GethandLeft) false false)))
    ;[1 1 1] Check if both hands are holding the bandage
    (if (and (Utilities|IsValid (Variables|Default|GetmainGripController)) (Utilities|IsValid (Variables|Default|GetsecondaryGripController)))
      ;[1 1 1] Start healing
      (Development|SetHiddeninGame (Variables|Default|GettimerText) false false)
      (bind _returnvalue_2 (Utilities|Time|SetTimerbyFunctionName 0 "heal" 9.9))
      (Variables|Default|SetheallTimerHandle _returnvalue_2)
      (bind _returnvalue_3 (Utilities|Time|SetTimerbyFunctionName 0 "timerUIHandler" 0.1 true))
      (Variables|Default|SetUITimerHandle _returnvalue_3)
      (bind _returnvalue_4 (Audio|SpawnSoundAttached "/Game/Sounds/bandaging.bandaging" (Variables|Default|Getbandage) "None" "0, 0, 0" "0, 0, 0" "KeepRelativeOffset" false 1.0 1.0 0.0 0 0))
      (bind _output_get_2 (Variables|Default|Setsound _returnvalue_4))
      (Audio|Components|Audio|Play _output_get_2 0.0))))

(event EventRelease
  (params (MotionController :type Motion%20Controller%20Component%20Object%20Reference))
  (if (== MotionController (Variables|Default|GetmainGripController))
    (Transformation|DetachFromComponent (Variables|Default|Getbandage) "KeepWorld" "KeepWorld" "KeepWorld" false)
    (if (Utilities|IsValid (Variables|Default|GetsecondaryGripController))
      (bind _output_get (Variables|Default|SetmainGripController (Variables|Default|GetsecondaryGripController)))
      (Variables|Default|SetsecondaryGripController 0)
      (CallFunction|StopHealing)
      (Transformation|AttachComponentToComponent (Variables|Default|Getbandage) _output_get "None" "SnapToTarget" "SnapToTarget" "KeepWorld" true)
      (else
        (Variables|Default|SetisAttachedToOneHand false)
        (Physics|SetSimulatePhysics (Variables|Default|Getbandage) true)
        (Variables|Default|SetphysicsEnabled true)))
    (if (Utilities|Enum|Equal(Enum) (Utilities|GetObjectName MotionController) "MotionControllerRight") :!label _label
      (Development|SetHiddeninGame (Variables|Default|GetplayerHandRight) false false)
      (Development|SetHiddeninGame (Variables|Default|GethandRight) true false)
      (else
        (Development|SetHiddeninGame (Variables|Default|GetplayerHandLeft) false false)
        (Development|SetHiddeninGame (Variables|Default|GethandLeft) true false)))
    (elif (== MotionController (Variables|Default|GetsecondaryGripController))
      (Variables|Default|SetsecondaryGripController 0)
      (CallFunction|StopHealing)
      (goto _label))))

(event EventBeginPlay
  (bind _returnvalue (Game|Player|GetPlayerPawn 0))
  (bind _returnvalue_2 (Actor|GetActorOfClass "/Game/Blueprints/Body.Body_C"))
  (Variables|Default|Setbody _returnvalue_2)
  (Variables|Default|SetVRPawn _returnvalue)
  (Variables|Default|SetplayerHandLeft (Utilities|Array|Get(acopy) (Actor|GetComponentsbyTag _returnvalue "/Script/Engine.SkeletalMeshComponent" "HandLeft")))
  (Variables|Default|SetplayerHandRight (Utilities|Array|Get(acopy) (Actor|GetComponentsbyTag _returnvalue "/Script/Engine.SkeletalMeshComponent" "HandRight"))))

(fn ConstructionScript)

(fn Heal
  (bind _asvrpawn (Utilities|Casting|CastToVRPawn (Variables|Default|GetVRPawn)))
  (Variables|/Game/VRTemplate/Blueprints/VRPawn.VRPawn_C|SetcurrentHealth _asvrpawn (Variables|/Game/VRTemplate/Blueprints/VRPawn.VRPawn_C|GetmaxHealth _asvrpawn))
  (Development|SetHiddeninGame (Variables|Default|GetplayerHandLeft) false false)
  (Development|SetHiddeninGame (Variables|Default|GetplayerHandRight) false false)
  (Actor|DestroyActor))

(fn TimerUIHandler
  (bind _output_get (Variables|Default|SetsecondsRemaining (- (Variables|Default|GetsecondsRemaining) 0.1)))
  (Rendering|Components|TextRender|SetText (Variables|Default|GettimerText) (Utilities|Text|ToText(Float) _output_get "HalfToEven")))

(fn StopHealing
  (bind _sound (Variables|Default|Getsound))
  (bind _timertext (Variables|Default|GettimerText))
  ;[1 1 1] Stop healing
  (if (Utilities|Time|IsValidTimerHandle (Variables|Default|GetheallTimerHandle))
    (Utilities|Time|ClearandInvalidateTimerbyHandle (Variables|Default|GetheallTimerHandle))
    (Utilities|Time|ClearandInvalidateTimerbyHandle (Variables|Default|GetUITimerHandle))
    (Development|SetHiddeninGame _timertext true false)
    (bind _output_get (Variables|Default|SetsecondsRemaining 9.9))
    (Rendering|Components|TextRender|SetText _timertext (Utilities|Text|ToText(Float) _output_get "HalfToEven")))
  (if (Utilities|IsValid _sound)
    (Audio|Components|Audio|Stop _sound))
  (return))