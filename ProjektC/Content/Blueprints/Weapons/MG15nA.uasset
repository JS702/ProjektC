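; VR MG15nA machine gun that the player grips, reloads and fires with motion controllers.
; Grab and Release pick main grip, secondary grip, top cover, magazine or bolt by grip-sphere distance, re-parenting GripPoint as hands change.
; Tick drives two-handed look-at aiming, top cover hinging and bolt travel that chambers a round.
; Magazines swap as spawned actors through the open cover; automatic fire loops on a delay, ejecting cases and links.
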(event Input|EnhancedActionEvents|EnhancedInputActionIA_Shoot_Left
  (params (ActionValue :type Boolean) (ElapsedSeconds :type Float%20%28double-precision%29) (TriggeredSeconds :type Float%20%28double-precision%29) (InputAction :type Input%20Action%20Object%20Reference :default "/Game/VRTemplate/Input/Actions/IA_Shoot_Left.IA_Shoot_Left"))
  (bind _isbulletinchamber (Variables|Default|GetisBulletInChamber))
  (bind _ejectionpoint (Variables|Default|GetEjectionPoint))
  (bind _returnvalue (Transformation|GetWorldLocation _ejectionpoint))
  (bind _returnvalue_2 (Transformation|GetWorldRotation _ejectionpoint))
  (bind _returnvalue_3 (Math|Transform|MakeTransform _returnvalue _returnvalue_2))
  ;[1 1 1] Shooting
  (:Started
    (Development|PrintString "Bullet is in chamber" _isbulletinchamber _isbulletinchamber "(R=0.129942,G=1.000000,B=0.000000,A=1.000000)")
    ;;[1 0 0] Prevents the gun from shooting if:
    ;; - no magazine is attached
    ;; - the top cover isn't closed
    ;; - there are no more bullets left in the magazine
    (if (Math|Boolean|ANDBoolean (Variables|Default|GetisMagazineAttached) (Variables|Default|GetisTopCoverClosed) (Variables|Default|GetisBulletInChamber) (> (Variables|Default|GetBulletsInMagazine) 0))
      (Variables|Default|SetisShooting true)
      ;;[1 1 1] Projectile spawning
      (Game|SpawnActorfromClass "/Game/Blueprints/Ammo/MyProjectile.MyProjectile_C" (Transformation|GetWorldTransform (Variables|Default|GetMuzzleEnd)) "Undefined" self (Game|Player|GetPlayerPawn 0) :!label _label)
      (Components|Activation|Activate (Variables|Default|GetMuzzleFlash) true)
      (Development|PrintString "ShootLog: Shot fired")
      (bind _output_get (Variables|Default|SetBulletsInMagazine (- (Variables|Default|GetBulletsInMagazine) 1)))
      (if (< _output_get 1)
        (Development|SetHiddeninGame (Variables|Default|Getmg15na_ammo_belt) true false))
      (if (and (> _output_get 0) (Variables|Default|GetisShooting))
        (bind _returnvalue_4 (Game|SpawnActorfromClass "/Game/Blueprints/Ammo/CartridgeCase.CartridgeCase_C" _returnvalue_3 "Undefined" 0 0))
        (bind _returnvalue_5 (Game|SpawnActorfromClass "/Game/Blueprints/Ammo/ChainLink.ChainLink_C" _returnvalue_3 "Undefined" 0 0))
        (Physics|SetSimulatePhysics (Variables|/Game/Blueprints/Ammo/CartridgeCase.CartridgeCase_C|GetCartridgeCase _returnvalue_4) true)
        (Physics|AddImpulse (Variables|/Game/Blueprints/Ammo/CartridgeCase.CartridgeCase_C|GetCartridgeCase _returnvalue_4) (* (Math|Vector|Normalize (- (Transformation|GetWorldLocation (Variables|Default|GetEjectionPoint)) (Transformation|GetWorldLocation (Variables|Default|GetEjectionDirection))) 0.1) "-2.000000,-2.000000,-2.000000") "None" false)
        (Utilities|FlowControl|Delay 0.12)
        (goto _label))))
  (:Completed
    (Variables|Default|SetisShooting false)))

(event Input|EnhancedActionEvents|EnhancedInputActionIA_Shoot_Right
  (params (ActionValue :type Boolean) (ElapsedSeconds :type Float%20%28double-precision%29) (TriggeredSeconds :type Float%20%28double-precision%29) (InputAction :type Input%20Action%20Object%20Reference :default "/Game/VRTemplate/Input/Actions/IA_Shoot_Right.IA_Shoot_Right"))
  (bind _isbulletinchamber (Variables|Default|GetisBulletInChamber))
  (bind _ejectionpoint (Variables|Default|GetEjectionPoint))
  (bind _returnvalue (Transformation|GetWorldLocation _ejectionpoint))
  (bind _returnvalue_2 (Transformation|GetWorldRotation _ejectionpoint))
  (bind _returnvalue_3 (Math|Transform|MakeTransform _returnvalue _returnvalue_2))
  ;[1 1 1] Shooting
  (:Started
    (Development|PrintString "Bullet is in chamber" _isbulletinchamber _isbulletinchamber "(R=0.129942,G=1.000000,B=0.000000,A=1.000000)")
    ;;[1 0 0] Prevents the gun from shooting if:
    ;; - no magazine is attached
    ;; - the top cover isn't closed
    ;; - there are no more bullets left in the magazine
    (if (Math|Boolean|ANDBoolean (Variables|Default|GetisMagazineAttached) (Variables|Default|GetisTopCoverClosed) (Variables|Default|GetisBulletInChamber) (> (Variables|Default|GetBulletsInMagazine) 0))
      (Variables|Default|SetisShooting true)
      ;;[1 1 1] Projectile spawning
      (Game|SpawnActorfromClass "/Game/Blueprints/Ammo/MyProjectile.MyProjectile_C" (Transformation|GetWorldTransform (Variables|Default|GetMuzzleEnd)) "Undefined" self (Game|Player|GetPlayerPawn 0) :!label _label)
      (Components|Activation|Activate (Variables|Default|GetMuzzleFlash) true)
      (Development|PrintString "ShootLog: Shot fired")
      (bind _output_get (Variables|Default|SetBulletsInMagazine (- (Variables|Default|GetBulletsInMagazine) 1)))
      (if (< _output_get 1)
        (Development|SetHiddeninGame (Variables|Default|Getmg15na_ammo_belt) true false))
      (if (and (> _output_get 0) (Variables|Default|GetisShooting))
        (bind _returnvalue_4 (Game|SpawnActorfromClass "/Game/Blueprints/Ammo/CartridgeCase.CartridgeCase_C" _returnvalue_3 "Undefined" 0 0))
        (bind _returnvalue_5 (Game|SpawnActorfromClass "/Game/Blueprints/Ammo/ChainLink.ChainLink_C" _returnvalue_3 "Undefined" 0 0))
        (Physics|SetSimulatePhysics (Variables|/Game/Blueprints/Ammo/CartridgeCase.CartridgeCase_C|GetCartridgeCase _returnvalue_4) true)
        (Physics|AddImpulse (Variables|/Game/Blueprints/Ammo/CartridgeCase.CartridgeCase_C|GetCartridgeCase _returnvalue_4) (* (Math|Vector|Normalize (- (Transformation|GetWorldLocation (Variables|Default|GetEjectionPoint)) (Transformation|GetWorldLocation (Variables|Default|GetEjectionDirection))) 0.1) "-2.000000,-2.000000,-2.000000") "None" false)
        (Utilities|FlowControl|Delay 0.12)
        (goto _label))))
  (:Completed
    (Variables|Default|SetisShooting false)))

(event Collision|EventActorBeginOverlap
  (params (OtherActor :type Actor%20Object%20Reference))
  ;[1 1 1] Reloading - Attaching magazine to gun
  (if (== (Utilities|GetClass OtherActor) "/Game/Blueprints/Ammo/Magazine_MG15nA.Magazine_MG15nA_C")
    (if (and (Variables|Default|GetisTopCoverOpen) (not (Variables|Default|GetisMagazineAttached)))
      (bind _asmagazine_mg15n_a (Utilities|Casting|CastToMagazine_MG15nA OtherActor))
      (bind _output_get (Variables|Default|SetMagazineActor _asmagazine_mg15n_a))
      (bind _output_get_2 (Variables|Default|SetBulletsInMagazine (Variables|/Game/Blueprints/Ammo/Magazine_MG15nA.Magazine_MG15nA_C|GetBulletsInMagazine _output_get)))
      (Actor|DestroyActor OtherActor)
      (Development|SetHiddeninGame (Variables|Default|Getmg15na_magazine) false true)
      (Development|SetHiddeninGame (Variables|Default|Getmg15na_ammo_belt) (< _output_get_2 1) false)
      (Variables|Default|SetisMagazineAttached true))))

(event EventTick
  (params (DeltaSeconds :type Float%20%28single-precision%29))
  (bind _maingripcontroller (Variables|Default|GetMainGripController))
  (bind _secondarygripcontroller (Variables|Default|GetSecondaryGripController))
  (bind _topcovergripcontroller (Variables|Default|GetTopCoverGripController))
  (bind _mg15na_top_cover (Variables|Default|Getmg15na_top_cover))
  (bind _mg15na_housing (Variables|Default|Getmg15na_housing))
  (bind _mg15na_top_cover_2 (Variables|Default|Getmg15na_top_cover))
  (bind _mg15na_handle_bolt (Variables|Default|Getmg15na_handle_bolt))
  (bind _mg15na_handle_bolt_2 (Variables|Default|Getmg15na_handle_bolt))
  (bind _mg15na_handle_bolt_3 (Variables|Default|Getmg15na_handle_bolt))
  (bind _returnvalue (Transformation|GetWorldLocation _maingripcontroller))
  (bind _returnvalue_2 (Transformation|GetWorldLocation _secondarygripcontroller))
  (bind _returnvalue_3 (Transformation|GetWorldRotation _mg15na_housing))
  (bind _relativelocation (Variables|/Script/Engine.SceneComponent|GetRelativeLocation _mg15na_handle_bolt_2))
  (bind _relativerotation (Variables|/Script/Engine.SceneComponent|GetRelativeRotation _mg15na_top_cover))
  (bind _returnvalue_4 (Math|Rotator|FindLookatRotation _returnvalue _returnvalue_2))
  (if (and (Utilities|IsValid (Variables|Default|GetMainGripController)) (Utilities|IsValid (Variables|Default|GetSecondaryGripController))) ; Checks if the player grabbed with both hands
    ;[1 1 1] Two handed grab rotating
    (Transformation|SetWorldRotation (Variables|Default|GetGripPoint) (Math|Rotator|MakeRotator 0.0 (+ (.pitch _returnvalue_4) 2e+01) (.yaw _returnvalue_4)) false false)
    (elif (Utilities|IsValid _topcovergripcontroller)
      ;[1 1 1] Top cover rotating
      (Transformation|SetWorldRotation _mg15na_top_cover (Math|Rotator|MakeRotator (- (.pitch (Math|Rotator|FindLookatRotation (Transformation|GetWorldLocation _mg15na_housing) (Transformation|GetWorldLocation _topcovergripcontroller))) 5e+01) (.pitch _returnvalue_3) (.yaw _returnvalue_3)) false false)
      ;[1 1 1] Controls the open/closed state of the top cover
      (Variables|Default|SetisTopCoverClosed (not (> (.roll _relativerotation) 0.0)))
      (if (> (.roll _relativerotation) 3e+01)
        (Variables|Default|SetisTopCoverOpen true)
        (if (> (.roll _relativerotation) 4e+01)
          (Transformation|SetRelativeRotation _mg15na_top_cover_2 "0.000000,0.000000,40.000000" false false))
        (elif (< (.roll _relativerotation) 2e+01)
          (Variables|Default|SetisTopCoverOpen false)
          (if (< (.roll _relativerotation) 0.0)
            (Variables|Default|SetisTopCoverClosed true)
            (Transformation|SetRelativeRotation _mg15na_top_cover_2 "0, 0, 0" false false))))
      (elif (Utilities|IsValid (Variables|Default|GetChargingHandleController))
        (Transformation|SetWorldLocation _mg15na_handle_bolt (Transformation|GetWorldLocation (Variables|Default|GetChargingHandleController)) false false)
        (Transformation|SetRelativeLocation _mg15na_handle_bolt (Math|Vector|MakeVector 0.0 (+ (.y (Variables|/Script/Engine.SceneComponent|GetRelativeLocation _mg15na_handle_bolt)) 17.0) 0.0) false false)
        (if (> (.y _relativelocation) 0.0)
          (Transformation|SetRelativeLocation _mg15na_handle_bolt_3 "0, 0, 0" false false)
          (bind _output_get (Variables|Default|SetisBulletInChamber (and (Variables|Default|GetpulledBack) (Variables|Default|GetisMagazineAttached))))
          (Development|PrintString "loaded bullet in chamber" _output_get _output_get "(R=1.000000,G=0.000000,B=0.726251,A=1.000000)")
          (elif (< (.y _relativelocation) -1e+01)
            (Transformation|SetRelativeLocation _mg15na_handle_bolt_3 "0.000000,-10.000000,0.000000" false false)
            (Variables|Default|SetpulledBack true)))))))

(event EventRelease
  (params (MotionController :type Motion%20Controller%20Component%20Object%20Reference))
  (bind _returnvalue (Game|GetPlayerController 0))
  (bind _mg15na_housing (Variables|Default|Getmg15na_housing))
  (bind _secondarygripcollision (Variables|Default|GetSecondaryGripCollision))
  (bind _returnvalue_2 (Transformation|GetWorldRotation _mg15na_housing))
  (bind _returnvalue_3 (Transformation|GetWorldTransform _secondarygripcollision))
  (Utilities|FlowControl|Sequence
    (:then_0
      (if (== MotionController (Variables|Default|GetMainGripController))
        (Transformation|DetachFromComponent (Variables|Default|GetGripPoint) "KeepWorld" "KeepWorld" "KeepWorld" true)
        ;[1 1 1] Trigger removal
        (Input|DisableInput _returnvalue)
        (Input|RemoveMappingContext (PlayerController|LocalPlayerSubsystems|GetEnhancedInputLocalPlayerSubsystem _returnvalue) (select (== (Variables|/Script/HeadMountedDisplay.MotionControllerComponent|GetMotionSource (Variables|Default|GetMainGripController)) "Right") "/Game/VRTemplate/Input/IMC_Weapon_Right.IMC_Weapon_Right" "/Game/VRTemplate/Input/IMC_Weapon_Left.IMC_Weapon_Left") "(bIgnoreAllPressedKeysUntilRelease=True,bForceImmediately=False)")
        (Variables|Default|SetMainGripController 0)
        (Utilities|String|LogString "MyLog: Detached Main Grip Controller")
        (bind _secondarygripcontroller (Variables|Default|GetSecondaryGripController)
          (:then
            (Transformation|DetachFromComponent _mg15na_housing "KeepWorld" "KeepWorld" "KeepWorld" true)
            (Transformation|SetWorldTransform (Variables|Default|GetGripPoint) (Math|Transform|MakeTransform (.location _returnvalue_3) (Math|Rotator|MakeRotator (+ (.roll (.rotation _returnvalue_3)) (- (.roll (Transformation|GetWorldRotation _secondarygripcontroller)) (.roll _returnvalue_2))) (+ (.pitch (.rotation _returnvalue_3)) (- (.pitch (Transformation|GetWorldRotation _secondarygripcontroller)) (.pitch _returnvalue_2))) (+ (.yaw (.rotation _returnvalue_3)) (- (.yaw (Transformation|GetWorldRotation _secondarygripcontroller)) (.yaw _returnvalue_2)))) (.scale _returnvalue_3)) false false)
            (Transformation|AttachComponentToComponent (Variables|Default|Getmg15na_housing) (Variables|Default|GetGripPoint) "None" "KeepWorld" "KeepWorld" "KeepWorld" true)
            (bind _returnvalue_4 (Transformation|AttachComponentToComponent (Variables|Default|GetGripPoint) _secondarygripcontroller "None" "SnapToTarget" "SnapToTarget" "KeepRelative" true))
            (Variables|Default|SetisSecondaryControllerAttached _returnvalue_4))
          (:else))))
    (:then_1
      (if (== MotionController (Variables|Default|GetSecondaryGripController))
        (if (Variables|Default|GetisSecondaryControllerAttached)
          (Transformation|DetachFromComponent (Variables|Default|GetGripPoint) "KeepWorld" "KeepWorld" "KeepWorld" true)
          (Variables|Default|SetisSecondaryControllerAttached false)
          (Transformation|DetachFromComponent (Variables|Default|Getmg15na_housing) "KeepWorld" "KeepWorld" "KeepWorld" true)
          (Transformation|SetWorldTransform (Variables|Default|GetGripPoint) (Transformation|GetWorldTransform (Variables|Default|GetMainGripCollision)) false false)
          (Transformation|AttachComponentToComponent (Variables|Default|Getmg15na_housing) (Variables|Default|GetGripPoint) "None" "KeepWorld" "KeepWorld" "KeepWorld" true)
          (if (Utilities|IsValid (Variables|Default|GetMainGripController))
            (Transformation|AttachComponentToComponent (Variables|Default|GetGripPoint) (Variables|Default|GetMainGripController) "None" "SnapToTarget" "SnapToTarget" "SnapToTarget" true)))
        (Variables|Default|SetSecondaryGripController 0)
        (Utilities|String|LogString "MyLog: Released Secondary Grip Controller")
        (if (Utilities|Enum|Equal(Enum) (Utilities|GetObjectName MotionController) "MotionControllerRight")
          (Development|SetHiddeninGame (Variables|Default|GetSecondaryHandRight) true false)
          (Development|SetHiddeninGame (Variables|Default|GetRightHand) false false)
          (else
            (Development|SetHiddeninGame (Variables|Default|GetSecondaryHandLeft) true false)
            (Development|SetHiddeninGame (Variables|Default|GetLeftHand) false false)))
        (bind _maingripcontroller (Variables|Default|GetMainGripController)
          (:then
            (Transformation|SetWorldRotation (Variables|Default|GetGripPoint) (Transformation|GetWorldRotation _maingripcontroller) false false))
          (:else))
        (elif (== MotionController (Variables|Default|GetTopCoverGripController))
          (Variables|Default|SetTopCoverGripController 0)
          (else
            ;[1 1 1] Reloading - Detaching magazine from hand
            (if (== MotionController (Variables|Default|GetMagazineGripController))
              (bind _magazineactor (Variables|Default|GetMagazineActor)
                (:then
                  (Transformation|DetachFromActor _magazineactor "KeepWorld" "KeepWorld" "KeepWorld")
                  (Variables|Default|SetMagazineGripController 0))
                (:else))
              (elif (== MotionController (Variables|Default|GetChargingHandleController))
                (Variables|Default|SetChargingHandleController 0)))))))))

(event EventGrab
  (params (MotionController :type Motion%20Controller%20Component%20Object%20Reference))
  (bind _returnvalue (Game|GetPlayerController 0))
  (bind _maingripcollision (Variables|Default|GetMainGripCollision))
  (bind _secondarygripcollision (Variables|Default|GetSecondaryGripCollision))
  (bind _magazinegripcollision (Variables|Default|GetMagazineGripCollision))
  (bind _topcovergripcollision (Variables|Default|GetTopCoverGripCollision))
  (bind _boltgripcollision (Variables|Default|GetBoltGripCollision))
  (Utilities|String|LogString "MyLog: Grab started")
  (if (<= (Math|Vector|Distance(Vector) (Transformation|GetWorldLocation MotionController) (Transformation|GetWorldLocation _maingripcollision)) (Variables|/Script/Engine.SphereComponent|GetSphereRadius _maingripcollision))
    (bind _output_get (Variables|Default|SetMainGripController MotionController))
    ;[1 1 1] Trigger assignment
    (Input|EnableInput _returnvalue)
    (bind _output_get_2 (Variables|Default|SetMappingContext (select (== (Variables|/Script/HeadMountedDisplay.MotionControllerComponent|GetMotionSource _output_get) "Right") "/Game/VRTemplate/Input/IMC_Weapon_Right.IMC_Weapon_Right" "/Game/VRTemplate/Input/IMC_Weapon_Left.IMC_Weapon_Left")))
    (Input|AddMappingContext (PlayerController|LocalPlayerSubsystems|GetEnhancedInputLocalPlayerSubsystem _returnvalue) _output_get_2 0 "(bIgnoreAllPressedKeysUntilRelease=True,bForceImmediately=False)")
    (Variables|Default|GetSecondaryGripController
      (:then
        (Transformation|DetachFromComponent (Variables|Default|GetGripPoint) "KeepWorld" "KeepWorld" "KeepWorld" true)
        (Transformation|DetachFromComponent (Variables|Default|Getmg15na_housing) "KeepWorld" "KeepWorld" "KeepWorld" true)
        (Transformation|SetWorldTransform (Variables|Default|GetGripPoint) (Transformation|GetWorldTransform (Variables|Default|GetMainGripCollision)) false false)
        (Transformation|AttachComponentToComponent (Variables|Default|Getmg15na_housing) (Variables|Default|GetGripPoint) "None" "KeepWorld" "KeepWorld" "KeepWorld" true))
      (:else
        _))
    (Transformation|AttachComponentToComponent (Variables|Default|GetGripPoint) _output_get "None" "SnapToTarget" "SnapToTarget" "KeepRelative" true)
    (Development|PrintString "MyLog: Attached Main Grip Controller" false)
    (Utilities|FlowControl|DelayUntilNextTick)
    (Utilities|FlowControl|DelayUntilNextTick)
    (if (Utilities|Enum|Equal(Enum) (Utilities|GetObjectName _output_get) "MotionControllerRight")
      (Variables|/Game/Characters/MannequinsXR/Meshes/SK_MannequinsXR_AnimBlueprint.SK_MannequinsXR_AnimBlueprint_C|SetBlendSpaceEnum (Variables|Default|GetRightHandAnim) "NewEnumerator10")
      (else
        (Variables|/Game/Characters/MannequinsXR/Meshes/SK_MannequinsXR_AnimBlueprint.SK_MannequinsXR_AnimBlueprint_C|SetBlendSpaceEnum (Variables|Default|GetLeftHandAnim) "NewEnumerator10")))
    (elif (<= (Math|Vector|Distance(Vector) (Transformation|GetWorldLocation MotionController) (Transformation|GetWorldLocation _secondarygripcollision)) (Variables|/Script/Engine.SphereComponent|GetSphereRadius _secondarygripcollision))
      (Variables|Default|SetSecondaryGripController MotionController)
      (Utilities|String|LogString "MyLog: Set Secondary Grip Controller")
      (if (Utilities|Enum|Equal(Enum) (Utilities|GetObjectName MotionController) "MotionControllerRight")
        (Development|SetHiddeninGame (Variables|Default|GetSecondaryHandRight) false false)
        (Development|SetHiddeninGame (Variables|Default|GetRightHand) true false)
        (else
          (Development|SetHiddeninGame (Variables|Default|GetSecondaryHandLeft) false false)
          (Development|SetHiddeninGame (Variables|Default|GetLeftHand) true false)))
      (if (not (Utilities|IsValid (Variables|Default|GetMainGripController)))
        (Transformation|AttachComponentToComponent (Variables|Default|GetGripPoint) (Variables|Default|GetSecondaryGripController) "None" "KeepWorld" "KeepWorld" "KeepWorld" true)
        (Variables|Default|SetisSecondaryControllerAttached true))
      (else
        ;[1 1 1] Reloading - Detaching magazine from gun
        (if (and (<= (Math|Vector|Distance(Vector) (Transformation|GetWorldLocation MotionController) (Transformation|GetWorldLocation _topcovergripcollision)) (Variables|/Script/Engine.SphereComponent|GetSphereRadius _topcovergripcollision)) (not (Variables|Default|GetisShooting)))
          (Variables|Default|SetTopCoverGripController MotionController)
          (if (Utilities|Enum|Equal(Enum) (Utilities|GetObjectName MotionController) "MotionControllerRight") :!label _label
            (Variables|/Game/Characters/MannequinsXR/Meshes/SK_MannequinsXR_AnimBlueprint.SK_MannequinsXR_AnimBlueprint_C|SetBlendSpaceEnum (Variables|Default|GetRightHandAnim) "NewEnumerator3")
            (else
              (Variables|/Game/Characters/MannequinsXR/Meshes/SK_MannequinsXR_AnimBlueprint.SK_MannequinsXR_AnimBlueprint_C|SetBlendSpaceEnum (Variables|Default|GetLeftHandAnim) "NewEnumerator3")))
          (elif (and (<= (Math|Vector|Distance(Vector) (Transformation|GetWorldLocation MotionController) (Transformation|GetWorldLocation _magazinegripcollision)) (Variables|/Script/Engine.SphereComponent|GetSphereRadius _magazinegripcollision)) (Variables|Default|GetisTopCoverOpen))
            (bind _output_get_3 (Variables|Default|SetMagazineGripController MotionController))
            (if (Variables|Default|GetisMagazineAttached)
              (Development|SetHiddeninGame (Variables|Default|Getmg15na_magazine) true true)
              (Variables|Default|SetisBulletInChamber false)
              (Variables|Default|SetpulledBack false)
              (bind _returnvalue_2 (Game|SpawnActorfromClass "/Game/Blueprints/Ammo/Magazine_MG15nA.Magazine_MG15nA_C" (Transformation|GetWorldTransform (Variables|Default|Getmg15na_magazine)) "Undefined" 0 0))
              (bind _output_get_4 (Variables|Default|SetMagazineActor _returnvalue_2))
              (bind _output_get_5 (Variables|/Game/Blueprints/Ammo/Magazine_MG15nA.Magazine_MG15nA_C|SetBulletsInMagazine _output_get_4 (Variables|Default|GetBulletsInMagazine)))
              (if (< _output_get_5 4)
                (Development|SetHiddeninGame (Variables|/Game/Blueprints/Ammo/Magazine_MG15nA.Magazine_MG15nA_C|Getmg15na_ammo_belt_short _output_get_4) true true))
              (if (Utilities|Enum|Equal(Enum) (Utilities|GetObjectName _output_get_3) "MotionControllerRight")
                (Variables|/Game/Characters/MannequinsXR/Meshes/SK_MannequinsXR_AnimBlueprint.SK_MannequinsXR_AnimBlueprint_C|SetBlendSpaceEnum (Variables|Default|GetRightHandAnim) "NewEnumerator6")
                (Transformation|AttachComponentToComponent (Variables|/Script/Engine.Actor|GetRootComponent _output_get_4) (Variables|Default|GetRightHand) "allFingerOpenGrabWideSocket" "SnapToTarget" "SnapToTarget" "SnapToTarget" true)
                (else
                  (Variables|/Game/Characters/MannequinsXR/Meshes/SK_MannequinsXR_AnimBlueprint.SK_MannequinsXR_AnimBlueprint_C|SetBlendSpaceEnum (Variables|Default|GetLeftHandAnim) "NewEnumerator6")
                  (Transformation|AttachComponentToComponent (Variables|/Script/Engine.Actor|GetRootComponent _output_get_4) (Variables|Default|GetLeftHand) "allFingerOpenGrabWideSocket" "SnapToTarget" "SnapToTarget" "SnapToTarget" true)))
              (Variables|Default|SetisMagazineAttached false))
            (elif (<= (Math|Vector|Distance(Vector) (Transformation|GetWorldLocation MotionController) (Transformation|GetWorldLocation _boltgripcollision)) (Variables|/Script/Engine.SphereComponent|GetSphereRadius _boltgripcollision))
              (Variables|Default|SetChargingHandleController MotionController)
              (goto _label))))))))

(event EventBeginPlay
  (bind _returnvalue (Game|Player|GetPlayerPawn 0))
  (bind _output_get (Variables|Default|SetLeftHand (Utilities|Array|Get(acopy) (Actor|GetComponentsbyTag _returnvalue "/Script/Engine.SkeletalMeshComponent" "HandLeft"))))
  (bind _output_get_2 (Variables|Default|SetRightHand (Utilities|Array|Get(acopy) (Actor|GetComponentsbyTag _returnvalue "/Script/Engine.SkeletalMeshComponent" "HandRight"))))
  (bind _assk_mannequins_xr_anim_blueprint (Utilities|Casting|CastToSK_MannequinsXR_AnimBlueprint (Components|SkeletalMesh|GetAnimInstance _output_get)))
  (Variables|Default|SetLeftHandAnim _assk_mannequins_xr_anim_blueprint)
  (bind _assk_mannequins_xr_anim_blueprint_2 (Utilities|Casting|CastToSK_MannequinsXR_AnimBlueprint (Components|SkeletalMesh|GetAnimInstance _output_get_2)))
  (Variables|Default|SetRightHandAnim _assk_mannequins_xr_anim_blueprint_2))

(fn ConstructionScript)