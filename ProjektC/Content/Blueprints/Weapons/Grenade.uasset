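; VR grenade that the player grabs from the body or world, arms with the trigger, and releases.
; GripCollision overlaps gate grabbing per hand; Grab notifies Body, sets the hand's animation pose, snaps to its socket and adds that hand's input mapping.
; Shoot input plays a click and starts a delayed explosion with radial damage, sound and particles.
; Release removes input, detaches the grenade, re-enables physics and sets a fixed projectile velocity.
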(event OnComponentBeginOverlap(GripCollision)
  (params (OverlappedComponent :type Primitive%20Component%20Object%20Reference) (OtherActor :type Actor%20Object%20Reference) (OtherComp :type Primitive%20Component%20Object%20Reference) (OtherBodyIndex :type Integer) (bFromSweep :type Boolean) (SweepResult :type Hit%20Result%20Structure%20%28by%20ref%29))
  (bind _returnvalue (Utilities|GetObjectName OtherComp))
  (if (Utilities|Enum|Equal(Enum) _returnvalue "HandCollisionLeft")
    (Variables|Default|SetgrabbableLeft true)
    (elif (Utilities|Enum|Equal(Enum) _returnvalue "HandCollisionRight")
      (Variables|Default|SetgrabbableRight true))))

(event OnComponentEndOverlap(GripCollision)
  (params (OverlappedComponent :type Primitive%20Component%20Object%20Reference) (OtherActor :type Actor%20Object%20Reference) (OtherComp :type Primitive%20Component%20Object%20Reference) (OtherBodyIndex :type Integer))
  (bind _returnvalue (Utilities|GetObjectName OtherComp))
  (if (Utilities|Enum|Equal(Enum) _returnvalue "HandCollisionLeft")
    (Variables|Default|SetgrabbableLeft false)
    (elif (Utilities|Enum|Equal(Enum) _returnvalue "HandCollisionRight")
      (Variables|Default|SetgrabbableRight false))))

(event Custom|ExplodeAfterTime
  (bind _grenade (Variables|Default|GetGrenade))
  (bind _returnvalue (Transformation|GetWorldLocation _grenade))
  (Utilities|FlowControl|Delay 8.0)
  (Game|Damage|ApplyRadialDamage 1e+02 _returnvalue 5e+02 0 0 self 0 false "ECC_Visibility")
  (Audio|PlaySoundatLocation "/Game/StarterContent/Audio/Explosion_Cue.Explosion_Cue" _returnvalue "0, 0, 0" 1.0 1.0 0.0 0 0 0 0)
  (Effects|SpawnEmitteratLocation "/Game/Realistic_Starter_VFX_Pack_Vol2/Particles/Explosion/P_Explosion_Big_A.P_Explosion_Big_A" _returnvalue)
  (Actor|DestroyActor))

(event Input|EnhancedActionEvents|EnhancedInputActionIA_Shoot_Left
  (params (ActionValue :type Boolean) (ElapsedSeconds :type Float%20%28double-precision%29) (TriggeredSeconds :type Float%20%28double-precision%29) (InputAction :type Input%20Action%20Object%20Reference :default "/Game/VRTemplate/Input/Actions/IA_Shoot_Left.IA_Shoot_Left"))
  (:Started
    (CallFunction|ExplodeAfterTime)
    (Audio|PlaySoundatLocation "/Game/Sounds/Weapons/Grenade/grenade_click.grenade_click" (Transformation|GetWorldLocation (Variables|Default|GetGrenade)) "0, 0, 0" 1.0 1.0 0.0 0 0 0 0)))

(event Input|EnhancedActionEvents|EnhancedInputActionIA_Shoot_Right
  (params (ActionValue :type Boolean) (ElapsedSeconds :type Float%20%28double-precision%29) (TriggeredSeconds :type Float%20%28double-precision%29) (InputAction :type Input%20Action%20Object%20Reference :default "/Game/VRTemplate/Input/Actions/IA_Shoot_Right.IA_Shoot_Right"))
  (:Started
    (CallFunction|ExplodeAfterTime)
    (Audio|PlaySoundatLocation "/Game/Sounds/Weapons/Grenade/grenade_click.grenade_click" (Transformation|GetWorldLocation (Variables|Default|GetGrenade)) "0, 0, 0" 1.0 1.0 0.0 0 0 0 0)))

(event EventBeginPlay
  (bind _returnvalue (Game|Player|GetPlayerPawn 0))
  (bind _returnvalue_2 (Actor|GetActorOfClass "/Game/Blueprints/Body.Body_C"))
  (Variables|Default|Setbody _returnvalue_2)
  (bind _output_get (Variables|Default|SetLeftHand (Utilities|Array|Get(acopy) (Actor|GetComponentsbyTag _returnvalue "/Script/Engine.SkeletalMeshComponent" "HandLeft"))))
  (bind _output_get_2 (Variables|Default|SetRightHand (Utilities|Array|Get(acopy) (Actor|GetComponentsbyTag _returnvalue "/Script/Engine.SkeletalMeshComponent" "HandRight"))))
  (bind _assk_mannequins_xr_anim_blueprint (Utilities|Casting|CastToSK_MannequinsXR_AnimBlueprint (Components|SkeletalMesh|GetAnimInstance _output_get)))
  (Variables|Default|SetLeftHandAnim _assk_mannequins_xr_anim_blueprint)
  (bind _assk_mannequins_xr_anim_blueprint_2 (Utilities|Casting|CastToSK_MannequinsXR_AnimBlueprint (Components|SkeletalMesh|GetAnimInstance _output_get_2)))
  (Variables|Default|SetRightHandAnim _assk_mannequins_xr_anim_blueprint_2)
  (Variables|/Script/Engine.MovementComponent|SetVelocity (Variables|Default|GetProjectileMovement) (* (Transformation|GetVelocity) (* (Transformation|GetDistanceTo (Game|Player|GetPlayerPawn 0)) 0.55)))
  (Utilities|FlowControl|Delay 0.2)
  (Collision|SetCollisionEnabled (Variables|Default|GetBox) "QueryOnly"))

(event EventRelease
  (params (MotionController :type Motion%20Controller%20Component%20Object%20Reference))
  (bind _returnvalue (Game|GetPlayerController 0))
  ;[1 1 1] Trigger removal
  (Input|DisableInput _returnvalue)
  (Input|RemoveMappingContext (PlayerController|LocalPlayerSubsystems|GetEnhancedInputLocalPlayerSubsystem _returnvalue) (select (== (Variables|/Script/HeadMountedDisplay.MotionControllerComponent|GetMotionSource (stale EventGrab MotionController)) "Right") "/Game/VRTemplate/Input/IMC_Weapon_Right.IMC_Weapon_Right" "/Game/VRTemplate/Input/IMC_Weapon_Left.IMC_Weapon_Left") "(bIgnoreAllPressedKeysUntilRelease=True,bForceImmediately=False)")
  (Transformation|DetachFromComponent (Variables|Default|GetBox) "KeepWorld" "KeepWorld" "KeepWorld" true)
  (Physics|SetSimulatePhysics (Variables|Default|GetGrenade) true)
  (Variables|Default|SetphysicsEnabled true)
  (Variables|/Script/Engine.MovementComponent|SetVelocity (Variables|Default|GetProjectileMovement) (Math|Vector|MakeVector 2e+01 0.0 1e+01)))

(event EventGrab
  (params (MotionController :type Motion%20Controller%20Component%20Object%20Reference))
  (bind _returnvalue (Game|GetPlayerController 0))
  (if (or (and (Utilities|Enum|Equal(Enum) (Utilities|GetObjectName MotionController) "MotionControllerRight") (Variables|Default|GetgrabbableRight)) (and (Utilities|Enum|Equal(Enum) (Utilities|GetObjectName MotionController) "MotionControllerLeft") (Variables|Default|GetgrabbableLeft)))
    (if (Variables|Default|GetspawnedOnBody)
      (Default|GrenadeGrabbed (Variables|Default|Getbody))
      (Variables|Default|SetspawnedOnBody false))
    (if (Variables|Default|GetphysicsEnabled)
      (Physics|SetSimulatePhysics (Variables|Default|GetGrenade) false)
      (Variables|Default|SetphysicsEnabled false))
    ;[1 1 1] Trigger assignment
    (Input|EnableInput _returnvalue)
    (bind _output_get (Variables|Default|SetMappingContext (select (== (Variables|/Script/HeadMountedDisplay.MotionControllerComponent|GetMotionSource MotionController) "Right") "/Game/VRTemplate/Input/IMC_Weapon_Right.IMC_Weapon_Right" "/Game/VRTemplate/Input/IMC_Weapon_Left.IMC_Weapon_Left")))
    (Input|AddMappingContext (PlayerController|LocalPlayerSubsystems|GetEnhancedInputLocalPlayerSubsystem _returnvalue) _output_get 0 "(bIgnoreAllPressedKeysUntilRelease=True,bForceImmediately=False)")
    (if (Utilities|Enum|Equal(Enum) (Utilities|GetObjectName MotionController) "MotionControllerRight")
      ;[1 1 1] adjust if new mesh is added
      (Variables|/Game/Characters/MannequinsXR/Meshes/SK_MannequinsXR_AnimBlueprint.SK_MannequinsXR_AnimBlueprint_C|SetBlendSpaceEnum (Variables|Default|GetRightHandAnim) "NewEnumerator3")
      (Transformation|AttachComponentToComponent (Variables|Default|GetBox) (Variables|Default|GetRightHand) "grenadeSocket" "SnapToTarget" "SnapToTarget" "SnapToTarget" true)
      (else
        (Variables|/Game/Characters/MannequinsXR/Meshes/SK_MannequinsXR_AnimBlueprint.SK_MannequinsXR_AnimBlueprint_C|SetBlendSpaceEnum (Variables|Default|GetLeftHandAnim) "NewEnumerator3")
        (Transformation|AttachComponentToComponent (Variables|Default|GetBox) (Variables|Default|GetLeftHand) "grenadeSocket" "SnapToTarget" "SnapToTarget" "SnapToTarget" true)
        (Transformation|SetWorldScale3D (Variables|Default|GetBox) "1.000000,1.000000,1.000000")))))

(fn ConstructionScript)