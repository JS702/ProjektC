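; VR bolt-action Gewehr 98 rifle that is grabbed by main grip, foregrip or bolt, swapping hand poses and dropping to physics when released.
; Tick aims two-handed grips via look-at rotation; otherwise it drives the bolt's twist and slide from the hand, ejecting casings or live rounds.
; Overlapping Bullet actors reload the open bolt.
; Shooting needs a closed, cycled bolt and spawns projectiles, with random spread unless the secondary grip is held.
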(event OnComponentBeginOverlap(SecondaryGripCollision)
  (params (OverlappedComponent :type Primitive%20Component%20Object%20Reference) (OtherActor :type Actor%20Object%20Reference) (OtherComp :type Primitive%20Component%20Object%20Reference) (OtherBodyIndex :type Integer) (bFromSweep :type Boolean) (SweepResult :type Hit%20Result%20Structure%20%28by%20ref%29))
  (bind _returnvalue (Utilities|GetObjectName OtherComp))
  (if (Utilities|Enum|Equal(Enum) _returnvalue "HandCollisionLeft")
    (Variables|Default|SetSecondaryGrabbableLeft true)
    (elif (Utilities|Enum|Equal(Enum) _returnvalue "HandCollisionRight")
      (Variables|Default|SetSecondaryGrabbableRight true))))

(event OnComponentEndOverlap(SecondaryGripCollision)
  (params (OverlappedComponent :type Primitive%20Component%20Object%20Reference) (OtherActor :type Actor%20Object%20Reference) (OtherComp :type Primitive%20Component%20Object%20Reference) (OtherBodyIndex :type Integer))
  (bind _returnvalue (Utilities|GetObjectName OtherComp))
  (if (Utilities|Enum|Equal(Enum) _returnvalue "HandCollisionLeft")
    (Variables|Default|SetSecondaryGrabbableLeft false)
    (elif (Utilities|Enum|Equal(Enum) _returnvalue "HandCollisionRight")
      (Variables|Default|SetSecondaryGrabbableRight false))))

(event OnComponentBeginOverlap(MainGripCollision)
  (params (OverlappedComponent :type Primitive%20Component%20Object%20Reference) (OtherActor :type Actor%20Object%20Reference) (OtherComp :type Primitive%20Component%20Object%20Reference) (OtherBodyIndex :type Integer) (bFromSweep :type Boolean) (SweepResult :type Hit%20Result%20Structure%20%28by%20ref%29))
  (bind _returnvalue (Utilities|GetObjectName OtherComp))
  (if (Utilities|Enum|Equal(Enum) _returnvalue "HandCollisionLeft")
    (Variables|Default|SetMainGrabbableLeft true)
    (elif (Utilities|Enum|Equal(Enum) _returnvalue "HandCollisionRight")
      (Variables|Default|SetMainGrabbableRight true))))

(event OnComponentEndOverlap(MainGripCollision)
  (params (OverlappedComponent :type Primitive%20Component%20Object%20Reference) (OtherActor :type Actor%20Object%20Reference) (OtherComp :type Primitive%20Component%20Object%20Reference) (OtherBodyIndex :type Integer))
  (bind _returnvalue (Utilities|GetObjectName OtherComp))
  (if (Utilities|Enum|Equal(Enum) _returnvalue "HandCollisionLeft")
    (Variables|Default|SetMainGrabbableLeft false)
    (elif (Utilities|Enum|Equal(Enum) _returnvalue "HandCollisionRight")
      (Variables|Default|SetMainGrabbableRight false))))

(event Input|EnhancedActionEvents|EnhancedInputActionIA_Shoot_Left
  (params (ActionValue :type Boolean) (ElapsedSeconds :type Float%20%28double-precision%29) (TriggeredSeconds :type Float%20%28double-precision%29) (InputAction :type Input%20Action%20Object%20Reference :default "/Game/VRTemplate/Input/Actions/IA_Shoot_Left.IA_Shoot_Left"))
  ;[1 1 1] Shooting
  (:Started
    ;;[1 0 0] Prevents the gun from shooting if:
    ;; - there are no more bullets left in the magazine
    ;; - the user didn't cycle the bolt
    ;; - the bolt isn't closed
    (if (Math|Boolean|ANDBoolean (> (Variables|Default|GetbulletsInMagazine) 0) (not (Variables|Default|GetjustShot)) (Variables|Default|GetisClosed))
      (bind _output_get (Variables|Default|SetbulletsInMagazine (- (Variables|Default|GetbulletsInMagazine) 1)))
      (Variables|Default|SetjustShot true)
      ;;[1 1 1] Visuals
      (Development|SetHiddeninGame (Variables|Default|GetBullet) true false)
      (Development|SetHiddeninGame (Variables|Default|GetCartridgeCase) false false)
      (if (== _output_get 1)
        (Development|SetHiddeninGame (Variables|Default|GetBulletReserve) true false))
      (Audio|PlaySoundatLocation "/Game/Sounds/Weapons/Gewehr98/Gewehr98_shot.Gewehr98_shot" (Transformation|GetWorldLocation (Variables|Default|GetMuzzleEnd)) "0, 0, 0" 1.0 1.0 0.0 0 0 0 0)
      ;;[1 1 1] Projectile spawning
      (bind _spawntransform (CallFunction|RandomBulletSpread (Variables|Default|GetMuzzleEnd) (Variables|Default|GetmaxSpread)))
      (bind _returnvalue (Game|SpawnActorfromClass "/Game/Blueprints/Ammo/MyProjectile.MyProjectile_C" _spawntransform "Undefined" self (Game|Player|GetPlayerPawn 0)))
      (Variables|/Game/Blueprints/Ammo/MyProjectile.MyProjectile_C|Setdamage _returnvalue (Variables|Default|Getdamage))
      (Components|Activation|Activate (Variables|Default|GetMuzzleFlash) true))))

(event Input|EnhancedActionEvents|EnhancedInputActionIA_Shoot_Right
  (params (ActionValue :type Boolean) (ElapsedSeconds :type Float%20%28double-precision%29) (TriggeredSeconds :type Float%20%28double-precision%29) (InputAction :type Input%20Action%20Object%20Reference :default "/Game/VRTemplate/Input/Actions/IA_Shoot_Right.IA_Shoot_Right"))
  ;[1 1 1] Shooting
  (:Started
    ;;[1 0 0] Prevents the gun from shooting if:
    ;; - there are no more bullets left in the magazine
    ;; - the user didn't cycle the bolt
    ;; - the bolt isn't closed
    (if (Math|Boolean|ANDBoolean (> (Variables|Default|GetbulletsInMagazine) 0) (not (Variables|Default|GetjustShot)) (Variables|Default|GetisClosed))
      (bind _output_get (Variables|Default|SetbulletsInMagazine (- (Variables|Default|GetbulletsInMagazine) 1)))
      (Variables|Default|SetjustShot true)
      ;;[1 1 1] Visuals
      (Development|SetHiddeninGame (Variables|Default|GetBullet) true false)
      (Development|SetHiddeninGame (Variables|Default|GetCartridgeCase) false false)
      (if (== _output_get 1)
        (Development|SetHiddeninGame (Variables|Default|GetBulletReserve) true false))
      (Audio|PlaySoundatLocation "/Game/Sounds/Weapons/Gewehr98/Gewehr98_shot.Gewehr98_shot" (Transformation|GetWorldLocation (Variables|Default|GetMuzzleEnd)) "0, 0, 0" 1.0 1.0 0.0 0 0 0 0)
      ;;[1 1 1] Projectile spawning
      (bind _spawntransform (CallFunction|RandomBulletSpread (Variables|Default|GetMuzzleEnd) (Variables|Default|GetmaxSpread)))
      (bind _returnvalue (Game|SpawnActorfromClass "/Game/Blueprints/Ammo/MyProjectile.MyProjectile_C" _spawntransform "Undefined" self (Game|Player|GetPlayerPawn 0)))
      (Variables|/Game/Blueprints/Ammo/MyProjectile.MyProjectile_C|Setdamage _returnvalue (Variables|Default|Getdamage))
      (Components|Activation|Activate (Variables|Default|GetMuzzleFlash) true))))

(event Collision|EventActorBeginOverlap
  (params (OtherActor :type Actor%20Object%20Reference))
  ;[1 1 1] Reloading
  (if (== (Utilities|GetClass OtherActor) "/Game/Blueprints/Ammo/Bullet.Bullet_C")
    (bind _asbullet (Utilities|Casting|CastToBullet OtherActor))
    (if (Math|Boolean|ANDBoolean (not (Variables|/Game/Blueprints/Ammo/Bullet.Bullet_C|GetjustSpawned _asbullet)) (Variables|Default|GetisOpen) (< (Variables|Default|GetbulletsInMagazine) (Variables|Default|GetmagazineSize)))
      (Actor|DestroyActor OtherActor)
      (Development|SetHiddeninGame (Variables|Default|GetBullet) false false)
      (bind _output_get (Variables|Default|SetbulletsInMagazine (+ (Variables|Default|GetbulletsInMagazine) 1)))
      (if (> _output_get 1)
        (Development|SetHiddeninGame (Variables|Default|GetBulletReserve) false false))
      (Development|PrintString (Utilities|String|Append "ReloadLog: Bullets in Magazine: " (Utilities|String|ToString(Integer) _output_get)) false))))

(event EventTick
  (params (DeltaSeconds :type Float%20%28single-precision%29))
  (bind _maingripcontroller (Variables|Default|GetMainGripController))
  (bind _secondarygripcontroller (Variables|Default|GetSecondaryGripController))
  (bind _boltpivot (Variables|Default|GetBoltPivot))
  (bind _rifle (Variables|Default|GetRifle))
  (bind _boltpivot_2 (Variables|Default|GetBoltPivot))
  (bind _boltpivot_3 (Variables|Default|GetBoltPivot))
  (bind _boltgripcontroller (Variables|Default|GetBoltGripController))
  (bind _boltgripcontrollerrotation (Variables|Default|GetBoltGripControllerRotation))
  (bind _boltpivot_4 (Variables|Default|GetBoltPivot))
  (bind _boltmiddlepivot (Variables|Default|GetBoltMiddlePivot))
  (bind _bullet (Variables|Default|GetBullet))
  (bind _returnvalue (Transformation|GetWorldRotation _bullet))
  (bind _returnvalue_2 (Transformation|GetWorldLocation _maingripcontroller))
  (bind _returnvalue_3 (Transformation|GetWorldLocation _secondarygripcontroller))
  (bind _returnvalue_4 (Transformation|GetWorldRotation _rifle))
  (bind _returnvalue_5 (Transformation|GetWorldLocation _bullet))
  (bind _relativelocation (Variables|/Script/Engine.SceneComponent|GetRelativeLocation _boltpivot_2))
  (bind _relativerotation (Variables|/Script/Engine.SceneComponent|GetRelativeRotation _boltgripcontroller))
  (bind _returnvalue_6 (Math|Rotator|FindLookatRotation _returnvalue_2 _returnvalue_3))
  (bind _returnvalue_7 (Math|Vector|MakeVector (.roll _returnvalue_4) (.pitch _returnvalue_4) (.yaw _returnvalue_4)))
  (bind _returnvalue_8 (Math|Transform|MakeTransform _returnvalue_5 _returnvalue))
  (bind _returnvalue_9 (- (.roll _relativerotation) (.roll _boltgripcontrollerrotation)))
  (bind _returnvalue_10 (Math|Vector|RotateVectorAroundAxis _returnvalue_7 9e+01 "0.000000,0.000000,1.000000"))
  (bind _returnvalue_11 (Math|Vector|Normalize _returnvalue_10))
  (if (and (Utilities|IsValid (Variables|Default|GetMainGripController)) (Utilities|IsValid (Variables|Default|GetSecondaryGripController))) ; Checks if the player grabbed with both hands
    ;[1 1 1] Two handed grab rotating
    (Transformation|SetWorldRotation (Variables|Default|GetGripPoint) (Math|Rotator|MakeRotator 0.0 (+ (.pitch _returnvalue_6) 45.0) (.yaw _returnvalue_6)) false false)
    (elif (Utilities|IsValid (Variables|Default|GetBoltGripController)) ; Checks if the player grabbed the bolt
      ;[1 1 1] Rotating
      (if (> (.y (Variables|/Script/Engine.SceneComponent|GetRelativeLocation (Variables|Default|GetBoltPivot))) -0.1) ; The Bolt is only allowed to rotate when its closed
        (if (> _returnvalue_9 -2.0)
          (Transformation|SetRelativeRotation _boltpivot_4 (Math|Rotator|MakeRotator 0.0 0.0 0.0) false false) ; Bolt is fully closed
          ;;[1 0 0] Prevents Bolt_Middle from rotating
          (Transformation|SetRelativeRotation _boltmiddlepivot "0, 0, 0" false false)
          (Variables|Default|SetisClosed true)
          (Variables|Default|Seteject true)
          (elif (< _returnvalue_9 -88.0)
            (Transformation|SetRelativeRotation _boltpivot_4 (Math|Rotator|MakeRotator 0.0 -9e+01 0.0) false false) ; Bolt is ready to be opened (awaiting y-translation)
            (Transformation|SetRelativeRotation _boltmiddlepivot "90.000000,0.000000,0.000000" false false)
            ;[1 1 1] Moving
            (Transformation|SetWorldLocation _boltpivot (Transformation|GetWorldLocation (Variables|Default|GetBoltGripController)) false false :!label _label)
            (Transformation|SetRelativeLocation _boltpivot (Math|Vector|MakeVector 0.0 (- (.y (Variables|/Script/Engine.SceneComponent|GetRelativeLocation _boltpivot)) 35.0) 4.381) false false)
            (if (> (.y _relativelocation) 0.0)
              (Transformation|SetRelativeLocation _boltpivot_3 (Math|Vector|MakeVector (.x _relativelocation) 0.0 (.z _relativelocation)) false false) ; Bolt is ready to be closed (awaiting rotation)
              (elif (< (.y _relativelocation) -1e+01)
                (Transformation|SetRelativeLocation _boltpivot_3 (Math|Vector|MakeVector (.x _relativelocation) -1e+01 (.z _relativelocation)) false false) ; Bolt is fully open
                (Variables|Default|SetisOpen true)
                ;[1 1 1] Ejecting
                (if (Variables|Default|Geteject)
                  (if (Variables|Default|GetjustShot)
                    (bind _returnvalue_12 (Game|SpawnActorfromClass "/Game/Blueprints/Ammo/CartridgeCase.CartridgeCase_C" _returnvalue_8 "Undefined" 0 0))
                    (Development|SetHiddeninGame (Variables|Default|GetCartridgeCase) true false)
                    (if (> (Variables|Default|GetbulletsInMagazine) 0)
                      (Development|SetHiddeninGame (Variables|Default|GetBullet) false false))
                    (Physics|SetSimulatePhysics (Variables|/Game/Blueprints/Ammo/CartridgeCase.CartridgeCase_C|GetCartridgeCase _returnvalue_12) true)
                    (Physics|AddImpulse (Variables|/Game/Blueprints/Ammo/CartridgeCase.CartridgeCase_C|GetCartridgeCase _returnvalue_12) _returnvalue_11 "None" false)
                    (Variables|Default|Seteject false :!label _label_2)
                    (Variables|Default|SetjustShot false)
                    (elif (> (Variables|Default|GetbulletsInMagazine) 0)
                      (bind _returnvalue_13 (Game|SpawnActorfromClass "/Game/Blueprints/Ammo/Bullet.Bullet_C" _returnvalue_8 "Undefined" 0 0))
                      (bind _output_get (Variables|Default|SetbulletsInMagazine (- (Variables|Default|GetbulletsInMagazine) 1)))
                      (if (== _output_get 1)
                        (Development|SetHiddeninGame (Variables|Default|GetBulletReserve) true false)
                        (elif (== _output_get 0)
                          (Development|SetHiddeninGame (Variables|Default|GetBullet) true false)))
                      (Physics|SetSimulatePhysics (Variables|/Game/Blueprints/Ammo/Bullet.Bullet_C|GetBullet _returnvalue_13) true)
                      (Physics|AddImpulse (Variables|/Game/Blueprints/Ammo/Bullet.Bullet_C|GetBullet _returnvalue_13) _returnvalue_11 "None" false)
                      (goto _label_2))))
                (else
                  ;[1 1 1] Bolt is moved somewhere on its y-Axis, but neither open nor closed
                  (Variables|Default|SetisOpen false))))
            (else
              (Transformation|SetRelativeRotation _boltpivot_4 (Math|Rotator|MakeRotator 0.0 _returnvalue_9 0.0) false false)
              (Transformation|SetRelativeRotation _boltmiddlepivot (Math|Rotator|MakeRotator 0.0 (* _returnvalue_9 -1.0) 0.0) false false)
              ;[1 1 1] Bolt is somehow rotated, but neither open nor closed
              (Variables|Default|SetisClosed false))))
        (else
          (goto _label))))))

(event EventGrab
  (params (MotionController :type Motion%20Controller%20Component%20Object%20Reference))
  (bind _returnvalue (Game|GetPlayerController 0))
  (bind _grippoint (Variables|Default|GetGripPoint))
  (bind _boltgripcollision (Variables|Default|GetBoltGripCollision))
  (if (Variables|Default|GetphysicsEnabled)
    (Physics|SetSimulatePhysics (Variables|Default|GetRifle) false)
    (Transformation|SetWorldTransform _grippoint (Transformation|GetWorldTransform (Variables|Default|GetMainGripPosition)) false false)
    (Transformation|AttachComponentToComponent (Variables|Default|GetRifle) _grippoint "None" "KeepWorld" "KeepWorld" "KeepWorld" true)
    (Variables|Default|SetphysicsEnabled false))
  (if (or (and (Utilities|Enum|Equal(Enum) (Utilities|GetObjectName MotionController) "MotionControllerRight") (Variables|Default|GetMainGrabbableRight)) (and (Utilities|Enum|Equal(Enum) (Utilities|GetObjectName MotionController) "MotionControllerLeft") (Variables|Default|GetMainGrabbableLeft)))
    (bind _output_get (Variables|Default|SetMainGripController MotionController))
    ;[1 1 1] Trigger assignment
    (Input|EnableInput _returnvalue)
    (bind _output_get_2 (Variables|Default|SetMappingContext (select (== (Variables|/Script/HeadMountedDisplay.MotionControllerComponent|GetMotionSource _output_get) "Right") "/Game/VRTemplate/Input/IMC_Weapon_Right.IMC_Weapon_Right" "/Game/VRTemplate/Input/IMC_Weapon_Left.IMC_Weapon_Left")))
    (Input|AddMappingContext (PlayerController|LocalPlayerSubsystems|GetEnhancedInputLocalPlayerSubsystem _returnvalue) _output_get_2 0 "(bIgnoreAllPressedKeysUntilRelease=True,bForceImmediately=False)")
    (Variables|Default|GetSecondaryGripController
      (:then
        (Transformation|DetachFromComponent (Variables|Default|GetGripPoint) "KeepWorld" "KeepWorld" "KeepWorld" true)
        (Transformation|DetachFromComponent (Variables|Default|GetRifle) "KeepWorld" "KeepWorld" "KeepWorld" true)
        (Transformation|SetWorldTransform (Variables|Default|GetGripPoint) (Transformation|GetWorldTransform (Variables|Default|GetMainGripPosition)) false false)
        (Transformation|AttachComponentToComponent (Variables|Default|GetRifle) (Variables|Default|GetGripPoint) "None" "KeepWorld" "KeepWorld" "KeepWorld" true))
      (:else
        _))
    (Transformation|AttachComponentToComponent (Variables|Default|GetGripPoint) _output_get "None" "SnapToTarget" "SnapToTarget" "KeepRelative" true)
    (Development|PrintString "MyLog: Attached Main Grip Controller" false)
    (Utilities|FlowControl|DelayUntilNextTick)
    (Utilities|FlowControl|DelayUntilNextTick)
    (if (Utilities|Enum|Equal(Enum) (Utilities|GetObjectName _output_get) "MotionControllerRight")
      (Variables|/Game/Characters/MannequinsXR/Meshes/SK_MannequinsXR_AnimBlueprint.SK_MannequinsXR_AnimBlueprint_C|SetBlendSpaceEnum (Variables|Default|GetRightHandAnim) "NewEnumerator10")
      (else
        (Variables|/Game/Characters/MannequinsXR/Meshes/SK_MannequinsXR_AnimBlueprint.SK_MannequinsXR_AnimBlueprint_C|SetBlendSpaceEnum (Variables|Default|GetLeftHandAnim) "NewEnumerator10")))
    (bind _asvrpawn (Utilities|Casting|CastToVRPawn (Variables|Default|GetVRPawn) :!label _label))
    (Variables|/Game/VRTemplate/Blueprints/VRPawn.VRPawn_C|SetactiveWeapon _asvrpawn self)
    (elif (or (and (Utilities|Enum|Equal(Enum) (Utilities|GetObjectName MotionController) "MotionControllerRight") (Variables|Default|GetSecondaryGrabbableRight)) (and (Utilities|Enum|Equal(Enum) (Utilities|GetObjectName MotionController) "MotionControllerLeft") (Variables|Default|GetSecondaryGrabbableLeft)))
      (Variables|Default|SetSecondaryGripController MotionController)
      (Utilities|String|LogString "MyLog: Set Secondary Grip Controller")
      (if (Utilities|Enum|Equal(Enum) (Utilities|GetObjectName MotionController) "MotionControllerRight")
        (Development|SetHiddeninGame (Variables|Default|GetSecondaryHandRight) false false)
        (Development|SetHiddeninGame (Variables|Default|GetRightHand) true false)
        (else
          (Development|SetHiddeninGame (Variables|Default|GetSecondaryHandLeft) false false)
          (Development|SetHiddeninGame (Variables|Default|GetLeftHand) true false)))
      (if (not (Utilities|IsValid (Variables|Default|GetMainGripController)))
        (Transformation|AttachComponentToComponent (Variables|Default|GetGripPoint) (Variables|Default|GetSecondaryGripController) "None" "KeepWorld" "KeepWorld" "KeepWorld" true)
        (Variables|Default|SetisSecondaryControllerAttached true)
        (goto _label))
      (elif (<= (Math|Vector|Distance(Vector) (Transformation|GetWorldLocation MotionController) (Transformation|GetWorldLocation _boltgripcollision)) (Variables|/Script/Engine.SphereComponent|GetSphereRadius _boltgripcollision))
        (bind _output_get_3 (Variables|Default|SetBoltGripController MotionController))
        (Variables|Default|Seteject false)
        (Variables|Default|SetBoltGripControllerRotation (Variables|/Script/Engine.SceneComponent|GetRelativeRotation _output_get_3))
        (if (Utilities|Enum|Equal(Enum) (Utilities|GetObjectName MotionController) "MotionControllerRight")
          (Variables|/Game/Characters/MannequinsXR/Meshes/SK_MannequinsXR_AnimBlueprint.SK_MannequinsXR_AnimBlueprint_C|SetBlendSpaceEnum (Variables|Default|GetRightHandAnim) "NewEnumerator3")
          (goto _label)
          (else
            (Variables|/Game/Characters/MannequinsXR/Meshes/SK_MannequinsXR_AnimBlueprint.SK_MannequinsXR_AnimBlueprint_C|SetBlendSpaceEnum (Variables|Default|GetLeftHandAnim) "NewEnumerator3")
            (goto _label)))))))

(event EventRelease
  (params (MotionController :type Motion%20Controller%20Component%20Object%20Reference))
  (bind _returnvalue (Game|GetPlayerController 0))
  (bind _secondarygripposition (Variables|Default|GetSecondaryGripPosition))
  (bind _rifle (Variables|Default|GetRifle))
  (bind _returnvalue_2 (Transformation|GetWorldRotation _rifle))
  (bind _returnvalue_3 (Transformation|GetWorldTransform _secondarygripposition))
  (Utilities|FlowControl|Sequence
    (:then_0
      (if (== MotionController (Variables|Default|GetMainGripController))
        (Transformation|DetachFromComponent (Variables|Default|GetGripPoint) "KeepWorld" "KeepWorld" "KeepWorld" true)
        ;[1 1 1] Trigger removal
        (Input|DisableInput _returnvalue)
        (Input|RemoveMappingContext (PlayerController|LocalPlayerSubsystems|GetEnhancedInputLocalPlayerSubsystem _returnvalue) (select (== (Variables|/Script/HeadMountedDisplay.MotionControllerComponent|GetMotionSource (Variables|Default|GetMainGripController)) "Right") "/Game/VRTemplate/Input/IMC_Weapon_Right.IMC_Weapon_Right" "/Game/VRTemplate/Input/IMC_Weapon_Left.IMC_Weapon_Left") "(bIgnoreAllPressedKeysUntilRelease=True,bForceImmediately=False)")
        (Variables|Default|SetMainGripController 0)
        (Utilities|String|LogString "MyLog: Detached Main Grip Controller")
        (bind _secondarygripcontroller (Variables|Default|GetSecondaryGripController)
          (:then
            (Transformation|DetachFromComponent _rifle "KeepWorld" "KeepWorld" "KeepWorld" true)
            (Transformation|SetWorldTransform (Variables|Default|GetGripPoint) (Math|Transform|MakeTransform (.location _returnvalue_3) (Math|Rotator|MakeRotator (+ (.roll (.rotation _returnvalue_3)) (- (.roll (Transformation|GetWorldRotation _secondarygripcontroller)) (.roll _returnvalue_2))) (+ (.pitch (.rotation _returnvalue_3)) (- (.pitch (Transformation|GetWorldRotation _secondarygripcontroller)) (.pitch _returnvalue_2))) (+ (.yaw (.rotation _returnvalue_3)) (- (.yaw (Transformation|GetWorldRotation _secondarygripcontroller)) (.yaw _returnvalue_2)))) (.scale _returnvalue_3)) false false)
            (Transformation|AttachComponentToComponent (Variables|Default|GetRifle) (Variables|Default|GetGripPoint) "None" "KeepWorld" "KeepWorld" "KeepWorld" true)
            (bind _returnvalue_4 (Transformation|AttachComponentToComponent (Variables|Default|GetGripPoint) _secondarygripcontroller "None" "SnapToTarget" "SnapToTarget" "KeepRelative" true))
            (Variables|Default|SetisSecondaryControllerAttached _returnvalue_4))
          (:else
            _))
        (if (and (not (Utilities|IsValid (Variables|Default|GetMainGripController))) (not (Utilities|IsValid (Variables|Default|GetSecondaryGripController)))) :!label _label
          (Variables|Default|SetBoltGripController 0)
          (Physics|SetSimulatePhysics (Variables|Default|GetRifle) true)
          (Variables|Default|SetphysicsEnabled true))))
    (:then_1
      (if (== MotionController (Variables|Default|GetSecondaryGripController))
        (if (Variables|Default|GetisSecondaryControllerAttached)
          (Transformation|DetachFromComponent (Variables|Default|GetGripPoint) "KeepWorld" "KeepWorld" "KeepWorld" true)
          (Variables|Default|SetisSecondaryControllerAttached false)
          (Transformation|DetachFromComponent (Variables|Default|GetRifle) "KeepWorld" "KeepWorld" "KeepWorld" true)
          (Transformation|SetWorldTransform (Variables|Default|GetGripPoint) (Transformation|GetWorldTransform (Variables|Default|GetMainGripPosition)) false false)
          (Transformation|AttachComponentToComponent (Variables|Default|GetRifle) (Variables|Default|GetGripPoint) "None" "KeepWorld" "KeepWorld" "KeepWorld" true)
          (if (Utilities|IsValid (Variables|Default|GetMainGripController))
            (Transformation|AttachComponentToComponent (Variables|Default|GetGripPoint) (Variables|Default|GetMainGripController) "None" "SnapToTarget" "SnapToTarget" "SnapToTarget" true)))
        (Variables|Default|SetSecondaryGripController 0)
        (Utilities|String|LogString "MyLog: Released Secondary Grip Controller")
        (if (Utilities|Enum|Equal(Enum) (Utilities|GetObjectName MotionController) "MotionControllerRight")
          (Development|SetHiddeninGame (Variables|Default|GetSecondaryHandRight) true false)
          (Development|SetHiddeninGame (Variables|Default|GetRightHand) false false)
          (else
            (Development|SetHiddeninGame (Variables|Default|GetSecondaryHandLeft) true false)
            (Development|SetHiddeninGame (Variables|Default|GetLeftHand) false false)))
        (bind _maingripcontroller (Variables|Default|GetMainGripController)
          (:then
            (Transformation|SetWorldRotation (Variables|Default|GetGripPoint) (Transformation|GetWorldRotation _maingripcontroller) false false)
            (goto _label))
          (:else
            (goto _label)))
        (elif (== MotionController (Variables|Default|GetBoltGripController))
          (Variables|Default|SetBoltGripController 0))))))

(event EventBeginPlay
  (bind _returnvalue (Game|Player|GetPlayerPawn 0))
  (Variables|Default|SetVRPawn _returnvalue)
  (bind _output_get (Variables|Default|SetLeftHand (Utilities|Array|Get(acopy) (Actor|GetComponentsbyTag _returnvalue "/Script/Engine.SkeletalMeshComponent" "HandLeft"))))
  (bind _output_get_2 (Variables|Default|SetRightHand (Utilities|Array|Get(acopy) (Actor|GetComponentsbyTag _returnvalue "/Script/Engine.SkeletalMeshComponent" "HandRight"))))
  (bind _assk_mannequins_xr_anim_blueprint (Utilities|Casting|CastToSK_MannequinsXR_AnimBlueprint (Components|SkeletalMesh|GetAnimInstance _output_get)))
  (Variables|Default|SetLeftHandAnim _assk_mannequins_xr_anim_blueprint)
  (bind _assk_mannequins_xr_anim_blueprint_2 (Utilities|Casting|CastToSK_MannequinsXR_AnimBlueprint (Components|SkeletalMesh|GetAnimInstance _output_get_2)))
  (Variables|Default|SetRightHandAnim _assk_mannequins_xr_anim_blueprint_2))

(fn ConstructionScript)

(fn RandomBulletSpread
  (params (spawnPoint :type Arrow%20Component%20Object%20Reference) (maxSpread :type Float%20%28double-precision%29))
  (bind _returnvalue (Transformation|GetWorldRotation spawnPoint))
  ;[1 1 1] Random bullet spread
  (if (Utilities|IsValid (Variables|Default|GetSecondaryGripController))
    (LocalVariables|Setspread 0.0)
    (else
      (LocalVariables|Setspread maxSpread)))
  (return (Math|Transform|MakeTransform (Transformation|GetWorldLocation spawnPoint) (Math|Rotator|MakeRotator (+ (.roll _returnvalue) (Math|Random|RandomFloatinRange (* (LocalVariables|Getspread) -1.0) (LocalVariables|Getspread))) (+ (.pitch _returnvalue) (Math|Random|RandomFloatinRange (* (LocalVariables|Getspread) -1.0) (LocalVariables|Getspread))) (+ (.yaw _returnvalue) (Math|Random|RandomFloatinRange (* (LocalVariables|Getspread) -1.0) (LocalVariables|Getspread)))) (Transformation|GetWorldScale spawnPoint))))