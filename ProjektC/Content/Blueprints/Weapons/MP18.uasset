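; VR MP18 submachine gun with one- or two-handed grabbing, manual reloading and automatic fire.
; Grab/Release route controllers to grips, magazine or charging handle, re-parenting housing around GripPoint and setting hand poses and input mappings.
; Tick aims two-handed grips by look-at rotation, otherwise moves the bolt.
; Shooting loops on delays, spawning spread projectiles and ejected casings; magazines swap between hidden mesh and spawned actor, carrying bullet count.
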(event OnComponentBeginOverlap(SecondaryGripCollision)
  (params (OverlappedComponent :type Primitive%20Component%20Object%20Reference) (OtherActor :type Actor%20Object%20Reference) (OtherComp :type Primitive%20Component%20Object%20Reference) (OtherBodyIndex :type Integer) (bFromSweep :type Boolean) (SweepResult :type Hit%20Result%20Structure%20%28by%20ref%29))
  (bind _returnvalue (Utilities|GetObjectName OtherComp))
  (if (Utilities|Enum|Equal(Enum) _returnvalue "HandCollisionLeft")
    (Variables|Default|SetSecondaryGrabbableLeft true)
    (elif (Utilities|Enum|Equal(Enum) _returnvalue "HandCollisionRight")
      (Variables|Default|SetSecondaryGrabbableRight true))))

(event OnComponentEndOverlap(SecondaryGripCollision)
  (params (OverlappedComponent :type Primitive%20Component%20Object%20Reference) (OtherActor :type Actor%20Object%20Reference) (OtherComp :type Primitive%20Component%20Object%20Reference) (OtherBodyIndex :type Integer))
  (bind _returnvalue (Utilities|GetObjectName OtherComp))
  (if (Utilities|Enum|Equal(Enum) _returnvalue "HandCollisionLeft")
    (Variables|Default|SetSecondaryGrabbableLeft false)
    (elif (Utilities|Enum|Equal(Enum) _returnvalue "HandCollisionRight")
      (Variables|Default|SetSecondaryGrabbableRight false))))

(event OnComponentBeginOverlap(MainGripCollision)
  (params (OverlappedComponent :type Primitive%20Component%20Object%20Reference) (OtherActor :type Actor%20Object%20Reference) (OtherComp :type Primitive%20Component%20Object%20Reference) (OtherBodyIndex :type Integer) (bFromSweep :type Boolean) (SweepResult :type Hit%20Result%20Structure%20%28by%20ref%29))
  (bind _returnvalue (Utilities|GetObjectName OtherComp))
  (if (Utilities|Enum|Equal(Enum) _returnvalue "HandCollisionLeft")
    (Variables|Default|SetMainGrabbableLeft true)
    (elif (Utilities|Enum|Equal(Enum) _returnvalue "HandCollisionRight")
      (Variables|Default|SetMainGrabbableRight true))))

(event OnComponentEndOverlap(MainGripCollision)
  (params (OverlappedComponent :type Primitive%20Component%20Object%20Reference) (OtherActor :type Actor%20Object%20Reference) (OtherComp :type Primitive%20Component%20Object%20Reference) (OtherBodyIndex :type Integer))
  (bind _returnvalue (Utilities|GetObjectName OtherComp))
  (if (Utilities|Enum|Equal(Enum) _returnvalue "HandCollisionLeft")
    (Variables|Default|SetMainGrabbableLeft false)
    (elif (Utilities|Enum|Equal(Enum) _returnvalue "HandCollisionRight")
      (Variables|Default|SetMainGrabbableRight false))))

(event Input|EnhancedActionEvents|EnhancedInputActionIA_Shoot_Left
  (params (ActionValue :type Boolean) (ElapsedSeconds :type Float%20%28double-precision%29) (TriggeredSeconds :type Float%20%28double-precision%29) (InputAction :type Input%20Action%20Object%20Reference :default "/Game/VRTemplate/Input/Actions/IA_Shoot_Left.IA_Shoot_Left"))
  (bind _mp18_bullet_indicator (Variables|Default|Getmp18_bullet_indicator))
  (bind _mp18_bolt (Variables|Default|Getmp18_bolt))
  (bind _ejectionpoint (Variables|Default|GetEjectionPoint))
  (bind _relativerotation (Variables|/Script/Engine.SceneComponent|GetRelativeRotation _mp18_bullet_indicator))
  ;[1 1 1] Shooting
  (:Started
    ;;[1 0 0] Prevents the gun from shooting if:
    ;; - the user wants to shoot faster then the guns rate of fire
    ;; - there are no more bullets left in the magazine and in the chamber
    (if (Math|Boolean|ANDBoolean (Variables|Default|GetisBulletInChamber) (Variables|Default|GetisMagazineAttached) (> (Variables|Default|GetBulletsInMagazine) 0))
      (Variables|Default|SetisShooting true)
      ;;[1 1 1] Projectile spawning
      (bind _spawntransform (CallFunction|RandomBulletSpread (Variables|Default|GetMuzzleEnd) (Variables|Default|GetmaxSpread) :!label _label))
      (Game|SpawnActorfromClass "/Game/Blueprints/Ammo/MyProjectile.MyProjectile_C" _spawntransform "Undefined" self (Game|Player|GetPlayerPawn 0))
      (Components|Activation|Activate (Variables|Default|GetMuzzleFlash) true)
      (Development|PrintString "ShootLog: Shot fired")
      (bind _output_get (Variables|Default|SetBulletsInMagazine (- (Variables|Default|GetBulletsInMagazine) 1)))
      (if (> _output_get 12)
        (Transformation|SetRelativeRotation _mp18_bullet_indicator (Math|Rotator|MakeRotator (+ (.roll _relativerotation) 13.0) (.pitch _relativerotation) (.yaw _relativerotation)) false false))
      (if (and (> _output_get 0) (Variables|Default|GetisShooting))
        (Variables|Default|SetslideForward true)
        (Utilities|FlowControl|Delay 0.06)
        (Variables|Default|SetslideForward false)
        (Transformation|SetRelativeLocation _mp18_bolt (Math|Vector|MakeVector 0.0 12.0 0.0) false false)
        (Variables|Default|SetslideBack true)
        (Utilities|FlowControl|Delay 0.06)
        (Variables|Default|SetslideBack false)
        (Transformation|SetRelativeLocation _mp18_bolt (Math|Vector|MakeVector 0.0 0.0 0.0) false false)
        ;;[1 1 1] Cardridge case ejection
        (bind _returnvalue (Game|SpawnActorfromClass "/Game/Blueprints/Ammo/CartridgeCase_MP18.CartridgeCase_MP18_C" (Math|Transform|MakeTransform (Transformation|GetWorldLocation _ejectionpoint) (Transformation|GetWorldRotation _ejectionpoint)) "Undefined" 0 0))
        (Physics|SetSimulatePhysics (Variables|/Game/Blueprints/Ammo/CartridgeCase_MP18.CartridgeCase_MP18_C|Getmp18_cartridgeCase _returnvalue) true)
        (Physics|AddImpulse (Variables|/Game/Blueprints/Ammo/CartridgeCase_MP18.CartridgeCase_MP18_C|Getmp18_cartridgeCase _returnvalue) (* (Math|Vector|Normalize (- (Transformation|GetWorldLocation (Variables|Default|GetEjectionPoint)) (Transformation|GetWorldLocation (Variables|Default|GetEjectionDirection))) 0.1) "-2.000000,-2.000000,-2.000000") "None" false)
        (goto _label))))
  (:Completed
    (Variables|Default|SetisShooting false)
    (if (<= (Variables|Default|GetBulletsInMagazine) 0)
      (Transformation|SetRelativeLocation (Variables|Default|Getmp18_bolt) (Math|Vector|MakeVector 0.0 12.0 0.0) false false)
      (Variables|Default|SetisBulletInChamber false))))

(event Input|EnhancedActionEvents|EnhancedInputActionIA_Shoot_Right
  (params (ActionValue :type Boolean) (ElapsedSeconds :type Float%20%28double-precision%29) (TriggeredSeconds :type Float%20%28double-precision%29) (InputAction :type Input%20Action%20Object%20Reference :default "/Game/VRTemplate/Input/Actions/IA_Shoot_Right.IA_Shoot_Right"))
  (bind _mp18_bullet_indicator (Variables|Default|Getmp18_bullet_indicator))
  (bind _mp18_bolt (Variables|Default|Getmp18_bolt))
  (bind _ejectionpoint (Variables|Default|GetEjectionPoint))
  (bind _relativerotation (Variables|/Script/Engine.SceneComponent|GetRelativeRotation _mp18_bullet_indicator))
  ;[1 1 1] Shooting
  (:Started
    ;;[1 0 0] Prevents the gun from shooting if:
    ;; - the user wants to shoot faster then the guns rate of fire
    ;; - there are no more bullets left in the magazine and in the chamber
    (if (Math|Boolean|ANDBoolean (Variables|Default|GetisBulletInChamber) (Variables|Default|GetisMagazineAttached) (> (Variables|Default|GetBulletsInMagazine) 0))
      (Variables|Default|SetisShooting true)
      ;;[1 1 1] Projectile spawning
      (bind _spawntransform (CallFunction|RandomBulletSpread (Variables|Default|GetMuzzleEnd) (Variables|Default|GetmaxSpread) :!label _label))
      (Game|SpawnActorfromClass "/Game/Blueprints/Ammo/MyProjectile.MyProjectile_C" _spawntransform "Undefined" self (Game|Player|GetPlayerPawn 0))
      (Components|Activation|Activate (Variables|Default|GetMuzzleFlash) true)
      (Development|PrintString "ShootLog: Shot fired")
      (bind _output_get (Variables|Default|SetBulletsInMagazine (- (Variables|Default|GetBulletsInMagazine) 1)))
      (if (> _output_get 12)
        (Transformation|SetRelativeRotation _mp18_bullet_indicator (Math|Rotator|MakeRotator (+ (.roll _relativerotation) 13.0) (.pitch _relativerotation) (.yaw _relativerotation)) false false))
      (if (and (> _output_get 0) (Variables|Default|GetisShooting))
        (Variables|Default|SetslideForward true)
        (Utilities|FlowControl|Delay 0.06)
        (Variables|Default|SetslideForward false)
        (Transformation|SetRelativeLocation _mp18_bolt (Math|Vector|MakeVector 0.0 12.0 0.0) false false)
        (Variables|Default|SetslideBack true)
        (Utilities|FlowControl|Delay 0.06)
        (Variables|Default|SetslideBack false)
        (Transformation|SetRelativeLocation _mp18_bolt (Math|Vector|MakeVector 0.0 0.0 0.0) false false)
        ;;[1 1 1] Cardridge case ejection
        (bind _returnvalue (Game|SpawnActorfromClass "/Game/Blueprints/Ammo/CartridgeCase_MP18.CartridgeCase_MP18_C" (Math|Transform|MakeTransform (Transformation|GetWorldLocation _ejectionpoint) (Transformation|GetWorldRotation _ejectionpoint)) "Undefined" 0 0))
        (Physics|SetSimulatePhysics (Variables|/Game/Blueprints/Ammo/CartridgeCase_MP18.CartridgeCase_MP18_C|Getmp18_cartridgeCase _returnvalue) true)
        (Physics|AddImpulse (Variables|/Game/Blueprints/Ammo/CartridgeCase_MP18.CartridgeCase_MP18_C|Getmp18_cartridgeCase _returnvalue) (* (Math|Vector|Normalize (- (Transformation|GetWorldLocation (Variables|Default|GetEjectionPoint)) (Transformation|GetWorldLocation (Variables|Default|GetEjectionDirection))) 0.1) "-2.000000,-2.000000,-2.000000") "None" false)
        (goto _label))))
  (:Completed
    (Variables|Default|SetisShooting false)
    (if (<= (Variables|Default|GetBulletsInMagazine) 0)
      (Transformation|SetRelativeLocation (Variables|Default|Getmp18_bolt) (Math|Vector|MakeVector 0.0 12.0 0.0) false false)
      (Variables|Default|SetisBulletInChamber false))))

(event Collision|EventActorBeginOverlap
  (params (OtherActor :type Actor%20Object%20Reference))
  ;[1 1 1] Reloading - Attaching magazine to gun
  (if (== (Utilities|GetClass OtherActor) "/Game/Blueprints/Ammo/Magazine_MP18.Magazine_MP18_C")
    (if (not (Variables|Default|GetisMagazineAttached))
      (bind _asmagazine_mp18 (Utilities|Casting|CastToMagazine_MP18 OtherActor))
      (bind _output_get (Variables|Default|SetMagazineActor _asmagazine_mp18))
      (Variables|Default|SetBulletsInMagazine (Variables|/Game/Blueprints/Ammo/Magazine_MP18.Magazine_MP18_C|GetBulletsInMagazine _output_get))
      (Transformation|SetRelativeRotation (Variables|Default|Getmp18_bullet_indicator) (Variables|/Script/Engine.SceneComponent|GetRelativeRotation (Variables|/Game/Blueprints/Ammo/Magazine_MP18.Magazine_MP18_C|Getmp18_bullet_indicator _output_get)) false false)
      (Actor|DestroyActor OtherActor)
      (Development|SetHiddeninGame (Variables|Default|Getmp18_mag) false true)
      (Variables|Default|SetisMagazineAttached true))))

(event EventTick
  (params (DeltaSeconds :type Float%20%28single-precision%29))
  (bind _maingripcontroller (Variables|Default|GetMainGripController))
  (bind _secondarygripcontroller (Variables|Default|GetSecondaryGripController))
  (bind _mp18_bolt (Variables|Default|Getmp18_bolt))
  (bind _mp18_bolt_2 (Variables|Default|Getmp18_bolt))
  (bind _mp18_bolt_3 (Variables|Default|Getmp18_bolt))
  (bind _mp18_bolt_4 (Variables|Default|Getmp18_bolt))
  (bind _mp18_bolt_5 (Variables|Default|Getmp18_bolt))
  (bind _boltspeed (Variables|Default|GetboltSpeed))
  (bind _returnvalue (Transformation|GetWorldLocation _maingripcontroller))
  (bind _returnvalue_2 (Transformation|GetWorldLocation _secondarygripcontroller))
  (bind _relativelocation (Variables|/Script/Engine.SceneComponent|GetRelativeLocation _mp18_bolt_3))
  (bind _relativelocation_2 (Variables|/Script/Engine.SceneComponent|GetRelativeLocation _mp18_bolt_4))
  (bind _relativelocation_3 (Variables|/Script/Engine.SceneComponent|GetRelativeLocation _mp18_bolt_5))
  (bind _returnvalue_3 (Math|Rotator|FindLookatRotation _returnvalue _returnvalue_2))
  (if (and (Utilities|IsValid (Variables|Default|GetMainGripController)) (Utilities|IsValid (Variables|Default|GetSecondaryGripController))) ; Checks if the player grabbed with both hands
    ;[1 1 1] Two handed grab rotating
    (Transformation|SetWorldRotation (Variables|Default|GetGripPoint) (Math|Rotator|MakeRotator 0.0 (+ (.pitch _returnvalue_3) 45.0) (.yaw _returnvalue_3)) false false)
    (else
      ;[1 1 1] Bolt sliding back "animation"
      (if (Variables|Default|GetslideBack)
        (if (> (.y _relativelocation_2) 0.0)
          (Transformation|SetRelativeLocation (Variables|Default|Getmp18_bolt) (Math|Vector|MakeVector 0.0 (- (.y _relativelocation_2) _boltspeed) 0.0) false false)
          (else
            (Variables|Default|SetslideBack false)
            (Transformation|SetRelativeLocation (Variables|Default|Getmp18_bolt) (Math|Vector|MakeVector 0.0 0.0 0.0) false false)))
        (else
          ;[1 1 1] Bolt sliding forward "animation"
          (if (Variables|Default|GetslideForward)
            (if (< (.y _relativelocation_3) 12.0)
              (Transformation|SetRelativeLocation (Variables|Default|Getmp18_bolt) (Math|Vector|MakeVector 0.0 (+ (.y _relativelocation_3) _boltspeed) 0.0) false false)
              (else
                (Variables|Default|SetslideForward false)
                (Transformation|SetRelativeLocation (Variables|Default|Getmp18_bolt) (Math|Vector|MakeVector 0.0 12.0 0.0) false false)))
            (elif (not (Variables|Default|GetisShooting))
              ;[1 1 1] Charging handle grabbing
              (bind _charginghandlecontroller (Variables|Default|GetChargingHandleController)
                (:then
                  (Transformation|SetWorldLocation _mp18_bolt (Transformation|GetWorldLocation _charginghandlecontroller) false false)
                  (Transformation|SetRelativeLocation _mp18_bolt (Math|Vector|MakeVector 0.0 (- (.y (Variables|/Script/Engine.SceneComponent|GetRelativeLocation _mp18_bolt)) 13.0) 0.0) false false)
                  (if (< (.y _relativelocation) 0.0)
                    (Transformation|SetRelativeLocation _mp18_bolt_2 "0, 0, 0" false false)
                    (Variables|Default|SetisBulletInChamber (Variables|Default|GetisMagazineAttached))
                    (elif (> (.y _relativelocation) 12.0)
                      (Transformation|SetRelativeLocation _mp18_bolt_2 "0.000000,12.000000,0.000000" false false))))
                (:else)))))))))

(event EventRelease
  (params (MotionController :type Motion%20Controller%20Component%20Object%20Reference))
  (bind _returnvalue (Game|GetPlayerController 0))
  (bind _mp18_housing (Variables|Default|Getmp18_housing))
  (bind _secondarygripposition (Variables|Default|GetSecondaryGripPosition))
  (bind _returnvalue_2 (Transformation|GetWorldRotation _mp18_housing))
  (bind _returnvalue_3 (Transformation|GetWorldTransform _secondarygripposition))
  (Utilities|FlowControl|Sequence
    (:then_0
      (if (== MotionController (Variables|Default|GetMainGripController))
        (Transformation|DetachFromComponent (Variables|Default|GetGripPoint) "KeepWorld" "KeepWorld" "KeepWorld" true)
        ;[1 1 1] Trigger removal
        (Input|DisableInput _returnvalue)
        (Input|RemoveMappingContext (PlayerController|LocalPlayerSubsystems|GetEnhancedInputLocalPlayerSubsystem _returnvalue) (select (== (Variables|/Script/HeadMountedDisplay.MotionControllerComponent|GetMotionSource (Variables|Default|GetMainGripController)) "Right") "/Game/VRTemplate/Input/IMC_Weapon_Right.IMC_Weapon_Right" "/Game/VRTemplate/Input/IMC_Weapon_Left.IMC_Weapon_Left") "(bIgnoreAllPressedKeysUntilRelease=True,bForceImmediately=False)")
        (Variables|Default|SetMainGripController 0)
        (Utilities|String|LogString "MyLog: Detached Main Grip Controller")
        (bind _secondarygripcontroller (Variables|Default|GetSecondaryGripController)
          (:then
            (Transformation|DetachFromComponent _mp18_housing "KeepWorld" "KeepWorld" "KeepWorld" true)
            (Transformation|SetWorldTransform (Variables|Default|GetGripPoint) (Math|Transform|MakeTransform (.location _returnvalue_3) (Math|Rotator|MakeRotator (+ (.roll (.rotation _returnvalue_3)) (- (.roll (Transformation|GetWorldRotation _secondarygripcontroller)) (.roll _returnvalue_2))) (+ (.pitch (.rotation _returnvalue_3)) (- (.pitch (Transformation|GetWorldRotation _secondarygripcontroller)) (.pitch _returnvalue_2))) (+ (.yaw (.rotation _returnvalue_3)) (- (.yaw (Transformation|GetWorldRotation _secondarygripcontroller)) (.yaw _returnvalue_2)))) (.scale _returnvalue_3)) false false)
            (Transformation|AttachComponentToComponent (Variables|Default|Getmp18_housing) (Variables|Default|GetGripPoint) "None" "KeepWorld" "KeepWorld" "KeepWorld" true)
            (bind _returnvalue_4 (Transformation|AttachComponentToComponent (Variables|Default|GetGripPoint) _secondarygripcontroller "None" "SnapToTarget" "SnapToTarget" "KeepRelative" true))
            (Variables|Default|SetisSecondaryControllerAttached _returnvalue_4))
          (:else))))
    (:then_1
      (if (== MotionController (Variables|Default|GetSecondaryGripController))
        (if (Variables|Default|GetisSecondaryControllerAttached)
          (Transformation|DetachFromComponent (Variables|Default|GetGripPoint) "KeepWorld" "KeepWorld" "KeepWorld" true)
          (Variables|Default|SetisSecondaryControllerAttached false)
          (Transformation|DetachFromComponent (Variables|Default|Getmp18_housing) "KeepWorld" "KeepWorld" "KeepWorld" true)
          (Transformation|SetWorldTransform (Variables|Default|GetGripPoint) (Transformation|GetWorldTransform (Variables|Default|GetMainGripPosition)) false false)
          (Transformation|AttachComponentToComponent (Variables|Default|Getmp18_housing) (Variables|Default|GetGripPoint) "None" "KeepWorld" "KeepWorld" "KeepWorld" true)
          (if (Utilities|IsValid (Variables|Default|GetMainGripController))
            (Transformation|AttachComponentToComponent (Variables|Default|GetGripPoint) (Variables|Default|GetMainGripController) "None" "SnapToTarget" "SnapToTarget" "SnapToTarget" true)))
        (Variables|Default|SetSecondaryGripController 0)
        (Utilities|String|LogString "MyLog: Released Secondary Grip Controller")
        (if (Utilities|Enum|Equal(Enum) (Utilities|GetObjectName MotionController) "MotionControllerRight")
          (Development|SetHiddeninGame (Variables|Default|GetSecondaryHandRight) true false)
          (Development|SetHiddeninGame (Variables|Default|GetRightHand) false false)
          (else
            (Development|SetHiddeninGame (Variables|Default|GetSecondaryHandLeft) true false)
            (Development|SetHiddeninGame (Variables|Default|GetLeftHand) false false)))
        (bind _maingripcontroller (Variables|Default|GetMainGripController)
          (:then
            (Transformation|SetWorldRotation (Variables|Default|GetGripPoint) (Transformation|GetWorldRotation _maingripcontroller) false false))
          (:else))
        (else
          ;[1 1 1] Reloading - Detaching magazine from hand
          (if (== MotionController (Variables|Default|GetMagazineGripController))
            (bind _magazineactor (Variables|Default|GetMagazineActor)
              (:then
                (Transformation|DetachFromActor _magazineactor "KeepWorld" "KeepWorld" "KeepWorld")
                (Variables|Default|SetMagazineGripController 0))
              (:else))
            (elif (== MotionController (Variables|Default|GetChargingHandleController))
              (Variables|Default|SetChargingHandleController 0))))))))

(event EventGrab
  (params (MotionController :type Motion%20Controller%20Component%20Object%20Reference))
  (bind _returnvalue (Game|GetPlayerController 0))
  (bind _charginghandlecollision (Variables|Default|GetChargingHandleCollision))
  (bind _magazinegripcollision (Variables|Default|GetMagazineGripCollision))
  (Utilities|String|LogString "MyLog: Grab started")
  (if (or (and (Utilities|Enum|Equal(Enum) (Utilities|GetObjectName MotionController) "MotionControllerRight") (Variables|Default|GetMainGrabbableRight)) (and (Utilities|Enum|Equal(Enum) (Utilities|GetObjectName MotionController) "MotionControllerLeft") (Variables|Default|GetMainGrabbableLeft)))
    (bind _output_get (Variables|Default|SetMainGripController MotionController))
    ;[1 1 1] Trigger assignment
    (Input|EnableInput _returnvalue)
    (bind _output_get_2 (Variables|Default|SetMappingContext (select (== (Variables|/Script/HeadMountedDisplay.MotionControllerComponent|GetMotionSource _output_get) "Right") "/Game/VRTemplate/Input/IMC_Weapon_Right.IMC_Weapon_Right" "/Game/VRTemplate/Input/IMC_Weapon_Left.IMC_Weapon_Left")))
    (Input|AddMappingContext (PlayerController|LocalPlayerSubsystems|GetEnhancedInputLocalPlayerSubsystem _returnvalue) _output_get_2 0 "(bIgnoreAllPressedKeysUntilRelease=True,bForceImmediately=False)")
    (Variables|Default|GetSecondaryGripController
      (:then
        (Transformation|DetachFromComponent (Variables|Default|GetGripPoint) "KeepWorld" "KeepWorld" "KeepWorld" true)
        (Transformation|DetachFromComponent (Variables|Default|Getmp18_housing) "KeepWorld" "KeepWorld" "KeepWorld" true)
        (Transformation|SetWorldTransform (Variables|Default|GetGripPoint) (Transformation|GetWorldTransform (Variables|Default|GetMainGripPosition)) false false)
        (Transformation|AttachComponentToComponent (Variables|Default|Getmp18_housing) (Variables|Default|GetGripPoint) "None" "KeepWorld" "KeepWorld" "KeepWorld" true))
      (:else
        _))
    (Transformation|AttachComponentToComponent (Variables|Default|GetGripPoint) _output_get "None" "SnapToTarget" "SnapToTarget" "KeepRelative" true)
    (Development|PrintString "MyLog: Attached Main Grip Controller" false)
    (Utilities|FlowControl|DelayUntilNextTick)
    (Utilities|FlowControl|DelayUntilNextTick)
    (if (Utilities|Enum|Equal(Enum) (Utilities|GetObjectName _output_get) "MotionControllerRight")
      (Variables|/Game/Characters/MannequinsXR/Meshes/SK_MannequinsXR_AnimBlueprint.SK_MannequinsXR_AnimBlueprint_C|SetBlendSpaceEnum (Variables|Default|GetRightHandAnim) "NewEnumerator10")
      (else
        (Variables|/Game/Characters/MannequinsXR/Meshes/SK_MannequinsXR_AnimBlueprint.SK_MannequinsXR_AnimBlueprint_C|SetBlendSpaceEnum (Variables|Default|GetLeftHandAnim) "NewEnumerator10")))
    (elif (or (and (Utilities|Enum|Equal(Enum) (Utilities|GetObjectName MotionController) "MotionControllerRight") (Variables|Default|GetSecondaryGrabbableRight)) (and (Utilities|Enum|Equal(Enum) (Utilities|GetObjectName MotionController) "MotionControllerLeft") (Variables|Default|GetSecondaryGrabbableLeft)))
      (Variables|Default|SetSecondaryGripController MotionController)
      (Utilities|String|LogString "MyLog: Set Secondary Grip Controller")
      (if (Utilities|Enum|Equal(Enum) (Utilities|GetObjectName MotionController) "MotionControllerRight")
        (Development|SetHiddeninGame (Variables|Default|GetSecondaryHandRight) false false)
        (Development|SetHiddeninGame (Variables|Default|GetRightHand) true false)
        (else
          (Development|SetHiddeninGame (Variables|Default|GetSecondaryHandLeft) false false)
          (Development|SetHiddeninGame (Variables|Default|GetLeftHand) true false)))
      (if (not (Utilities|IsValid (Variables|Default|GetMainGripController)))
        (Transformation|AttachComponentToComponent (Variables|Default|GetGripPoint) (Variables|Default|GetSecondaryGripController) "None" "KeepWorld" "KeepWorld" "KeepWorld" true)
        (Variables|Default|SetisSecondaryControllerAttached true))
      (else
        ;[1 1 1] Reloading - Detaching magazine from gun
        (if (<= (Math|Vector|Distance(Vector) (Transformation|GetWorldLocation MotionController) (Transformation|GetWorldLocation _magazinegripcollision)) (Variables|/Script/Engine.SphereComponent|GetSphereRadius _magazinegripcollision))
          (bind _output_get_3 (Variables|Default|SetMagazineGripController MotionController))
          (if (Variables|Default|GetisMagazineAttached)
            (Development|SetHiddeninGame (Variables|Default|Getmp18_mag) true true)
            (bind _returnvalue_2 (Game|SpawnActorfromClass "/Game/Blueprints/Ammo/Magazine_MP18.Magazine_MP18_C" (Transformation|GetWorldTransform (Variables|Default|Getmp18_mag)) "Undefined" 0 0))
            (bind _output_get_4 (Variables|Default|SetMagazineActor _returnvalue_2))
            (bind _output_get_5 (Variables|/Game/Blueprints/Ammo/Magazine_MP18.Magazine_MP18_C|SetBulletsInMagazine _output_get_4 (Variables|Default|GetBulletsInMagazine)))
            (if (<= _output_get_5 0)
              (Development|SetHiddeninGame (Variables|/Game/Blueprints/Ammo/Magazine_MP18.Magazine_MP18_C|Getmp18_bullet _output_get_4) true false))
            (Transformation|SetRelativeRotation (Variables|/Game/Blueprints/Ammo/Magazine_MP18.Magazine_MP18_C|Getmp18_bullet_indicator _output_get_4) (Variables|/Script/Engine.SceneComponent|GetRelativeRotation (Variables|Default|Getmp18_bullet_indicator)) false false)
            (if (Utilities|Enum|Equal(Enum) (Utilities|GetObjectName _output_get_3) "MotionControllerRight")
              (Variables|/Game/Characters/MannequinsXR/Meshes/SK_MannequinsXR_AnimBlueprint.SK_MannequinsXR_AnimBlueprint_C|SetBlendSpaceEnum (Variables|Default|GetRightHandAnim) "NewEnumerator8")
              (Transformation|AttachComponentToComponent (Variables|/Script/Engine.Actor|GetRootComponent _output_get_4) (Variables|Default|GetRightHand) "allFingerFistGrabThumbOpenSocket" "SnapToTarget" "SnapToTarget" "SnapToTarget" true)
              (else
                (Variables|/Game/Characters/MannequinsXR/Meshes/SK_MannequinsXR_AnimBlueprint.SK_MannequinsXR_AnimBlueprint_C|SetBlendSpaceEnum (Variables|Default|GetLeftHandAnim) "NewEnumerator8")
                (Transformation|AttachComponentToComponent (Variables|/Script/Engine.Actor|GetRootComponent _output_get_4) (Variables|Default|GetLeftHand) "allFingerFistGrabThumbOpenSocket" "SnapToTarget" "SnapToTarget" "SnapToTarget" true)
                (Transformation|SetWorldScale3D (Variables|/Script/Engine.Actor|GetRootComponent _output_get_4) "1.000000,1.000000,1.000000")
                (Transformation|SetRelativeRotation (Variables|/Script/Engine.Actor|GetRootComponent _output_get_4) (Math|Rotator|MakeRotator (.roll (Variables|/Script/Engine.SceneComponent|GetRelativeRotation (Variables|/Script/Engine.Actor|GetRootComponent _output_get_4))) (.pitch (Variables|/Script/Engine.SceneComponent|GetRelativeRotation (Variables|/Script/Engine.Actor|GetRootComponent _output_get_4))) (- (.yaw (Variables|/Script/Engine.SceneComponent|GetRelativeRotation (Variables|/Script/Engine.Actor|GetRootComponent _output_get_4))) 45.0)) false false)
                (Transformation|SetRelativeLocation (Variables|/Script/Engine.Actor|GetRootComponent _output_get_4) (Math|Vector|MakeVector (.x (Variables|/Script/Engine.SceneComponent|GetRelativeLocation (Variables|/Script/Engine.Actor|GetRootComponent _output_get_4))) (+ (.y (Variables|/Script/Engine.SceneComponent|GetRelativeLocation (Variables|/Script/Engine.Actor|GetRootComponent _output_get_4))) 2.0) (.z (Variables|/Script/Engine.SceneComponent|GetRelativeLocation (Variables|/Script/Engine.Actor|GetRootComponent _output_get_4)))) false false)))
            (Variables|Default|SetisMagazineAttached false))
          (elif (<= (Math|Vector|Distance(Vector) (Transformation|GetWorldLocation MotionController) (Transformation|GetWorldLocation _charginghandlecollision)) (Variables|/Script/Engine.SphereComponent|GetSphereRadius _charginghandlecollision))
            (Variables|Default|SetChargingHandleController MotionController)
            (if (Utilities|Enum|Equal(Enum) (Utilities|GetObjectName MotionController) "MotionControllerRight")
              (Variables|/Game/Characters/MannequinsXR/Meshes/SK_MannequinsXR_AnimBlueprint.SK_MannequinsXR_AnimBlueprint_C|SetBlendSpaceEnum (Variables|Default|GetRightHandAnim) "NewEnumerator3")
              (else
                (Variables|/Game/Characters/MannequinsXR/Meshes/SK_MannequinsXR_AnimBlueprint.SK_MannequinsXR_AnimBlueprint_C|SetBlendSpaceEnum (Variables|Default|GetLeftHandAnim) "NewEnumerator3")))))))))

(event EventBeginPlay
  (bind _returnvalue (Game|Player|GetPlayerPawn 0))
  (bind _output_get (Variables|Default|SetLeftHand (Utilities|Array|Get(acopy) (Actor|GetComponentsbyTag _returnvalue "/Script/Engine.SkeletalMeshComponent" "HandLeft"))))
  (bind _output_get_2 (Variables|Default|SetRightHand (Utilities|Array|Get(acopy) (Actor|GetComponentsbyTag _returnvalue "/Script/Engine.SkeletalMeshComponent" "HandRight"))))
  (bind _assk_mannequins_xr_anim_blueprint (Utilities|Casting|CastToSK_MannequinsXR_AnimBlueprint (Components|SkeletalMesh|GetAnimInstance _output_get)))
  (Variables|Default|SetLeftHandAnim _assk_mannequins_xr_anim_blueprint)
  (bind _assk_mannequins_xr_anim_blueprint_2 (Utilities|Casting|CastToSK_MannequinsXR_AnimBlueprint (Components|SkeletalMesh|GetAnimInstance _output_get_2)))
  (Variables|Default|SetRightHandAnim _assk_mannequins_xr_anim_blueprint_2))

(fn ConstructionScript)

(fn RandomBulletSpread
  (params (spawnPoint :type Arrow%20Component%20Object%20Reference) (maxSpread :type Float%20%28double-precision%29))
  (bind _returnvalue (Transformation|GetWorldRotation spawnPoint))
  ;[1 1 1] Random bullet spread
  (if (Variables|Default|GetisSecondaryControllerAttached)
    (LocalVariables|Setspread (/ maxSpread (LocalVariables|GetspreadDivider)))
    (else
      (LocalVariables|Setspread maxSpread)))
  (return (Math|Transform|MakeTransform (Transformation|GetWorldLocation spawnPoint) (Math|Rotator|MakeRotator (+ (.roll _returnvalue) (Math|Random|RandomFloatinRange (* (LocalVariables|Getspread) -1.0) (LocalVariables|Getspread))) (+ (.pitch _returnvalue) (Math|Random|RandomFloatinRange (* (LocalVariables|Getspread) -1.0) (LocalVariables|Getspread))) (+ (.yaw _returnvalue) (Math|Random|RandomFloatinRange (* (LocalVariables|Getspread) -1.0) (LocalVariables|Getspread)))) (Transformation|GetWorldScale spawnPoint))))