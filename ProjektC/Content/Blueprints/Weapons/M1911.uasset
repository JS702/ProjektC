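; VR M1911 pistol that the player grips, fires and reloads by hand using motion controllers.
; Grab and Release route controllers to grip, magazine or slide, swapping hand poses and input mappings; a dropped gun can return to a body holster after a delay.
; Magazine actors carry the round count in and out, while pulling the slide chambers or ejects rounds.
; Shots spawn projectiles with rapid-fire spread, and Tick animates the slide and ejects casings.
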(event OnComponentBeginOverlap(SledGripCollision)
  (params (OverlappedComponent :type Primitive%20Component%20Object%20Reference) (OtherActor :type Actor%20Object%20Reference) (OtherComp :type Primitive%20Component%20Object%20Reference) (OtherBodyIndex :type Integer) (bFromSweep :type Boolean) (SweepResult :type Hit%20Result%20Structure%20%28by%20ref%29))
  (bind _returnvalue (Utilities|GetObjectName OtherComp))
  (if (Utilities|Enum|Equal(Enum) _returnvalue "HandCollisionLeft")
    (Variables|Default|SetsledGrabbableLeft true)
    (elif (Utilities|Enum|Equal(Enum) _returnvalue "HandCollisionRight")
      (Variables|Default|SetsledGrabbableRight true))))

(event OnComponentBeginOverlap(ReloadZone)
  (params (OverlappedComponent :type Primitive%20Component%20Object%20Reference) (OtherActor :type Actor%20Object%20Reference) (OtherComp :type Primitive%20Component%20Object%20Reference) (OtherBodyIndex :type Integer) (bFromSweep :type Boolean) (SweepResult :type Hit%20Result%20Structure%20%28by%20ref%29))
  ;[1 1 1] Reloading - Attaching magazine to gun
  (if (not (Variables|Default|GetjustRemovedMagazine))
    (if (== (Utilities|GetClass OtherActor) "/Game/Blueprints/Ammo/Magazine_M1911.Magazine_M1911_C")
      (if (not (Variables|Default|GetisMagazineAttached))
        (bind _asmagazine_m1911 (Utilities|Casting|CastToMagazine_M1911 OtherActor))
        (bind _output_get (Variables|Default|SetMagazineActor _asmagazine_m1911))
        (Variables|Default|SetBulletsInMagazine (Variables|/Game/Blueprints/Ammo/Magazine_M1911.Magazine_M1911_C|GetBulletsInMagazine _output_get))
        (Actor|DestroyActor OtherActor)
        (Development|SetHiddeninGame (Variables|Default|Getm1911_magazine) false false)
        (Variables|Default|SetisMagazineAttached true)
        (Audio|PlaySoundatLocation "/Game/Sounds/Weapons/M1911/M1911_magazineAttached.M1911_magazineAttached" (Transformation|GetWorldLocation (Variables|Default|Getm1911_magazine)) "0, 0, 0" 1.0 1.0 0.0 0 0 0 0)))))

(event OnComponentEndOverlap(SledGripCollision)
  (params (OverlappedComponent :type Primitive%20Component%20Object%20Reference) (OtherActor :type Actor%20Object%20Reference) (OtherComp :type Primitive%20Component%20Object%20Reference) (OtherBodyIndex :type Integer))
  (bind _returnvalue (Utilities|GetObjectName OtherComp))
  (if (Utilities|Enum|Equal(Enum) _returnvalue "HandCollisionLeft")
    (Variables|Default|SetsledGrabbableLeft false)
    (elif (Utilities|Enum|Equal(Enum) _returnvalue "HandCollisionRight")
      (Variables|Default|SetsledGrabbableRight false))))

(event OnComponentBeginOverlap(MainGripCollision)
  (params (OverlappedComponent :type Primitive%20Component%20Object%20Reference) (OtherActor :type Actor%20Object%20Reference) (OtherComp :type Primitive%20Component%20Object%20Reference) (OtherBodyIndex :type Integer) (bFromSweep :type Boolean) (SweepResult :type Hit%20Result%20Structure%20%28by%20ref%29))
  (bind _returnvalue (Utilities|GetObjectName OtherComp))
  (if (Utilities|Enum|Equal(Enum) _returnvalue "HandCollisionLeft")
    (Variables|Default|SetMainGrabbableLeft true)
    (elif (Utilities|Enum|Equal(Enum) _returnvalue "HandCollisionRight")
      (Variables|Default|SetMainGrabbableRight true))))

(event OnComponentEndOverlap(MainGripCollision)
  (params (OverlappedComponent :type Primitive%20Component%20Object%20Reference) (OtherActor :type Actor%20Object%20Reference) (OtherComp :type Primitive%20Component%20Object%20Reference) (OtherBodyIndex :type Integer))
  (bind _returnvalue (Utilities|GetObjectName OtherComp))
  (if (Utilities|Enum|Equal(Enum) _returnvalue "HandCollisionLeft")
    (Variables|Default|SetMainGrabbableLeft false)
    (elif (Utilities|Enum|Equal(Enum) _returnvalue "HandCollisionRight")
      (Variables|Default|SetMainGrabbableRight false))))

(event Input|EnhancedActionEvents|EnhancedInputActionIA_Shoot_Left
  (params (ActionValue :type Boolean) (ElapsedSeconds :type Float%20%28double-precision%29) (TriggeredSeconds :type Float%20%28double-precision%29) (InputAction :type Input%20Action%20Object%20Reference :default "/Game/VRTemplate/Input/Actions/IA_Shoot_Left.IA_Shoot_Left"))
  ;[1 1 1] Shooting
  (:Started
    (Utilities|Time|SetTimerbyFunctionName 0 "spreadHandler" 1.0)
    ;;[1 0 0] Prevents the gun from shooting if:
    ;; - the user wants to shoot faster then the guns rate of fire
    ;; - there are no more bullets left in the magazine and in the chamber
    (if (and (Variables|Default|GetisShootable) (Variables|Default|GetisBulletInChamber))
      (if (Variables|Default|GetisMagazineAttached)
        (if (> (Variables|Default|GetBulletsInMagazine) 0)
          (Variables|Default|SetBulletsInMagazine (- (Variables|Default|GetBulletsInMagazine) 1))
          (else
            (Variables|Default|SetisBulletInChamber false :!label _label)))
        (else
          (goto _label)))
      (Audio|PlaySoundatLocation "/Game/Sounds/Weapons/M1911/M1911_shot.M1911_shot" (Transformation|GetWorldLocation (Variables|Default|GetMuzzleEnd)) "0, 0, 0" 1.0 1.0 0.0 0 0 0 0)
      ;;[1 1 1] Projectile spawning
      (if (not (Variables|Default|GetshouldSpread))
        (Variables|Default|SetbulletSpawnTransform (Transformation|GetWorldTransform (Variables|Default|GetMuzzleEnd)))
        (else
          (bind _spawntransform (CallFunction|RandomBulletSpread (Variables|Default|GetMuzzleEnd) (Variables|Default|GetmaxSpread)))
          (Variables|Default|SetbulletSpawnTransform _spawntransform)))
      (bind _returnvalue (Game|SpawnActorfromClass "/Game/Blueprints/Ammo/MyProjectile.MyProjectile_C" (Variables|Default|GetbulletSpawnTransform) "Undefined" self (Game|Player|GetPlayerPawn 0)))
      (Variables|/Game/Blueprints/Ammo/MyProjectile.MyProjectile_C|Setdamage _returnvalue (Variables|Default|Getdamage))
      (Components|Activation|Activate (Variables|Default|GetMuzzleFlash) true)
      (Development|PrintString "ShootLog: Shot fired" false)
      (Variables|Default|SetshouldSpread true)
      ;;[1 1 1] Rate of fire delay + "animation" management
      (Variables|Default|SetslideBack true)
      (Variables|Default|SetejectCardrigeCase true)
      (Variables|Default|SetisShootable false)
      (Utilities|FlowControl|Delay 0.13)
      (Variables|Default|SetslideForward true)
      (Utilities|FlowControl|Delay 0.13)
      (Variables|Default|SetisShootable true))))

(event Input|EnhancedActionEvents|EnhancedInputActionIA_Shoot_Right
  (params (ActionValue :type Boolean) (ElapsedSeconds :type Float%20%28double-precision%29) (TriggeredSeconds :type Float%20%28double-precision%29) (InputAction :type Input%20Action%20Object%20Reference :default "/Game/VRTemplate/Input/Actions/IA_Shoot_Right.IA_Shoot_Right"))
  ;[1 1 1] Shooting
  (:Started
    (Utilities|Time|SetTimerbyFunctionName 0 "spreadHandler" 1.0)
    ;;[1 0 0] Prevents the gun from shooting if:
    ;; - the user wants to shoot faster then the guns rate of fire
    ;; - there are no more bullets left in the magazine and in the chamber
    (if (and (Variables|Default|GetisShootable) (Variables|Default|GetisBulletInChamber))
      (if (Variables|Default|GetisMagazineAttached)
        (if (> (Variables|Default|GetBulletsInMagazine) 0)
          (Variables|Default|SetBulletsInMagazine (- (Variables|Default|GetBulletsInMagazine) 1))
          (else
            (Variables|Default|SetisBulletInChamber false :!label _label)))
        (else
          (goto _label)))
      (Audio|PlaySoundatLocation "/Game/Sounds/Weapons/M1911/M1911_shot.M1911_shot" (Transformation|GetWorldLocation (Variables|Default|GetMuzzleEnd)) "0, 0, 0" 1.0 1.0 0.0 0 0 0 0)
      ;;[1 1 1] Projectile spawning
      (if (not (Variables|Default|GetshouldSpread))
        (Variables|Default|SetbulletSpawnTransform (Transformation|GetWorldTransform (Variables|Default|GetMuzzleEnd)))
        (else
          (bind _spawntransform (CallFunction|RandomBulletSpread (Variables|Default|GetMuzzleEnd) (Variables|Default|GetmaxSpread)))
          (Variables|Default|SetbulletSpawnTransform _spawntransform)))
      (bind _returnvalue (Game|SpawnActorfromClass "/Game/Blueprints/Ammo/MyProjectile.MyProjectile_C" (Variables|Default|GetbulletSpawnTransform) "Undefined" self (Game|Player|GetPlayerPawn 0)))
      (Variables|/Game/Blueprints/Ammo/MyProjectile.MyProjectile_C|Setdamage _returnvalue (Variables|Default|Getdamage))
      (Components|Activation|Activate (Variables|Default|GetMuzzleFlash) true)
      (Development|PrintString "ShootLog: Shot fired" false)
      (Variables|Default|SetshouldSpread true)
      ;;[1 1 1] Rate of fire delay + "animation" management
      (Variables|Default|SetslideBack true)
      (Variables|Default|SetejectCardrigeCase true)
      (Variables|Default|SetisShootable false)
      (Utilities|FlowControl|Delay 0.13)
      (Variables|Default|SetslideForward true)
      (Utilities|FlowControl|Delay 0.13)
      (Variables|Default|SetisShootable true))))

(event EventTick
  (params (DeltaSeconds :type Float%20%28single-precision%29))
  (bind _m1911_sled (Variables|Default|Getm1911_sled))
  (bind _m1911_sled_2 (Variables|Default|Getm1911_sled))
  (bind _m1911_sled_3 (Variables|Default|Getm1911_sled))
  (bind _m1911_sled_4 (Variables|Default|Getm1911_sled))
  (bind _ejectionpoint (Variables|Default|GetEjectionPoint))
  (bind _m1911_sled_5 (Variables|Default|Getm1911_sled))
  (bind _sledspeed (Variables|Default|GetsledSpeed))
  (bind _ejectionpoint_2 (Variables|Default|GetEjectionPoint))
  (bind _relativelocation (Variables|/Script/Engine.SceneComponent|GetRelativeLocation _m1911_sled_2))
  (bind _relativelocation_2 (Variables|/Script/Engine.SceneComponent|GetRelativeLocation _m1911_sled_3))
  (bind _relativelocation_3 (Variables|/Script/Engine.SceneComponent|GetRelativeLocation _m1911_sled_5))
  (Utilities|FlowControl|Sequence
    (:then_0
      ;[1 1 1] Bolt sliding back "animation"
      (if (Variables|Default|GetslideBack)
        (if (> (.y _relativelocation_2) -4.0)
          (Transformation|SetRelativeLocation (Variables|Default|Getm1911_sled) (Math|Vector|MakeVector 0.0 (- (.y _relativelocation_2) _sledspeed) 0.0) false false)
          (else
            (Variables|Default|SetslideBack false)
            (Transformation|SetRelativeLocation (Variables|Default|Getm1911_sled) (Math|Vector|MakeVector 0.0 -4.0 0.0) false false)
            ;[1 1 1] Eject cartride case after shot is fired
            (if (Variables|Default|GetejectCardrigeCase)
              (Variables|Default|SetejectCardrigeCase false)
              (bind _returnvalue (Game|SpawnActorfromClass "/Game/Blueprints/Ammo/CartridgeCase_M1911.CartridgeCase_M1911_C" (Math|Transform|MakeTransform (Transformation|GetWorldLocation _ejectionpoint_2) (Transformation|GetWorldRotation _ejectionpoint_2)) "Undefined" 0 0))
              (Physics|SetSimulatePhysics (Variables|/Game/Blueprints/Ammo/CartridgeCase_M1911.CartridgeCase_M1911_C|Getm1911_cartdrige_case _returnvalue) true)
              (Physics|AddImpulse (Variables|/Game/Blueprints/Ammo/CartridgeCase_M1911.CartridgeCase_M1911_C|Getm1911_cartdrige_case _returnvalue) (* (Math|Vector|Normalize (- (Transformation|GetWorldLocation (Variables|Default|GetEjectionPoint)) (Transformation|GetWorldLocation (Variables|Default|GetEjectionDirection))) 0.1) "-2.000000,-2.000000,-2.000000") "None" false))))))
    (:then_1
      ;[1 1 1] Bolt sliding forward "animation"
      (if (Variables|Default|GetslideForward)
        (if (< (.y _relativelocation_3) 0.0)
          (Transformation|SetRelativeLocation (Variables|Default|Getm1911_sled) (Math|Vector|MakeVector 0.0 (+ (.y _relativelocation_3) _sledspeed) 0.0) false false)
          (else
            (Variables|Default|SetslideForward false)
            (Transformation|SetRelativeLocation (Variables|Default|Getm1911_sled) (Math|Vector|MakeVector 0.0 0.0 0.0) false false)))))
    (:then_2
      ;[1 1 1] Empty reload - put bullet in chamber
      (if (Utilities|IsValid (Variables|Default|GetSledController))
        (Transformation|SetWorldLocation _m1911_sled (Transformation|GetWorldLocation (Variables|Default|GetSledController)) false false)
        (Transformation|SetRelativeLocation _m1911_sled (Math|Vector|MakeVector 0.0 (.y (Variables|/Script/Engine.SceneComponent|GetRelativeLocation _m1911_sled)) 0.0) false false)
        (if (>= (.y _relativelocation) 0.0)
          (Transformation|SetRelativeLocation _m1911_sled_4 (Math|Vector|MakeVector 0.0 0.0 0.0) false false)
          (elif (<= (.y _relativelocation) -4.0)
            (Transformation|SetRelativeLocation _m1911_sled_4 (Math|Vector|MakeVector 0.0 -4.0 0.0) false false)
            (Variables|Default|SetSledController 0)
            (Audio|PlaySoundatLocation "/Game/Sounds/Weapons/M1911/M1911_sled.M1911_sled" (Transformation|GetWorldLocation (Variables|Default|Getm1911_magazine)) "0, 0, 0" 1.0 1.0 0.0 0 0 0 0)
            (if (Utilities|Enum|Equal(Enum) (Utilities|GetObjectName (stale EventRelease MotionController)) "MotionControllerRight")
              (Development|SetHiddeninGame (Variables|Default|GetSledHandRight) true false)
              (Development|SetHiddeninGame (Variables|Default|GetRightHand) false false)
              (else
                (Development|SetHiddeninGame (Variables|Default|GetSledHandLeft) true false)
                (Development|SetHiddeninGame (Variables|Default|GetLeftHand) false false)))
            (if (and (Variables|Default|GetisMagazineAttached) (> (Variables|Default|GetBulletsInMagazine) 0))
              (if (Variables|Default|GetisBulletInChamber)
                ;[1 1 1] Eject bullet
                (bind _returnvalue_2 (Game|SpawnActorfromClass "/Game/Blueprints/Ammo/Bullet_M1911.Bullet_M1911_C" (Math|Transform|MakeTransform (Transformation|GetWorldLocation _ejectionpoint) (Transformation|GetWorldRotation _ejectionpoint)) "Undefined" 0 0))
                (Physics|SetSimulatePhysics (Variables|/Game/Blueprints/Ammo/Bullet_M1911.Bullet_M1911_C|Getm1911_bullet _returnvalue_2) true)
                (Physics|AddImpulse (Variables|/Game/Blueprints/Ammo/Bullet_M1911.Bullet_M1911_C|Getm1911_bullet _returnvalue_2) (* (Math|Vector|Normalize (- (Transformation|GetWorldLocation (Variables|Default|GetEjectionPoint)) (Transformation|GetWorldLocation (Variables|Default|GetEjectionDirection))) 0.1) "-2.000000,-2.000000,-2.000000") "None" false)
                (Audio|PlaySoundatLocation "/Game/Sounds/Weapons/Bullet_ejecting.Bullet_ejecting" (Transformation|GetWorldLocation (Variables|Default|Getm1911_sled)) "0, 0, 0" 1.0 1.0 0.0 0 0 0 0)
                (else
                  (Variables|Default|SetisBulletInChamber true)))
              (Variables|Default|SetBulletsInMagazine (- (Variables|Default|GetBulletsInMagazine) 1)))
            (Variables|Default|SetslideForward true)))))))

(event EventRelease
  (params (MotionController :type Motion%20Controller%20Component%20Object%20Reference))
  (bind _returnvalue (Game|GetPlayerController 0))
  (bind _magazineactor (Variables|Default|GetMagazineActor))
  (Utilities|FlowControl|Sequence
    (:then_0
      (if (== MotionController (Variables|Default|GetMainGripController))
        (Transformation|DetachFromComponent (Variables|Default|GetGripPoint) "KeepWorld" "KeepWorld" "KeepWorld" true)
        ;[1 1 1] Trigger removal
        (Input|DisableInput _returnvalue)
        (Input|RemoveMappingContext (PlayerController|LocalPlayerSubsystems|GetEnhancedInputLocalPlayerSubsystem _returnvalue) (select (== (Variables|/Script/HeadMountedDisplay.MotionControllerComponent|GetMotionSource (Variables|Default|GetMainGripController)) "Right") "/Game/VRTemplate/Input/IMC_Weapon_Right.IMC_Weapon_Right" "/Game/VRTemplate/Input/IMC_Weapon_Left.IMC_Weapon_Left") "(bIgnoreAllPressedKeysUntilRelease=True,bForceImmediately=False)")
        (Variables|Default|SetMainGripController 0)
        (Utilities|String|LogString "MyLog: Detached Main Grip Controller")
        (if (Variables|Default|GetbelongsToBody)
          (bind _returnvalue_2 (Utilities|Time|SetTimerbyFunctionName 0 "attachToBody" 5.0))
          (Variables|Default|SettimerHandle _returnvalue_2)
          (if (not (Utilities|IsValid (Variables|Default|GetMainGripController)))
            (if (Utilities|Enum|Equal(Enum) (Utilities|GetObjectName (Variables|Default|GetSledController)) "MotionControllerRight")
              (Development|SetHiddeninGame (Variables|Default|GetSledHandRight) true false)
              (Development|SetHiddeninGame (Variables|Default|GetRightHand) false false)
              (else
                (Development|SetHiddeninGame (Variables|Default|GetSledHandLeft) true false)
                (Development|SetHiddeninGame (Variables|Default|GetLeftHand) false false)))
            (Variables|Default|SetSledController 0)
            (Physics|SetSimulatePhysics (Variables|Default|Getm1911_housing) true)
            (Variables|Default|SetphysicsEnabled true)))))
    (:then_1
      ;[1 1 1] Reloading - Detaching magazine from hand
      (if (== MotionController (Variables|Default|GetMagazineGripController))
        (bind _magazineactor_2 (Variables|Default|GetMagazineActor)
          (:then
            (Transformation|DetachFromActor _magazineactor_2 "KeepWorld" "KeepWorld" "KeepWorld")
            (Variables|Default|SetMagazineGripController 0)
            (Physics|SetSimulatePhysics (Variables|/Game/Blueprints/Ammo/Magazine_M1911.Magazine_M1911_C|Getm1911_magazine _magazineactor) true)
            (Variables|/Game/Blueprints/Ammo/Magazine_M1911.Magazine_M1911_C|SetphysicsEnabled _magazineactor true))
          (:else))
        (elif (== MotionController (Variables|Default|GetSledController))
          (Variables|Default|SetSledController 0)
          (if (Utilities|Enum|Equal(Enum) (Utilities|GetObjectName MotionController) "MotionControllerRight")
            (Development|SetHiddeninGame (Variables|Default|GetSledHandRight) true false)
            (Development|SetHiddeninGame (Variables|Default|GetRightHand) false false)
            (else
              (Development|SetHiddeninGame (Variables|Default|GetSledHandLeft) true false)
              (Development|SetHiddeninGame (Variables|Default|GetLeftHand) false false))))))))

(event EventGrab
  (params (MotionController :type Motion%20Controller%20Component%20Object%20Reference))
  (bind _returnvalue (Game|GetPlayerController 0))
  (bind _grippoint (Variables|Default|GetGripPoint))
  (bind _timerhandle (Variables|Default|GettimerHandle))
  (bind _magazinegripcollision (Variables|Default|GetMagazineGripCollision))
  (if (Variables|Default|GetphysicsEnabled)
    (Physics|SetSimulatePhysics (Variables|Default|Getm1911_housing) false)
    (Transformation|SetWorldTransform _grippoint (Transformation|GetWorldTransform (Variables|Default|GetMainGripPosition)) false false)
    (Transformation|AttachComponentToComponent (Variables|Default|Getm1911_housing) _grippoint "None" "KeepWorld" "KeepWorld" "KeepWorld" true)
    (Variables|Default|SetphysicsEnabled false))
  (if (or (and (Utilities|Enum|Equal(Enum) (Utilities|GetObjectName MotionController) "MotionControllerRight") (Variables|Default|GetMainGrabbableRight)) (and (Utilities|Enum|Equal(Enum) (Utilities|GetObjectName MotionController) "MotionControllerLeft") (Variables|Default|GetMainGrabbableLeft)))
    (bind _output_get (Variables|Default|SetMainGripController MotionController))
    ;[1 1 1] Trigger assignment
    (Input|EnableInput _returnvalue)
    (bind _output_get_2 (Variables|Default|SetMappingContext (select (== (Variables|/Script/HeadMountedDisplay.MotionControllerComponent|GetMotionSource _output_get) "Right") "/Game/VRTemplate/Input/IMC_Weapon_Right.IMC_Weapon_Right" "/Game/VRTemplate/Input/IMC_Weapon_Left.IMC_Weapon_Left")))
    (Input|AddMappingContext (PlayerController|LocalPlayerSubsystems|GetEnhancedInputLocalPlayerSubsystem _returnvalue) _output_get_2 0 "(bIgnoreAllPressedKeysUntilRelease=True,bForceImmediately=False)")
    (Transformation|AttachComponentToComponent (Variables|Default|GetGripPoint) _output_get "None" "SnapToTarget" "SnapToTarget" "KeepRelative" true)
    (Development|PrintString "MyLog: Attached Main Grip Controller" false)
    (Utilities|FlowControl|DelayUntilNextTick)
    (Utilities|FlowControl|DelayUntilNextTick)
    (if (Utilities|Enum|Equal(Enum) (Utilities|GetObjectName _output_get) "MotionControllerRight")
      (Variables|/Game/Characters/MannequinsXR/Meshes/SK_MannequinsXR_AnimBlueprint.SK_MannequinsXR_AnimBlueprint_C|SetBlendSpaceEnum (Variables|Default|GetRightHandAnim) "NewEnumerator10")
      (else
        (Variables|/Game/Characters/MannequinsXR/Meshes/SK_MannequinsXR_AnimBlueprint.SK_MannequinsXR_AnimBlueprint_C|SetBlendSpaceEnum (Variables|Default|GetLeftHandAnim) "NewEnumerator10")))
    (bind _asvrpawn (Utilities|Casting|CastToVRPawn (Variables|Default|GetVRPawn))
      (:then
        (Variables|/Game/VRTemplate/Blueprints/VRPawn.VRPawn_C|SetactiveWeapon _asvrpawn self))
      (:CastFailed
        _))
    (if (Utilities|Time|IsValidTimerHandle _timerhandle)
      (Utilities|Time|ClearandInvalidateTimerbyHandle _timerhandle))
    (elif (Utilities|IsValid (Variables|Default|GetMainGripController))
      ;[1 1 1] Reloading - Detaching magazine from gun
      (if (<= (Math|Vector|Distance(Vector) (Transformation|GetWorldLocation MotionController) (Transformation|GetWorldLocation _magazinegripcollision)) (Variables|/Script/Engine.SphereComponent|GetSphereRadius _magazinegripcollision))
        (bind _output_get_3 (Variables|Default|SetMagazineGripController MotionController))
        (if (Variables|Default|GetisMagazineAttached)
          (Variables|Default|SetjustRemovedMagazine true)
          (Development|SetHiddeninGame (Variables|Default|Getm1911_magazine) true false)
          (bind _returnvalue_2 (Game|SpawnActorfromClass "/Game/Blueprints/Ammo/Magazine_M1911.Magazine_M1911_C" (Transformation|GetWorldTransform (Variables|Default|Getm1911_magazine)) "Undefined" 0 0))
          (bind _output_get_4 (Variables|Default|SetMagazineActor _returnvalue_2))
          (bind _output_get_5 (Variables|/Game/Blueprints/Ammo/Magazine_M1911.Magazine_M1911_C|SetBulletsInMagazine _output_get_4 (Variables|Default|GetBulletsInMagazine)))
          (if (< _output_get_5 2)
            (Development|SetHiddeninGame (Variables|/Game/Blueprints/Ammo/Magazine_M1911.Magazine_M1911_C|GetnextToLastBullet _output_get_4) true false))
          (if (< _output_get_5 1)
            (Development|SetHiddeninGame (Variables|/Game/Blueprints/Ammo/Magazine_M1911.Magazine_M1911_C|GetlastBullet _output_get_4) true false))
          (if (Utilities|Enum|Equal(Enum) (Utilities|GetObjectName _output_get_3) "MotionControllerRight")
            (Variables|/Game/Characters/MannequinsXR/Meshes/SK_MannequinsXR_AnimBlueprint.SK_MannequinsXR_AnimBlueprint_C|SetBlendSpaceEnum (Variables|Default|GetRightHandAnim) "NewEnumerator5")
            (Transformation|AttachComponentToComponent (Variables|/Script/Engine.Actor|GetRootComponent _output_get_4) (Variables|Default|GetRightHand) "M1911MagazineSocket" "SnapToTarget" "SnapToTarget" "SnapToTarget" true)
            (else
              (Variables|/Game/Characters/MannequinsXR/Meshes/SK_MannequinsXR_AnimBlueprint.SK_MannequinsXR_AnimBlueprint_C|SetBlendSpaceEnum (Variables|Default|GetLeftHandAnim) "NewEnumerator5")
              (Transformation|AttachComponentToComponent (Variables|/Script/Engine.Actor|GetRootComponent _output_get_4) (Variables|Default|GetLeftHand) "M1911MagazineSocket" "SnapToTarget" "SnapToTarget" "SnapToTarget" true)
              (Transformation|SetWorldScale3D (Variables|/Script/Engine.Actor|GetRootComponent _output_get_4) "1.000000,1.000000,1.000000")))
          (Variables|Default|SetisMagazineAttached false)
          (Audio|PlaySoundatLocation "/Game/Sounds/Weapons/M1911/M1911_magazineDetached.M1911_magazineDetached" (Transformation|GetWorldLocation (Variables|Default|Getm1911_magazine)) "0, 0, 0" 1.0 1.0 0.0 0 0 0 0)
          (Utilities|FlowControl|Delay 0.5)
          (Variables|Default|SetjustRemovedMagazine false))
        (elif (and (Utilities|IsValid (Variables|Default|GetMainGripController)) (or (and (Utilities|Enum|Equal(Enum) (Utilities|GetObjectName MotionController) "MotionControllerRight") (Variables|Default|GetsledGrabbableRight)) (and (Utilities|Enum|Equal(Enum) (Utilities|GetObjectName MotionController) "MotionControllerLeft") (Variables|Default|GetsledGrabbableLeft))))
          (Variables|Default|SetSledController MotionController)
          (if (Utilities|Enum|Equal(Enum) (Utilities|GetObjectName MotionController) "MotionControllerRight")
            (Development|SetHiddeninGame (Variables|Default|GetSledHandRight) false false)
            (Development|SetHiddeninGame (Variables|Default|GetRightHand) true false)
            (else
              (Development|SetHiddeninGame (Variables|Default|GetSledHandLeft) false false)
              (Development|SetHiddeninGame (Variables|Default|GetLeftHand) true false))))))))

(event EventBeginPlay
  (bind _returnvalue (Game|Player|GetPlayerPawn 0))
  (Variables|Default|SetVRPawn _returnvalue)
  (bind _output_get (Variables|Default|SetLeftHand (Utilities|Array|Get(acopy) (Actor|GetComponentsbyTag _returnvalue "/Script/Engine.SkeletalMeshComponent" "HandLeft"))))
  (bind _output_get_2 (Variables|Default|SetRightHand (Utilities|Array|Get(acopy) (Actor|GetComponentsbyTag _returnvalue "/Script/Engine.SkeletalMeshComponent" "HandRight"))))
  (bind _assk_mannequins_xr_anim_blueprint (Utilities|Casting|CastToSK_MannequinsXR_AnimBlueprint (Components|SkeletalMesh|GetAnimInstance _output_get)))
  (Variables|Default|SetLeftHandAnim _assk_mannequins_xr_anim_blueprint)
  (bind _assk_mannequins_xr_anim_blueprint_2 (Utilities|Casting|CastToSK_MannequinsXR_AnimBlueprint (Components|SkeletalMesh|GetAnimInstance _output_get_2)))
  (Variables|Default|SetRightHandAnim _assk_mannequins_xr_anim_blueprint_2)
  (bind _returnvalue_2 (Actor|GetActorOfClass "/Game/Blueprints/Body.Body_C"))
  (Variables|Default|Setbody _returnvalue_2))

(fn ConstructionScript)

(fn RandomBulletSpread
  (params (spawnPoint :type Arrow%20Component%20Object%20Reference) (maxSpread :type Float%20%28double-precision%29))
  (bind _returnvalue (Transformation|GetWorldRotation spawnPoint))
  (bind _returnvalue_2 (* maxSpread -1.0))
  (return (Math|Transform|MakeTransform (Transformation|GetWorldLocation spawnPoint) (Math|Rotator|MakeRotator (+ (.roll _returnvalue) (Math|Random|RandomFloatinRange _returnvalue_2 maxSpread)) (+ (.pitch _returnvalue) (Math|Random|RandomFloatinRange _returnvalue_2 maxSpread)) (+ (.yaw _returnvalue) (Math|Random|RandomFloatinRange _returnvalue_2 maxSpread))) (Transformation|GetWorldScale spawnPoint))))

(fn SpreadHandler
  (Variables|Default|SetshouldSpread false))

(fn AttachtoBody
  (bind _grippoint (Variables|Default|GetGripPoint))
  (if (Variables|Default|GetphysicsEnabled)
    (Physics|SetSimulatePhysics (Variables|Default|Getm1911_housing) false)
    (Transformation|SetWorldTransform _grippoint (Transformation|GetWorldTransform (Variables|Default|GetMainGripPosition)) false false)
    (Transformation|AttachComponentToComponent (Variables|Default|Getm1911_housing) _grippoint "None" "KeepWorld" "KeepWorld" "KeepWorld" true)
    (Variables|Default|SetphysicsEnabled false)
    (Transformation|AttachComponentToComponent (Variables|Default|GetGripPoint) (Variables|/Game/Blueprints/Body.Body_C|GethandgunParent (Variables|Default|Getbody)) "None" "SnapToTarget" "SnapToTarget" "SnapToTarget" false)))