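; VR Selbstlader M1916 rifle with physical grabbing, manual reloading and projectile firing.
; Grab and Release route hands to main grip, secondary grip, magazine or charging handle, re-parenting via GripPoint and toggling physics and hand poses.
; Magazines detach as spawned actors and reattach on overlap; pulling the handle chambers rounds.
; Tick animates the bolt, ejects casings and aims two-handed grips; shots are rate-limited, with spread reduced by two-handed holding.
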(event OnComponentBeginOverlap(SecondaryGripCollision)
  (params (OverlappedComponent :type Primitive%20Component%20Object%20Reference) (OtherActor :type Actor%20Object%20Reference) (OtherComp :type Primitive%20Component%20Object%20Reference) (OtherBodyIndex :type Integer) (bFromSweep :type Boolean) (SweepResult :type Hit%20Result%20Structure%20%28by%20ref%29))
  (bind _returnvalue (Utilities|GetObjectName OtherComp))
  (if (Utilities|Enum|Equal(Enum) _returnvalue "HandCollisionLeft")
    (Variables|Default|SetSecondaryGrabbableLeft true)
    (elif (Utilities|Enum|Equal(Enum) _returnvalue "HandCollisionRight")
      (Variables|Default|SetSecondaryGrabbableRight true))))

(event OnComponentEndOverlap(SecondaryGripCollision)
  (params (OverlappedComponent :type Primitive%20Component%20Object%20Reference) (OtherActor :type Actor%20Object%20Reference) (OtherComp :type Primitive%20Component%20Object%20Reference) (OtherBodyIndex :type Integer))
  (bind _returnvalue (Utilities|GetObjectName OtherComp))
  (if (Utilities|Enum|Equal(Enum) _returnvalue "HandCollisionLeft")
    (Variables|Default|SetSecondaryGrabbableLeft false)
    (elif (Utilities|Enum|Equal(Enum) _returnvalue "HandCollisionRight")
      (Variables|Default|SetSecondaryGrabbableRight false))))

(event OnComponentBeginOverlap(MainGripCollision)
  (params (OverlappedComponent :type Primitive%20Component%20Object%20Reference) (OtherActor :type Actor%20Object%20Reference) (OtherComp :type Primitive%20Component%20Object%20Reference) (OtherBodyIndex :type Integer) (bFromSweep :type Boolean) (SweepResult :type Hit%20Result%20Structure%20%28by%20ref%29))
  (bind _returnvalue (Utilities|GetObjectName OtherComp))
  (if (Utilities|Enum|Equal(Enum) _returnvalue "HandCollisionLeft")
    (Variables|Default|SetMainGrabbableLeft true)
    (elif (Utilities|Enum|Equal(Enum) _returnvalue "HandCollisionRight")
      (Variables|Default|SetMainGrabbableRight true))))

(event OnComponentEndOverlap(MainGripCollision)
  (params (OverlappedComponent :type Primitive%20Component%20Object%20Reference) (OtherActor :type Actor%20Object%20Reference) (OtherComp :type Primitive%20Component%20Object%20Reference) (OtherBodyIndex :type Integer))
  (bind _returnvalue (Utilities|GetObjectName OtherComp))
  (if (Utilities|Enum|Equal(Enum) _returnvalue "HandCollisionLeft")
    (Variables|Default|SetMainGrabbableLeft false)
    (elif (Utilities|Enum|Equal(Enum) _returnvalue "HandCollisionRight")
      (Variables|Default|SetMainGrabbableRight false))))

(event Input|EnhancedActionEvents|EnhancedInputActionIA_Shoot_Left
  (params (ActionValue :type Boolean) (ElapsedSeconds :type Float%20%28double-precision%29) (TriggeredSeconds :type Float%20%28double-precision%29) (InputAction :type Input%20Action%20Object%20Reference :default "/Game/VRTemplate/Input/Actions/IA_Shoot_Left.IA_Shoot_Left"))
  (:Started
    ;[1 1 1] Shooting
    (Utilities|Time|SetTimerbyFunctionName 0 "spreadHandler" 1.0)
    ;;[1 0 0] Prevents the gun from shooting if:
    ;; - the user wants to shoot faster then the guns rate of fire
    ;; - there are no more bullets left in the magazine and in the chamber
    (if (and (Variables|Default|GetisShootable) (Variables|Default|GetisBulletInChamber))
      (if (Variables|Default|GetisMagazineAttached)
        (if (> (Variables|Default|GetBulletsInMagazine) 0)
          (Variables|Default|SetBulletsInMagazine (- (Variables|Default|GetBulletsInMagazine) 1))
          (else
            (Variables|Default|SetisBulletInChamber false :!label _label)))
        (else
          (goto _label)))
      (Audio|PlaySoundatLocation "/Game/Sounds/Weapons/SelbstladerM1916/SelbstladerM1916_shot.SelbstladerM1916_shot" (Transformation|GetWorldLocation (Variables|Default|GetMuzzleEnd)) "0, 0, 0" 1.0 1.0 0.0 0 0 0 0)
      ;;[1 1 1] Projectile spawning
      (if (and (not (Variables|Default|GetshouldSpread)) (Utilities|IsValid (Variables|Default|GetSecondaryGripController)))
        (Variables|Default|SetbulletSpawnTransform (Transformation|GetWorldTransform (Variables|Default|GetMuzzleEnd)))
        (else
          (bind _spawntransform (CallFunction|RandomBulletSpread (Variables|Default|GetMuzzleEnd) (Variables|Default|GetmaxSpread)))
          (Variables|Default|SetbulletSpawnTransform _spawntransform)))
      (bind _returnvalue (Game|SpawnActorfromClass "/Game/Blueprints/Ammo/MyProjectile.MyProjectile_C" (Variables|Default|GetbulletSpawnTransform) "Undefined" self (Game|Player|GetPlayerPawn 0)))
      (Variables|/Game/Blueprints/Ammo/MyProjectile.MyProjectile_C|Setdamage _returnvalue (Variables|Default|Getdamage))
      (Components|Activation|Activate (Variables|Default|GetMuzzleFlash) true)
      (Development|PrintString "ShootLog: Shot fired" false)
      (Variables|Default|SetshouldSpread true)
      ;;[1 1 1] Rate of fire delay + "animation" management
      (Variables|Default|SetslideBack true)
      (Variables|Default|SetejectCardrigeCase true)
      (Variables|Default|SetisShootable false)
      (Utilities|FlowControl|Delay 0.13)
      (Variables|Default|SetslideForward true)
      (Utilities|FlowControl|Delay 0.13)
      (Variables|Default|SetisShootable true))))

(event Input|EnhancedActionEvents|EnhancedInputActionIA_Shoot_Right
  (params (ActionValue :type Boolean) (ElapsedSeconds :type Float%20%28double-precision%29) (TriggeredSeconds :type Float%20%28double-precision%29) (InputAction :type Input%20Action%20Object%20Reference :default "/Game/VRTemplate/Input/Actions/IA_Shoot_Right.IA_Shoot_Right"))
  (:Started
    ;[1 1 1] Shooting
    (Utilities|Time|SetTimerbyFunctionName 0 "spreadHandler" 1.0)
    ;;[1 0 0] Prevents the gun from shooting if:
    ;; - the user wants to shoot faster then the guns rate of fire
    ;; - there are no more bullets left in the magazine and in the chamber
    (if (and (Variables|Default|GetisShootable) (Variables|Default|GetisBulletInChamber))
      (if (Variables|Default|GetisMagazineAttached)
        (if (> (Variables|Default|GetBulletsInMagazine) 0)
          (Variables|Default|SetBulletsInMagazine (- (Variables|Default|GetBulletsInMagazine) 1))
          (else
            (Variables|Default|SetisBulletInChamber false :!label _label)))
        (else
          (goto _label)))
      (Audio|PlaySoundatLocation "/Game/Sounds/Weapons/SelbstladerM1916/SelbstladerM1916_shot.SelbstladerM1916_shot" (Transformation|GetWorldLocation (Variables|Default|GetMuzzleEnd)) "0, 0, 0" 1.0 1.0 0.0 0 0 0 0)
      ;;[1 1 1] Projectile spawning
      (if (and (not (Variables|Default|GetshouldSpread)) (Utilities|IsValid (Variables|Default|GetSecondaryGripController)))
        (Variables|Default|SetbulletSpawnTransform (Transformation|GetWorldTransform (Variables|Default|GetMuzzleEnd)))
        (else
          (bind _spawntransform (CallFunction|RandomBulletSpread (Variables|Default|GetMuzzleEnd) (Variables|Default|GetmaxSpread)))
          (Variables|Default|SetbulletSpawnTransform _spawntransform)))
      (bind _returnvalue (Game|SpawnActorfromClass "/Game/Blueprints/Ammo/MyProjectile.MyProjectile_C" (Variables|Default|GetbulletSpawnTransform) "Undefined" self (Game|Player|GetPlayerPawn 0)))
      (Variables|/Game/Blueprints/Ammo/MyProjectile.MyProjectile_C|Setdamage _returnvalue (Variables|Default|Getdamage))
      (Components|Activation|Activate (Variables|Default|GetMuzzleFlash) true)
      (Development|PrintString "ShootLog: Shot fired" false)
      (Variables|Default|SetshouldSpread true)
      ;;[1 1 1] Rate of fire delay + "animation" management
      (Variables|Default|SetslideBack true)
      (Variables|Default|SetejectCardrigeCase true)
      (Variables|Default|SetisShootable false)
      (Utilities|FlowControl|Delay 0.13)
      (Variables|Default|SetslideForward true)
      (Utilities|FlowControl|Delay 0.13)
      (Variables|Default|SetisShootable true))))

(event Collision|EventActorBeginOverlap
  (params (OtherActor :type Actor%20Object%20Reference))
  ;[1 1 1] Reloading - Attaching magazine to gun
  (if (== (Utilities|GetClass OtherActor) "/Game/Blueprints/Ammo/Magazine_SelbstladerM1916.Magazine_SelbstladerM1916_C")
    (if (not (Variables|Default|GetisMagazineAttached))
      (bind _asmagazine_selbstlader_m1916 (Utilities|Casting|CastToMagazine_SelbstladerM1916 OtherActor))
      (bind _output_get (Variables|Default|SetMagazineActor _asmagazine_selbstlader_m1916))
      (Variables|Default|SetBulletsInMagazine (Variables|/Game/Blueprints/Ammo/Magazine_SelbstladerM1916.Magazine_SelbstladerM1916_C|GetBulletsInMagazine _output_get))
      (Actor|DestroyActor OtherActor)
      (Development|SetHiddeninGame (Variables|Default|GetselbstladerM1916_mag) false false)
      (Variables|Default|SetisMagazineAttached true)
      (Audio|PlaySoundatLocation "/Game/Sounds/Weapons/SelbstladerM1916/SelbstladerM1916_magazineAttached.SelbstladerM1916_magazineAttached" (Transformation|GetWorldLocation (Variables|Default|GetselbstladerM1916_mag)) "0, 0, 0" 1.0 1.0 0.0 0 0 0 0))))

(event EventTick
  (params (DeltaSeconds :type Float%20%28single-precision%29))
  (bind _maingripcontroller (Variables|Default|GetMainGripController))
  (bind _secondarygripcontroller (Variables|Default|GetSecondaryGripController))
  (bind _bulletspawnpoint (Variables|Default|GetBulletSpawnPoint))
  (bind _selbstladerm1916_housing (Variables|Default|GetselbstladerM1916_housing))
  (bind _selbstladerm1916_charging_handle (Variables|Default|GetselbstladerM1916_charging_handle))
  (bind _selbstladerm1916_charging_handle_2 (Variables|Default|GetselbstladerM1916_charging_handle))
  (bind _selbstladerm1916_charging_handle_3 (Variables|Default|GetselbstladerM1916_charging_handle))
  (bind _bulletspawnpoint_2 (Variables|Default|GetBulletSpawnPoint))
  (bind _selbstladerm1916_charging_handle_4 (Variables|Default|GetselbstladerM1916_charging_handle))
  (bind _selbstladerm1916_charging_handle_5 (Variables|Default|GetselbstladerM1916_charging_handle))
  (bind _boltspeed (Variables|Default|GetboltSpeed))
  (bind _selbstladerm1916_housing_2 (Variables|Default|GetselbstladerM1916_housing))
  (bind _returnvalue (Transformation|GetWorldRotation _selbstladerm1916_housing))
  (bind _returnvalue_2 (Transformation|GetWorldLocation _maingripcontroller))
  (bind _returnvalue_3 (Transformation|GetWorldLocation _secondarygripcontroller))
  (bind _returnvalue_4 (Transformation|GetWorldRotation _selbstladerm1916_housing_2))
  (bind _relativelocation (Variables|/Script/Engine.SceneComponent|GetRelativeLocation _selbstladerm1916_charging_handle))
  (bind _relativelocation_2 (Variables|/Script/Engine.SceneComponent|GetRelativeLocation _selbstladerm1916_charging_handle_4))
  (bind _relativelocation_3 (Variables|/Script/Engine.SceneComponent|GetRelativeLocation _selbstladerm1916_charging_handle_5))
  (bind _returnvalue_5 (Math|Rotator|FindLookatRotation _returnvalue_2 _returnvalue_3))
  (Utilities|FlowControl|Sequence
    (:then_0
      (Utilities|FlowControl|Sequence
        (:then_0
          ;[1 1 1] Bolt sliding back "animation"
          (if (Variables|Default|GetslideBack)
            (if (> (.y _relativelocation_2) -8.0)
              (Transformation|SetRelativeLocation (Variables|Default|GetselbstladerM1916_charging_handle) (Math|Vector|MakeVector 0.0 (- (.y _relativelocation_2) _boltspeed) 0.0) false false)
              (else
                (Variables|Default|SetslideBack false)
                (Transformation|SetRelativeLocation (Variables|Default|GetselbstladerM1916_charging_handle) (Math|Vector|MakeVector 0.0 -8.0 0.0) false false)
                ;[1 1 1] Eject cartride case after shot is fired
                (if (Variables|Default|GetejectCardrigeCase)
                  (Variables|Default|SetejectCardrigeCase false)
                  (bind _returnvalue_6 (Game|SpawnActorfromClass "/Game/Blueprints/Ammo/CartridgeCase.CartridgeCase_C" (Math|Transform|MakeTransform (Transformation|GetWorldLocation _bulletspawnpoint_2) (Transformation|GetWorldRotation _bulletspawnpoint_2)) "Undefined" 0 0))
                  (Physics|SetSimulatePhysics (Variables|/Game/Blueprints/Ammo/CartridgeCase.CartridgeCase_C|GetCartridgeCase _returnvalue_6) true)
                  (Physics|AddImpulse (Variables|/Game/Blueprints/Ammo/CartridgeCase.CartridgeCase_C|GetCartridgeCase _returnvalue_6) (* (Math|Vector|Normalize (Math|Vector|MakeVector (.roll _returnvalue) (.pitch _returnvalue) (.yaw _returnvalue))) "5.000000,5.000000,5.000000") "None" false))))))
        (:then_1
          ;[1 1 1] Bolt sliding forward "animation"
          (if (Variables|Default|GetslideForward)
            (if (< (.y _relativelocation_3) 0.0)
              (Transformation|SetRelativeLocation (Variables|Default|GetselbstladerM1916_charging_handle) (Math|Vector|MakeVector 0.0 (+ (.y _relativelocation_3) _boltspeed) 0.0) false false)
              (else
                (Variables|Default|SetslideForward false)
                (Transformation|SetRelativeLocation (Variables|Default|GetselbstladerM1916_charging_handle) (Math|Vector|MakeVector 0.0 0.0 0.0) false false)))))
        (:then_2
          ;[1 1 1] Empty reload - put bullet in chamber
          (if (Utilities|IsValid (Variables|Default|GetChargingHandleController))
            (Transformation|SetWorldLocation _selbstladerm1916_charging_handle_3 (Transformation|GetWorldLocation (Variables|Default|GetChargingHandleController)) false false)
            (Transformation|SetRelativeLocation _selbstladerm1916_charging_handle_3 (Math|Vector|MakeVector 0.0 (- (.y (Variables|/Script/Engine.SceneComponent|GetRelativeLocation _selbstladerm1916_charging_handle_3)) 25.0) 0.0) false false)
            (if (> (.y _relativelocation) 0.0)
              (Transformation|SetRelativeLocation _selbstladerm1916_charging_handle_2 (Math|Vector|MakeVector 0.0 0.0 0.0) false false)
              (elif (< (.y _relativelocation) -8.0)
                (Transformation|SetRelativeLocation _selbstladerm1916_charging_handle_2 (Math|Vector|MakeVector 0.0 -8.0 0.0) false false)
                (Variables|Default|SetChargingHandleController 0)
                (if (and (Variables|Default|GetisMagazineAttached) (> (Variables|Default|GetBulletsInMagazine) 0))
                  (if (Variables|Default|GetisBulletInChamber)
                    ;[1 1 1] Eject bullet
                    (bind _returnvalue_7 (Game|SpawnActorfromClass "/Game/Blueprints/Ammo/Bullet.Bullet_C" (Math|Transform|MakeTransform (Transformation|GetWorldLocation _bulletspawnpoint) (Transformation|GetWorldRotation _bulletspawnpoint)) "Undefined" 0 0))
                    (Physics|SetSimulatePhysics (Variables|/Game/Blueprints/Ammo/Bullet.Bullet_C|GetBullet _returnvalue_7) true)
                    (Physics|AddImpulse (Variables|/Game/Blueprints/Ammo/Bullet.Bullet_C|GetBullet _returnvalue_7) (* (Math|Vector|Normalize (Math|Vector|MakeVector (.roll _returnvalue_4) (.pitch _returnvalue_4) (.yaw _returnvalue_4))) "5.000000,5.000000,5.000000") "None" false)
                    (else
                      (Variables|Default|SetisBulletInChamber true)))
                  (Variables|Default|SetBulletsInMagazine (- (Variables|Default|GetBulletsInMagazine) 1)))
                (Variables|Default|SetslideForward true)
                (Audio|PlaySoundatLocation "/Game/Sounds/Weapons/SelbstladerM1916/SelbstladerM1916_bolt.SelbstladerM1916_bolt" (Transformation|GetWorldLocation (Variables|Default|GetselbstladerM1916_charging_handle)) "0, 0, 0" 1.0 1.0 0.0 0 0 0 0)))))))
    (:then_1
      (if (and (Utilities|IsValid (Variables|Default|GetMainGripController)) (Utilities|IsValid (Variables|Default|GetSecondaryGripController))) ; Checks if the player grabbed with both hands
        ;[1 1 1] Two handed grab rotating
        (Transformation|SetWorldRotation (Variables|Default|GetGripPoint) (Math|Rotator|MakeRotator 0.0 (+ (.pitch _returnvalue_5) 45.0) (.yaw _returnvalue_5)) false false)))))

(event EventGrab
  (params (MotionController :type Motion%20Controller%20Component%20Object%20Reference))
  (bind _returnvalue (Game|GetPlayerController 0))
  (bind _grippoint (Variables|Default|GetGripPoint))
  (bind _charginghandlecollision (Variables|Default|GetChargingHandleCollision))
  (bind _magazinegripcollision (Variables|Default|GetMagazineGripCollision))
  (if (Variables|Default|GetphysicsEnabled)
    (Physics|SetSimulatePhysics (Variables|Default|GetselbstladerM1916_housing) false)
    (Transformation|SetWorldTransform _grippoint (Transformation|GetWorldTransform (Variables|Default|GetMainGripPosition)) false false)
    (Transformation|AttachComponentToComponent (Variables|Default|GetselbstladerM1916_housing) _grippoint "None" "KeepWorld" "KeepWorld" "KeepWorld" true)
    (Variables|Default|SetphysicsEnabled false))
  (if (or (and (Utilities|Enum|Equal(Enum) (Utilities|GetObjectName MotionController) "MotionControllerRight") (Variables|Default|GetMainGrabbableRight)) (and (Utilities|Enum|Equal(Enum) (Utilities|GetObjectName MotionController) "MotionControllerLeft") (Variables|Default|GetMainGrabbableLeft)))
    (bind _output_get (Variables|Default|SetMainGripController MotionController))
    ;[1 1 1] Trigger assignment
    (Input|EnableInput _returnvalue)
    (bind _output_get_2 (Variables|Default|SetMappingContext (select (== (Variables|/Script/HeadMountedDisplay.MotionControllerComponent|GetMotionSource _output_get) "Right") "/Game/VRTemplate/Input/IMC_Weapon_Right.IMC_Weapon_Right" "/Game/VRTemplate/Input/IMC_Weapon_Left.IMC_Weapon_Left")))
    (Input|AddMappingContext (PlayerController|LocalPlayerSubsystems|GetEnhancedInputLocalPlayerSubsystem _returnvalue) _output_get_2 0 "(bIgnoreAllPressedKeysUntilRelease=True,bForceImmediately=False)")
    (Variables|Default|GetSecondaryGripController
      (:then
        (Transformation|DetachFromComponent (Variables|Default|GetGripPoint) "KeepWorld" "KeepWorld" "KeepWorld" true)
        (Transformation|DetachFromComponent (Variables|Default|GetselbstladerM1916_housing) "KeepWorld" "KeepWorld" "KeepWorld" true)
        (Transformation|SetWorldTransform (Variables|Default|GetGripPoint) (Transformation|GetWorldTransform (Variables|Default|GetMainGripPosition)) false false)
        (Transformation|AttachComponentToComponent (Variables|Default|GetselbstladerM1916_housing) (Variables|Default|GetGripPoint) "None" "KeepWorld" "KeepWorld" "KeepWorld" true))
      (:else
        _))
    (Transformation|AttachComponentToComponent (Variables|Default|GetGripPoint) _output_get "None" "SnapToTarget" "SnapToTarget" "KeepRelative" true)
    (Development|PrintString "MyLog: Attached Main Grip Controller" false)
    (Utilities|FlowControl|DelayUntilNextTick)
    (Utilities|FlowControl|DelayUntilNextTick)
    (if (Utilities|Enum|Equal(Enum) (Utilities|GetObjectName _output_get) "MotionControllerRight")
      (Variables|/Game/Characters/MannequinsXR/Meshes/SK_MannequinsXR_AnimBlueprint.SK_MannequinsXR_AnimBlueprint_C|SetBlendSpaceEnum (Variables|Default|GetRightHandAnim) "NewEnumerator10")
      (else
        (Variables|/Game/Characters/MannequinsXR/Meshes/SK_MannequinsXR_AnimBlueprint.SK_MannequinsXR_AnimBlueprint_C|SetBlendSpaceEnum (Variables|Default|GetLeftHandAnim) "NewEnumerator10")))
    (bind _asvrpawn (Utilities|Casting|CastToVRPawn (Variables|Default|GetVRPawn) :!label _label))
    (Variables|/Game/VRTemplate/Blueprints/VRPawn.VRPawn_C|SetactiveWeapon _asvrpawn self)
    (elif (or (and (Utilities|Enum|Equal(Enum) (Utilities|GetObjectName MotionController) "MotionControllerRight") (Variables|Default|GetSecondaryGrabbableRight)) (and (Utilities|Enum|Equal(Enum) (Utilities|GetObjectName MotionController) "MotionControllerLeft") (Variables|Default|GetSecondaryGrabbableLeft)))
      (Variables|Default|SetSecondaryGripController MotionController)
      (Utilities|String|LogString "MyLog: Set Secondary Grip Controller")
      (if (Utilities|Enum|Equal(Enum) (Utilities|GetObjectName MotionController) "MotionControllerRight")
        (Development|SetHiddeninGame (Variables|Default|GetSecondaryHandRight) false false)
        (Development|SetHiddeninGame (Variables|Default|GetRightHand) true false)
        (else
          (Development|SetHiddeninGame (Variables|Default|GetSecondaryHandLeft) false false)
          (Development|SetHiddeninGame (Variables|Default|GetLeftHand) true false)))
      (if (not (Utilities|IsValid (Variables|Default|GetMainGripController)))
        (Transformation|AttachComponentToComponent (Variables|Default|GetGripPoint) (Variables|Default|GetSecondaryGripController) "None" "KeepWorld" "KeepWorld" "KeepWorld" true)
        (Variables|Default|SetisSecondaryControllerAttached true)
        (goto _label))
      (else
        ;[1 1 1] Reloading - Detaching magazine from gun
        (if (<= (Math|Vector|Distance(Vector) (Transformation|GetWorldLocation MotionController) (Transformation|GetWorldLocation _magazinegripcollision)) (Variables|/Script/Engine.SphereComponent|GetSphereRadius _magazinegripcollision))
          (bind _output_get_3 (Variables|Default|SetMagazineGripController MotionController))
          (if (Variables|Default|GetisMagazineAttached)
            (Development|SetHiddeninGame (Variables|Default|GetselbstladerM1916_mag) true false)
            (bind _returnvalue_2 (Game|SpawnActorfromClass "/Game/Blueprints/Ammo/Magazine_SelbstladerM1916.Magazine_SelbstladerM1916_C" (Transformation|GetWorldTransform (Variables|Default|GetselbstladerM1916_mag)) "Undefined" 0 0))
            (bind _output_get_4 (Variables|Default|SetMagazineActor _returnvalue_2))
            (bind _output_get_5 (Variables|/Game/Blueprints/Ammo/Magazine_SelbstladerM1916.Magazine_SelbstladerM1916_C|SetBulletsInMagazine _output_get_4 (Variables|Default|GetBulletsInMagazine)))
            (if (<= _output_get_5 0)
              (Development|SetHiddeninGame (Variables|/Game/Blueprints/Ammo/Magazine_SelbstladerM1916.Magazine_SelbstladerM1916_C|GetBullet _output_get_4) true false))
            (if (Utilities|Enum|Equal(Enum) (Utilities|GetObjectName _output_get_3) "MotionControllerRight")
              (Variables|/Game/Characters/MannequinsXR/Meshes/SK_MannequinsXR_AnimBlueprint.SK_MannequinsXR_AnimBlueprint_C|SetBlendSpaceEnum (Variables|Default|GetRightHandAnim) "NewEnumerator5")
              (Transformation|AttachComponentToComponent (Variables|/Script/Engine.Actor|GetRootComponent _output_get_4) (Variables|Default|GetRightHand) "allFingerOpenGrabSocket" "SnapToTarget" "SnapToTarget" "SnapToTarget" true)
              (else
                (Variables|/Game/Characters/MannequinsXR/Meshes/SK_MannequinsXR_AnimBlueprint.SK_MannequinsXR_AnimBlueprint_C|SetBlendSpaceEnum (Variables|Default|GetLeftHandAnim) "NewEnumerator5")
                (Transformation|AttachComponentToComponent (Variables|/Script/Engine.Actor|GetRootComponent _output_get_4) (Variables|Default|GetLeftHand) "allFingerOpenGrabSocket" "SnapToTarget" "SnapToTarget" "SnapToTarget" true)
                (Transformation|SetWorldScale3D (Variables|/Script/Engine.Actor|GetRootComponent _output_get_4) "1.000000,1.000000,1.000000")))
            (Variables|Default|SetisMagazineAttached false)
            (Audio|PlaySoundatLocation "/Game/Sounds/Weapons/SelbstladerM1916/SelbstladerM1916_magazineDetached.SelbstladerM1916_magazineDetached" (Transformation|GetWorldLocation (Variables|Default|GetselbstladerM1916_mag)) "0, 0, 0" 1.0 1.0 0.0 0 0 0 0)
            (goto _label))
          (elif (and (<= (Math|Vector|Distance(Vector) (Transformation|GetWorldLocation MotionController) (Transformation|GetWorldLocation _charginghandlecollision)) (Variables|/Script/Engine.SphereComponent|GetSphereRadius _charginghandlecollision)) (or (Utilities|IsValid (Variables|Default|GetMainGripController)) (Utilities|IsValid (Variables|Default|GetSecondaryGripController))))
            (Variables|Default|SetChargingHandleController MotionController)
            (if (Utilities|Enum|Equal(Enum) (Utilities|GetObjectName MotionController) "MotionControllerRight")
              (Variables|/Game/Characters/MannequinsXR/Meshes/SK_MannequinsXR_AnimBlueprint.SK_MannequinsXR_AnimBlueprint_C|SetBlendSpaceEnum (Variables|Default|GetRightHandAnim) "NewEnumerator3")
              (goto _label)
              (else
                (Variables|/Game/Characters/MannequinsXR/Meshes/SK_MannequinsXR_AnimBlueprint.SK_MannequinsXR_AnimBlueprint_C|SetBlendSpaceEnum (Variables|Default|GetLeftHandAnim) "NewEnumerator3")
                (goto _label)))))))))

(event EventRelease
  (params (MotionController :type Motion%20Controller%20Component%20Object%20Reference))
  (bind _returnvalue (Game|GetPlayerController 0))
  (bind _selbstladerm1916_housing (Variables|Default|GetselbstladerM1916_housing))
  (bind _secondarygripposition (Variables|Default|GetSecondaryGripPosition))
  (bind _magazineactor (Variables|Default|GetMagazineActor))
  (bind _returnvalue_2 (Transformation|GetWorldRotation _selbstladerm1916_housing))
  (bind _returnvalue_3 (Transformation|GetWorldTransform _secondarygripposition))
  (Utilities|FlowControl|Sequence
    (:then_0
      (if (== MotionController (Variables|Default|GetMainGripController))
        (Transformation|DetachFromComponent (Variables|Default|GetGripPoint) "KeepWorld" "KeepWorld" "KeepWorld" true)
        ;[1 1 1] Trigger removal
        (Input|DisableInput _returnvalue)
        (Input|RemoveMappingContext (PlayerController|LocalPlayerSubsystems|GetEnhancedInputLocalPlayerSubsystem _returnvalue) (select (== (Variables|/Script/HeadMountedDisplay.MotionControllerComponent|GetMotionSource (Variables|Default|GetMainGripController)) "Right") "/Game/VRTemplate/Input/IMC_Weapon_Right.IMC_Weapon_Right" "/Game/VRTemplate/Input/IMC_Weapon_Left.IMC_Weapon_Left") "(bIgnoreAllPressedKeysUntilRelease=True,bForceImmediately=False)")
        (Variables|Default|SetMainGripController 0)
        (Utilities|String|LogString "MyLog: Detached Main Grip Controller")
        (bind _secondarygripcontroller (Variables|Default|GetSecondaryGripController)
          (:then
            (Transformation|DetachFromComponent _selbstladerm1916_housing "KeepWorld" "KeepWorld" "KeepWorld" true)
            (Transformation|SetWorldTransform (Variables|Default|GetGripPoint) (Math|Transform|MakeTransform (.location _returnvalue_3) (Math|Rotator|MakeRotator (+ (.roll (.rotation _returnvalue_3)) (- (.roll (Transformation|GetWorldRotation _secondarygripcontroller)) (.roll _returnvalue_2))) (+ (.pitch (.rotation _returnvalue_3)) (- (.pitch (Transformation|GetWorldRotation _secondarygripcontroller)) (.pitch _returnvalue_2))) (+ (.yaw (.rotation _returnvalue_3)) (- (.yaw (Transformation|GetWorldRotation _secondarygripcontroller)) (.yaw _returnvalue_2)))) (.scale _returnvalue_3)) false false)
            (Transformation|AttachComponentToComponent (Variables|Default|GetselbstladerM1916_housing) (Variables|Default|GetGripPoint) "None" "KeepWorld" "KeepWorld" "KeepWorld" true)
            (bind _returnvalue_4 (Transformation|AttachComponentToComponent (Variables|Default|GetGripPoint) _secondarygripcontroller "None" "SnapToTarget" "SnapToTarget" "KeepRelative" true))
            (Variables|Default|SetisSecondaryControllerAttached _returnvalue_4))
          (:else
            _))
        (if (and (not (Utilities|IsValid (Variables|Default|GetMainGripController))) (not (Utilities|IsValid (Variables|Default|GetSecondaryGripController)))) :!label _label
          (Variables|Default|SetChargingHandleController 0)
          (Physics|SetSimulatePhysics (Variables|Default|GetselbstladerM1916_housing) true)
          (Variables|Default|SetphysicsEnabled true))))
    (:then_1
      (if (== MotionController (Variables|Default|GetSecondaryGripController))
        (if (Variables|Default|GetisSecondaryControllerAttached)
          (Transformation|DetachFromComponent (Variables|Default|GetGripPoint) "KeepWorld" "KeepWorld" "KeepWorld" true)
          (Variables|Default|SetisSecondaryControllerAttached false)
          (Transformation|DetachFromComponent (Variables|Default|GetselbstladerM1916_housing) "KeepWorld" "KeepWorld" "KeepWorld" true)
          (Transformation|SetWorldTransform (Variables|Default|GetGripPoint) (Transformation|GetWorldTransform (Variables|Default|GetMainGripPosition)) false false)
          (Transformation|AttachComponentToComponent (Variables|Default|GetselbstladerM1916_housing) (Variables|Default|GetGripPoint) "None" "KeepWorld" "KeepWorld" "KeepWorld" true)
          (if (Utilities|IsValid (Variables|Default|GetMainGripController))
            (Transformation|AttachComponentToComponent (Variables|Default|GetGripPoint) (Variables|Default|GetMainGripController) "None" "SnapToTarget" "SnapToTarget" "SnapToTarget" true)))
        (Variables|Default|SetSecondaryGripController 0)
        (Utilities|String|LogString "MyLog: Released Secondary Grip Controller")
        (if (Utilities|Enum|Equal(Enum) (Utilities|GetObjectName MotionController) "MotionControllerRight")
          (Development|SetHiddeninGame (Variables|Default|GetSecondaryHandRight) true false)
          (Development|SetHiddeninGame (Variables|Default|GetRightHand) false false)
          (else
            (Development|SetHiddeninGame (Variables|Default|GetSecondaryHandLeft) true false)
            (Development|SetHiddeninGame (Variables|Default|GetLeftHand) false false)))
        (bind _maingripcontroller (Variables|Default|GetMainGripController)
          (:then
            (Transformation|SetWorldRotation (Variables|Default|GetGripPoint) (Transformation|GetWorldRotation _maingripcontroller) false false)
            (goto _label))
          (:else
            (goto _label)))
        (else
          ;[1 1 1] Reloading - Detaching magazine from hand
          (if (== MotionController (Variables|Default|GetMagazineGripController))
            (bind _magazineactor_2 (Variables|Default|GetMagazineActor)
              (:then
                (Transformation|DetachFromActor _magazineactor_2 "KeepWorld" "KeepWorld" "KeepWorld")
                (Variables|Default|SetMagazineGripController 0)
                (Physics|SetSimulatePhysics (Variables|/Game/Blueprints/Ammo/Magazine_SelbstladerM1916.Magazine_SelbstladerM1916_C|GetselbstladerM1916_mag _magazineactor) true)
                (Variables|/Game/Blueprints/Ammo/Magazine_SelbstladerM1916.Magazine_SelbstladerM1916_C|SetphysicsEnabled _magazineactor true))
              (:else))
            (elif (== MotionController (Variables|Default|GetChargingHandleController))
              (Variables|Default|SetChargingHandleController 0))))))))

(event EventBeginPlay
  (bind _returnvalue (Game|Player|GetPlayerPawn 0))
  (Variables|Default|SetVRPawn _returnvalue)
  (bind _output_get (Variables|Default|SetLeftHand (Utilities|Array|Get(acopy) (Actor|GetComponentsbyTag _returnvalue "/Script/Engine.SkeletalMeshComponent" "HandLeft"))))
  (bind _output_get_2 (Variables|Default|SetRightHand (Utilities|Array|Get(acopy) (Actor|GetComponentsbyTag _returnvalue "/Script/Engine.SkeletalMeshComponent" "HandRight"))))
  (bind _assk_mannequins_xr_anim_blueprint (Utilities|Casting|CastToSK_MannequinsXR_AnimBlueprint (Components|SkeletalMesh|GetAnimInstance _output_get)))
  (Variables|Default|SetLeftHandAnim _assk_mannequins_xr_anim_blueprint)
  (bind _assk_mannequins_xr_anim_blueprint_2 (Utilities|Casting|CastToSK_MannequinsXR_AnimBlueprint (Components|SkeletalMesh|GetAnimInstance _output_get_2)))
  (Variables|Default|SetRightHandAnim _assk_mannequins_xr_anim_blueprint_2))

(fn ConstructionScript)

(fn RandomBulletSpread
  (params (spawnPoint :type Arrow%20Component%20Object%20Reference) (maxSpread :type Float%20%28double-precision%29))
  (bind _returnvalue (Transformation|GetWorldRotation spawnPoint))
  ;[1 1 1] Random bullet spread
  (if (Utilities|IsValid (Variables|Default|GetSecondaryGripController))
    (LocalVariables|Setspread (/ maxSpread (LocalVariables|GetspreadDivider)))
    (else
      (LocalVariables|Setspread maxSpread)))
  (return (Math|Transform|MakeTransform (Transformation|GetWorldLocation spawnPoint) (Math|Rotator|MakeRotator (+ (.roll _returnvalue) (Math|Random|RandomFloatinRange (* (LocalVariables|Getspread) -1.0) (LocalVariables|Getspread))) (+ (.pitch _returnvalue) (Math|Random|RandomFloatinRange (* (LocalVariables|Getspread) -1.0) (LocalVariables|Getspread))) (+ (.yaw _returnvalue) (Math|Random|RandomFloatinRange (* (LocalVariables|Getspread) -1.0) (LocalVariables|Getspread)))) (Transformation|GetWorldScale spawnPoint))))

(fn SpreadHandler
  (Variables|Default|SetshouldSpread false))