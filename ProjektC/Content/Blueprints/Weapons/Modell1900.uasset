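; VR break-action double-barrel Modell 1900 shotgun with main, secondary and barrel grips that swap hand meshes or poses.
; Grab and Release re-parent GripPoint between controllers, while Tick aims two-handed via look-at or hinges the barrel.
; Opening the barrel ejects spent cases and lets overlap zones load shells.
; Firing requires a closed barrel and spawns pellets through a tick-delayed loop, with spread divided while the secondary grip is held.
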(event OnComponentBeginOverlap(ReloadZoneRight)
  (params (OverlappedComponent :type Primitive%20Component%20Object%20Reference) (OtherActor :type Actor%20Object%20Reference) (OtherComp :type Primitive%20Component%20Object%20Reference) (OtherBodyIndex :type Integer) (bFromSweep :type Boolean) (SweepResult :type Hit%20Result%20Structure%20%28by%20ref%29))
  (CallFunction|Reload false OtherActor))

(event OnComponentBeginOverlap(ReloadZoneLeft)
  (params (OverlappedComponent :type Primitive%20Component%20Object%20Reference) (OtherActor :type Actor%20Object%20Reference) (OtherComp :type Primitive%20Component%20Object%20Reference) (OtherBodyIndex :type Integer) (bFromSweep :type Boolean) (SweepResult :type Hit%20Result%20Structure%20%28by%20ref%29))
  (CallFunction|Reload true OtherActor))

(event OnComponentBeginOverlap(SecondaryGripCollision)
  (params (OverlappedComponent :type Primitive%20Component%20Object%20Reference) (OtherActor :type Actor%20Object%20Reference) (OtherComp :type Primitive%20Component%20Object%20Reference) (OtherBodyIndex :type Integer) (bFromSweep :type Boolean) (SweepResult :type Hit%20Result%20Structure%20%28by%20ref%29))
  (bind _returnvalue (Utilities|GetObjectName OtherComp))
  (if (Utilities|Enum|Equal(Enum) _returnvalue "HandCollisionLeft")
    (Variables|Default|SetSecondaryGrabbableLeft true)
    (elif (Utilities|Enum|Equal(Enum) _returnvalue "HandCollisionRight")
      (Variables|Default|SetSecondaryGrabbableRight true))))

(event OnComponentEndOverlap(SecondaryGripCollision)
  (params (OverlappedComponent :type Primitive%20Component%20Object%20Reference) (OtherActor :type Actor%20Object%20Reference) (OtherComp :type Primitive%20Component%20Object%20Reference) (OtherBodyIndex :type Integer))
  (bind _returnvalue (Utilities|GetObjectName OtherComp))
  (if (Utilities|Enum|Equal(Enum) _returnvalue "HandCollisionLeft")
    (Variables|Default|SetSecondaryGrabbableLeft false)
    (elif (Utilities|Enum|Equal(Enum) _returnvalue "HandCollisionRight")
      (Variables|Default|SetSecondaryGrabbableRight false))))

(event OnComponentBeginOverlap(BarrelGripCollision)
  (params (OverlappedComponent :type Primitive%20Component%20Object%20Reference) (OtherActor :type Actor%20Object%20Reference) (OtherComp :type Primitive%20Component%20Object%20Reference) (OtherBodyIndex :type Integer) (bFromSweep :type Boolean) (SweepResult :type Hit%20Result%20Structure%20%28by%20ref%29))
  (bind _returnvalue (Utilities|GetObjectName OtherComp))
  (if (Utilities|Enum|Equal(Enum) _returnvalue "HandCollisionLeft")
    (Variables|Default|SetBarrelGrabbableLeft true)
    (elif (Utilities|Enum|Equal(Enum) _returnvalue "HandCollisionRight")
      (Variables|Default|SetBarrelGrabbableRight true))))

(event OnComponentEndOverlap(BarrelGripCollision)
  (params (OverlappedComponent :type Primitive%20Component%20Object%20Reference) (OtherActor :type Actor%20Object%20Reference) (OtherComp :type Primitive%20Component%20Object%20Reference) (OtherBodyIndex :type Integer))
  (bind _returnvalue (Utilities|GetObjectName OtherComp))
  (if (Utilities|Enum|Equal(Enum) _returnvalue "HandCollisionLeft")
    (Variables|Default|SetBarrelGrabbableLeft false)
    (elif (Utilities|Enum|Equal(Enum) _returnvalue "HandCollisionRight")
      (Variables|Default|SetBarrelGrabbableRight false))))

(event OnComponentBeginOverlap(MainGripCollision)
  (params (OverlappedComponent :type Primitive%20Component%20Object%20Reference) (OtherActor :type Actor%20Object%20Reference) (OtherComp :type Primitive%20Component%20Object%20Reference) (OtherBodyIndex :type Integer) (bFromSweep :type Boolean) (SweepResult :type Hit%20Result%20Structure%20%28by%20ref%29))
  (bind _returnvalue (Utilities|GetObjectName OtherComp))
  (if (Utilities|Enum|Equal(Enum) _returnvalue "HandCollisionLeft")
    (Variables|Default|SetMainGrabbableLeft true)
    (elif (Utilities|Enum|Equal(Enum) _returnvalue "HandCollisionRight")
      (Variables|Default|SetMainGrabbableRight true))))

(event OnComponentEndOverlap(MainGripCollision)
  (params (OverlappedComponent :type Primitive%20Component%20Object%20Reference) (OtherActor :type Actor%20Object%20Reference) (OtherComp :type Primitive%20Component%20Object%20Reference) (OtherBodyIndex :type Integer))
  (bind _returnvalue (Utilities|GetObjectName OtherComp))
  (if (Utilities|Enum|Equal(Enum) _returnvalue "HandCollisionLeft")
    (Variables|Default|SetMainGrabbableLeft false)
    (elif (Utilities|Enum|Equal(Enum) _returnvalue "HandCollisionRight")
      (Variables|Default|SetMainGrabbableRight false))))

(event Input|EnhancedActionEvents|EnhancedInputActionIA_Shoot_Left
  (params (ActionValue :type Boolean) (ElapsedSeconds :type Float%20%28double-precision%29) (TriggeredSeconds :type Float%20%28double-precision%29) (InputAction :type Input%20Action%20Object%20Reference :default "/Game/VRTemplate/Input/Actions/IA_Shoot_Left.IA_Shoot_Left"))
  ;[1 1 1] Shooting
  (:Started
    ;;[1 0 0] Prevents the gun from shooting if:
    ;; - the barrel is not closed
    ;; - neither the left or the right bullet is loaded
    (if (Variables|Default|GetisBarrelClosed)
      (if (Variables|Default|GetisLeftBulletLoaded)
        (Variables|Default|SetisLeftBulletLoaded false)
        (Variables|Default|SetejectLeft true)
        (Components|Activation|Activate (Variables|Default|GetMuzzleFlash) true :!label _label)
        ;[1 1 1] Projectile spawning
        (bind _spawntransform (CallFunction|RandomBulletSpread (Variables|Default|GetMuzzleEnd) (Variables|Default|GetmaxSpread) :!label _label_2))
        (Game|SpawnActorfromClass "/Game/Blueprints/Ammo/MyProjectile.MyProjectile_C" _spawntransform "Undefined" self (Game|Player|GetPlayerPawn 0))
        ;[1 1 1] For-loop didn't work
        (Variables|Default|SetpelletsFired (+ 1 (Variables|Default|GetpelletsFired)))
        (if (< (Variables|Default|GetpelletsFired) (Variables|Default|GetpelletsPerShot))
          ;[1 1 1] Preventing the bullets from hitting each other
          (Utilities|FlowControl|DelayUntilNextTick)
          (Utilities|FlowControl|DelayUntilNextTick)
          (goto _label_2)
          (else
            (Variables|Default|SetpelletsFired 0)))
        (elif (Variables|Default|GetisRightBulletLoaded)
          (Variables|Default|SetisRightBulletLoaded false)
          (Variables|Default|SetejectRight true)
          (goto _label))))))

(event Input|EnhancedActionEvents|EnhancedInputActionIA_Shoot_Right
  (params (ActionValue :type Boolean) (ElapsedSeconds :type Float%20%28double-precision%29) (TriggeredSeconds :type Float%20%28double-precision%29) (InputAction :type Input%20Action%20Object%20Reference :default "/Game/VRTemplate/Input/Actions/IA_Shoot_Right.IA_Shoot_Right"))
  ;[1 1 1] Shooting
  (:Started
    ;;[1 0 0] Prevents the gun from shooting if:
    ;; - the barrel is not closed
    ;; - neither the left or the right bullet is loaded
    (if (Variables|Default|GetisBarrelClosed)
      (if (Variables|Default|GetisLeftBulletLoaded)
        (Variables|Default|SetisLeftBulletLoaded false)
        (Variables|Default|SetejectLeft true)
        (Components|Activation|Activate (Variables|Default|GetMuzzleFlash) true :!label _label)
        ;[1 1 1] Projectile spawning
        (bind _spawntransform (CallFunction|RandomBulletSpread (Variables|Default|GetMuzzleEnd) (Variables|Default|GetmaxSpread) :!label _label_2))
        (Game|SpawnActorfromClass "/Game/Blueprints/Ammo/MyProjectile.MyProjectile_C" _spawntransform "Undefined" self (Game|Player|GetPlayerPawn 0))
        ;[1 1 1] For-loop didn't work
        (Variables|Default|SetpelletsFired (+ 1 (Variables|Default|GetpelletsFired)))
        (if (< (Variables|Default|GetpelletsFired) (Variables|Default|GetpelletsPerShot))
          ;[1 1 1] Preventing the bullets from hitting each other
          (Utilities|FlowControl|DelayUntilNextTick)
          (Utilities|FlowControl|DelayUntilNextTick)
          (goto _label_2)
          (else
            (Variables|Default|SetpelletsFired 0)))
        (elif (Variables|Default|GetisRightBulletLoaded)
          (Variables|Default|SetisRightBulletLoaded false)
          (Variables|Default|SetejectRight true)
          (goto _label))))))

(event EventTick
  (params (DeltaSeconds :type Float%20%28single-precision%29))
  (bind _maingripcontroller (Variables|Default|GetMainGripController))
  (bind _secondarygripcontroller (Variables|Default|GetSecondaryGripController))
  (bind _barrelgripcontroller (Variables|Default|GetBarrelGripController))
  (bind _modell1900_barrel (Variables|Default|Getmodell1900_barrel))
  (bind _modell1900_stock (Variables|Default|Getmodell1900_stock))
  (bind _modell1900_barrel_2 (Variables|Default|Getmodell1900_barrel))
  (bind _returnvalue (Transformation|GetWorldLocation _maingripcontroller))
  (bind _returnvalue_2 (Transformation|GetWorldLocation _secondarygripcontroller))
  (bind _returnvalue_3 (Transformation|GetWorldRotation _modell1900_stock))
  (bind _relativerotation (Variables|/Script/Engine.SceneComponent|GetRelativeRotation _modell1900_barrel))
  (bind _returnvalue_4 (Math|Rotator|FindLookatRotation _returnvalue _returnvalue_2))
  (if (and (Utilities|IsValid (Variables|Default|GetMainGripController)) (Utilities|IsValid (Variables|Default|GetSecondaryGripController))) ; Checks if the player grabbed with both hands
    ;[1 1 1] Two handed grab rotating
    (Transformation|SetWorldRotation (Variables|Default|GetGripPoint) (Math|Rotator|MakeRotator 0.0 (+ (.pitch _returnvalue_4) 45.0) (.yaw _returnvalue_4)) false false)
    (else
      ;[1 1 1] Barrel rotating
      (if (Utilities|IsValid _barrelgripcontroller)
        (Transformation|SetWorldRotation _modell1900_barrel (Math|Rotator|MakeRotator (* (.pitch (Math|Rotator|FindLookatRotation (Transformation|GetWorldLocation _modell1900_stock) (Transformation|GetWorldLocation _barrelgripcontroller))) -1.0) (.pitch _returnvalue_3) (.yaw _returnvalue_3)) false false)
        ;[1 1 1] Controls the open/closed state of the barrel
        (Variables|Default|SetisBarrelClosed (not (> (.roll _relativerotation) 0.0)))
        (if (> (.roll _relativerotation) 3e+01)
          (Variables|Default|SetisBarrelOpen true)
          ;;[1 1 1] Visuals
          (if (Variables|Default|GetejectLeft)
            (Development|SetHiddeninGame (Variables|Default|Getbullet_left) true false)
            (CallFunction|EjectCartridgeCase (Variables|Default|GetejecttionPointLeft))
            (Variables|Default|SetejectLeft false))
          (if (Variables|Default|GetejectRight)
            (Development|SetHiddeninGame (Variables|Default|Getbullet_right) true false)
            (CallFunction|EjectCartridgeCase (Variables|Default|GetejecttionPointRight))
            (Variables|Default|SetejectRight false))
          (if (> (.roll _relativerotation) 4e+01)
            (Transformation|SetRelativeRotation _modell1900_barrel_2 "0.000000,0.000000,40.000000" false false))
          (elif (< (.roll _relativerotation) 2e+01)
            (Variables|Default|SetisBarrelOpen false)
            (if (< (.roll _relativerotation) 0.0)
              (Variables|Default|SetisBarrelClosed true)
              (Transformation|SetRelativeRotation _modell1900_barrel_2 "0, 0, 0" false false))))))))

(event EventGrab
  (params (MotionController :type Motion%20Controller%20Component%20Object%20Reference))
  (bind _returnvalue (Game|GetPlayerController 0))
  (Utilities|String|LogString "MyLog: Grab started")
  (if (or (and (Utilities|Enum|Equal(Enum) (Utilities|GetObjectName MotionController) "MotionControllerRight") (Variables|Default|GetMainGrabbableRight)) (and (Utilities|Enum|Equal(Enum) (Utilities|GetObjectName MotionController) "MotionControllerLeft") (Variables|Default|GetMainGrabbableLeft)))
    (bind _output_get (Variables|Default|SetMainGripController MotionController))
    ;[1 1 1] Trigger assignment
    (Input|EnableInput _returnvalue)
    (bind _output_get_2 (Variables|Default|SetMappingContext (select (== (Variables|/Script/HeadMountedDisplay.MotionControllerComponent|GetMotionSource _output_get) "Right") "/Game/VRTemplate/Input/IMC_Weapon_Right.IMC_Weapon_Right" "/Game/VRTemplate/Input/IMC_Weapon_Left.IMC_Weapon_Left")))
    (Input|AddMappingContext (PlayerController|LocalPlayerSubsystems|GetEnhancedInputLocalPlayerSubsystem _returnvalue) _output_get_2 0 "(bIgnoreAllPressedKeysUntilRelease=True,bForceImmediately=False)")
    (Variables|Default|GetSecondaryGripController
      (:then
        (Transformation|DetachFromComponent (Variables|Default|GetGripPoint) "KeepWorld" "KeepWorld" "KeepWorld" true)
        (Transformation|DetachFromComponent (Variables|Default|Getmodell1900_stock) "KeepWorld" "KeepWorld" "KeepWorld" true)
        (Transformation|SetWorldTransform (Variables|Default|GetGripPoint) (Transformation|GetWorldTransform (Variables|Default|GetMainGripPoint)) false false)
        (Transformation|AttachComponentToComponent (Variables|Default|Getmodell1900_stock) (Variables|Default|GetGripPoint) "None" "KeepWorld" "KeepWorld" "KeepWorld" true))
      (:else
        _))
    (Transformation|AttachComponentToComponent (Variables|Default|GetGripPoint) _output_get "None" "SnapToTarget" "SnapToTarget" "KeepRelative" true)
    (Development|PrintString "MyLog: Attached Main Grip Controller" false)
    (Utilities|FlowControl|DelayUntilNextTick)
    (Utilities|FlowControl|DelayUntilNextTick)
    (if (Utilities|Enum|Equal(Enum) (Utilities|GetObjectName _output_get) "MotionControllerRight")
      (Variables|/Game/Characters/MannequinsXR/Meshes/SK_MannequinsXR_AnimBlueprint.SK_MannequinsXR_AnimBlueprint_C|SetBlendSpaceEnum (Variables|Default|GetRightHandAnim) "NewEnumerator11")
      (else
        (Variables|/Game/Characters/MannequinsXR/Meshes/SK_MannequinsXR_AnimBlueprint.SK_MannequinsXR_AnimBlueprint_C|SetBlendSpaceEnum (Variables|Default|GetLeftHandAnim) "NewEnumerator11")))
    (bind _asvrpawn (Utilities|Casting|CastToVRPawn (Variables|Default|GetVRPawn) :!label _label))
    (Variables|/Game/VRTemplate/Blueprints/VRPawn.VRPawn_C|SetactiveWeapon _asvrpawn self)
    (elif (or (and (Utilities|Enum|Equal(Enum) (Utilities|GetObjectName MotionController) "MotionControllerRight") (Variables|Default|GetSecondaryGrabbableRight)) (and (Utilities|Enum|Equal(Enum) (Utilities|GetObjectName MotionController) "MotionControllerLeft") (Variables|Default|GetSecondaryGrabbableLeft)))
      (Variables|Default|SetSecondaryGripController MotionController)
      (Utilities|String|LogString "MyLog: Set Secondary Grip Controller")
      (if (Utilities|Enum|Equal(Enum) (Utilities|GetObjectName MotionController) "MotionControllerRight")
        (Development|SetHiddeninGame (Variables|Default|GetSecondaryHandRight) false false)
        (Development|SetHiddeninGame (Variables|Default|GetRightHand) true false)
        (else
          (Development|SetHiddeninGame (Variables|Default|GetSecondaryHandLeft) false false)
          (Development|SetHiddeninGame (Variables|Default|GetLeftHand) true false)))
      (if (not (Utilities|IsValid (Variables|Default|GetMainGripController)))
        (Transformation|AttachComponentToComponent (Variables|Default|GetGripPoint) (Variables|Default|GetSecondaryGripController) "None" "KeepWorld" "KeepWorld" "KeepWorld" true)
        (Variables|Default|SetisSecondaryControllerAttached true)
        (goto _label))
      (elif (and (or (and (Utilities|Enum|Equal(Enum) (Utilities|GetObjectName MotionController) "MotionControllerRight") (Variables|Default|GetBarrelGrabbableRight)) (and (Utilities|Enum|Equal(Enum) (Utilities|GetObjectName MotionController) "MotionControllerLeft") (Variables|Default|GetBarrelGrabbableLeft))) (or (Utilities|IsValid (Variables|Default|GetMainGripController)) (Utilities|IsValid (Variables|Default|GetSecondaryGripController))))
        (Variables|Default|SetBarrelGripController MotionController)
        (if (Utilities|Enum|Equal(Enum) (Utilities|GetObjectName MotionController) "MotionControllerRight")
          (Development|SetHiddeninGame (Variables|Default|GetBarrelGripHandRight) false false)
          (Development|SetHiddeninGame (Variables|Default|GetRightHand) true false)
          (goto _label)
          (else
            (Development|SetHiddeninGame (Variables|Default|GetBarrelGripHandLeft) false false)
            (Development|SetHiddeninGame (Variables|Default|GetLeftHand) true false)
            (goto _label)))))))

(event EventRelease
  (params (MotionController :type Motion%20Controller%20Component%20Object%20Reference))
  (bind _returnvalue (Utilities|GetObjectName MotionController))
  (bind _returnvalue_2 (Game|GetPlayerController 0))
  (bind _modell1900_stock (Variables|Default|Getmodell1900_stock))
  (bind _secondarygrippoint (Variables|Default|GetSecondaryGripPoint))
  (bind _returnvalue_3 (Utilities|Enum|Equal(Enum) _returnvalue "MotionControllerRight"))
  (bind _returnvalue_4 (Transformation|GetWorldRotation _modell1900_stock))
  (bind _returnvalue_5 (Transformation|GetWorldTransform _secondarygrippoint))
  (Utilities|FlowControl|Sequence
    (:then_0
      (if (== MotionController (Variables|Default|GetMainGripController))
        (Transformation|DetachFromComponent (Variables|Default|GetGripPoint) "KeepWorld" "KeepWorld" "KeepWorld" true)
        ;[1 1 1] Trigger removal
        (Input|DisableInput _returnvalue_2)
        (Input|RemoveMappingContext (PlayerController|LocalPlayerSubsystems|GetEnhancedInputLocalPlayerSubsystem _returnvalue_2) (select (== (Variables|/Script/HeadMountedDisplay.MotionControllerComponent|GetMotionSource (Variables|Default|GetMainGripController)) "Right") "/Game/VRTemplate/Input/IMC_Weapon_Right.IMC_Weapon_Right" "/Game/VRTemplate/Input/IMC_Weapon_Left.IMC_Weapon_Left") "(bIgnoreAllPressedKeysUntilRelease=True,bForceImmediately=False)")
        (Variables|Default|SetMainGripController 0)
        (Utilities|String|LogString "MyLog: Detached Main Grip Controller")
        (bind _secondarygripcontroller (Variables|Default|GetSecondaryGripController)
          (:then
            (Transformation|DetachFromComponent _modell1900_stock "KeepWorld" "KeepWorld" "KeepWorld" true)
            (Transformation|SetWorldTransform (Variables|Default|GetGripPoint) (Math|Transform|MakeTransform (.location _returnvalue_5) (Math|Rotator|MakeRotator (+ (.roll (.rotation _returnvalue_5)) (- (.roll (Transformation|GetWorldRotation _secondarygripcontroller)) (.roll _returnvalue_4))) (+ (.pitch (.rotation _returnvalue_5)) (- (.pitch (Transformation|GetWorldRotation _secondarygripcontroller)) (.pitch _returnvalue_4))) (+ (.yaw (.rotation _returnvalue_5)) (- (.yaw (Transformation|GetWorldRotation _secondarygripcontroller)) (.yaw _returnvalue_4)))) (.scale _returnvalue_5)) false false)
            (Transformation|AttachComponentToComponent (Variables|Default|Getmodell1900_stock) (Variables|Default|GetGripPoint) "None" "KeepWorld" "KeepWorld" "KeepWorld" true)
            (bind _returnvalue_6 (Transformation|AttachComponentToComponent (Variables|Default|GetGripPoint) _secondarygripcontroller "None" "SnapToTarget" "SnapToTarget" "KeepRelative" true))
            (Variables|Default|SetisSecondaryControllerAttached _returnvalue_6))
          (:else))))
    (:then_1
      (if (== MotionController (Variables|Default|GetSecondaryGripController))
        (if (Variables|Default|GetisSecondaryControllerAttached)
          (Transformation|DetachFromComponent (Variables|Default|GetGripPoint) "KeepWorld" "KeepWorld" "KeepWorld" true)
          (Variables|Default|SetisSecondaryControllerAttached false)
          (Transformation|DetachFromComponent (Variables|Default|Getmodell1900_stock) "KeepWorld" "KeepWorld" "KeepWorld" true)
          (Transformation|SetWorldTransform (Variables|Default|GetGripPoint) (Transformation|GetWorldTransform (Variables|Default|GetMainGripPoint)) false false)
          (Transformation|AttachComponentToComponent (Variables|Default|Getmodell1900_stock) (Variables|Default|GetGripPoint) "None" "KeepWorld" "KeepWorld" "KeepWorld" true)
          (if (Utilities|IsValid (Variables|Default|GetMainGripController))
            (Transformation|AttachComponentToComponent (Variables|Default|GetGripPoint) (Variables|Default|GetMainGripController) "None" "SnapToTarget" "SnapToTarget" "SnapToTarget" true)))
        (Variables|Default|SetSecondaryGripController 0)
        (Utilities|String|LogString "MyLog: Released Secondary Grip Controller")
        (if _returnvalue_3
          (Development|SetHiddeninGame (Variables|Default|GetSecondaryHandRight) true false)
          (Development|SetHiddeninGame (Variables|Default|GetRightHand) false false)
          (else
            (Development|SetHiddeninGame (Variables|Default|GetSecondaryHandLeft) true false)
            (Development|SetHiddeninGame (Variables|Default|GetLeftHand) false false)))
        (bind _maingripcontroller (Variables|Default|GetMainGripController)
          (:then
            (Transformation|SetWorldRotation (Variables|Default|GetGripPoint) (Transformation|GetWorldRotation _maingripcontroller) false false))
          (:else))
        (elif (== MotionController (Variables|Default|GetBarrelGripController))
          (Variables|Default|SetBarrelGripController 0)
          (if _returnvalue_3
            (Development|SetHiddeninGame (Variables|Default|GetBarrelGripHandRight) true false)
            (Development|SetHiddeninGame (Variables|Default|GetRightHand) false false)
            (else
              (Development|SetHiddeninGame (Variables|Default|GetBarrelGripHandLeft) true false)
              (Development|SetHiddeninGame (Variables|Default|GetLeftHand) false false))))))))

(event EventBeginPlay
  (bind _returnvalue (Game|Player|GetPlayerPawn 0))
  (Variables|Default|SetVRPawn _returnvalue)
  (bind _output_get (Variables|Default|SetLeftHand (Utilities|Array|Get(acopy) (Actor|GetComponentsbyTag _returnvalue "/Script/Engine.SkeletalMeshComponent" "HandLeft"))))
  (bind _output_get_2 (Variables|Default|SetRightHand (Utilities|Array|Get(acopy) (Actor|GetComponentsbyTag _returnvalue "/Script/Engine.SkeletalMeshComponent" "HandRight"))))
  (bind _assk_mannequins_xr_anim_blueprint (Utilities|Casting|CastToSK_MannequinsXR_AnimBlueprint (Components|SkeletalMesh|GetAnimInstance _output_get)))
  (Variables|Default|SetLeftHandAnim _assk_mannequins_xr_anim_blueprint)
  (bind _assk_mannequins_xr_anim_blueprint_2 (Utilities|Casting|CastToSK_MannequinsXR_AnimBlueprint (Components|SkeletalMesh|GetAnimInstance _output_get_2)))
  (Variables|Default|SetRightHandAnim _assk_mannequins_xr_anim_blueprint_2))

(fn ConstructionScript)

(fn EjectCartridgeCase
  (params (SpawnPoint :type Arrow%20Component%20Object%20Reference))
  (bind _ejecttionpointright (Variables|Default|GetejecttionPointRight))
  (bind _returnvalue (Transformation|GetWorldRotation _ejecttionpointright))
  ;[1 1 1] Eject bullet
  (bind _returnvalue_2 (Game|SpawnActorfromClass "/Game/Blueprints/Ammo/CartridgeCase_Modell1900.CartridgeCase_Modell1900_C" (Math|Transform|MakeTransform (Transformation|GetWorldLocation SpawnPoint) (Transformation|GetWorldRotation SpawnPoint)) "Undefined" 0 0))
  (Physics|SetSimulatePhysics (Variables|/Game/Blueprints/Ammo/CartridgeCase_Modell1900.CartridgeCase_Modell1900_C|Getmodell1900_cartridgeCase _returnvalue_2) true)
  (Physics|AddImpulse (Variables|/Game/Blueprints/Ammo/CartridgeCase_Modell1900.CartridgeCase_Modell1900_C|Getmodell1900_cartridgeCase _returnvalue_2) (* (Math|Vector|Normalize (Math|Vector|MakeVector (.roll _returnvalue) (.pitch _returnvalue) (.yaw _returnvalue))) "10.000000,10.000000,10.000000") "None" false))

(fn Reload
  (params (isLeft :type Boolean) (otherActor :type Actor%20Object%20Reference))
  (bind _isbarrelopen (Variables|Default|GetisBarrelOpen))
  ;[1 1 1] Reloading
  (if (== (Utilities|GetClass otherActor) "/Game/Blueprints/Ammo/Bullet_Modell1900.Bullet_Modell1900_C")
    (if isLeft
      (if (and (not (Variables|Default|GetisLeftBulletLoaded)) _isbarrelopen)
        (Actor|DestroyActor otherActor)
        (Development|SetHiddeninGame (Variables|Default|Getbullet_left) false false)
        (Variables|Default|SetisLeftBulletLoaded true))
      (elif (and _isbarrelopen (not (Variables|Default|GetisRightBulletLoaded)))
        (Actor|DestroyActor otherActor)
        (Development|SetHiddeninGame (Variables|Default|Getbullet_right) false false)
        (Variables|Default|SetisRightBulletLoaded true)))))

(fn RandomBulletSpread
  (params (spawnPoint :type Arrow%20Component%20Object%20Reference) (maxSpread :type Float%20%28double-precision%29))
  (bind _returnvalue (Transformation|GetWorldRotation spawnPoint))
  ;[1 1 1] Random bullet spread
  (if (Utilities|IsValid (Variables|Default|GetSecondaryGripController))
    (LocalVariables|Setspread (/ maxSpread (LocalVariables|GetspreadDivider)))
    (else
      (LocalVariables|Setspread maxSpread)))
  (return (Math|Transform|MakeTransform (Transformation|GetWorldLocation spawnPoint) (Math|Rotator|MakeRotator (+ (.roll _returnvalue) (Math|Random|RandomFloatinRange (* (LocalVariables|Getspread) -1.0) (LocalVariables|Getspread))) (+ (.pitch _returnvalue) (Math|Random|RandomFloatinRange (* (LocalVariables|Getspread) -1.0) (LocalVariables|Getspread))) (+ (.yaw _returnvalue) (Math|Random|RandomFloatinRange (* (LocalVariables|Getspread) -1.0) (LocalVariables|Getspread)))) (Transformation|GetWorldScale spawnPoint))))