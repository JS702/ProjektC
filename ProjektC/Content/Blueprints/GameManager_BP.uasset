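; GameManager_BP runs a VR wave-based shooter, managing enemy waves, coins and item purchases.
; Each wave grows the enemy count, hides the shop UI and spawns enemies at random spawn points through a delayed self-calling event, with weighted, capped snipers.
; Kills award coins; the last ends the wave, restoring menu interaction and removing any purchased weapon.
; BuyItem checks coins and forwards weapon or item requests to ItemSpawner.
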(event Custom|SpawnEnemy
  (if (not (== (Variables|Default|Getcounter) (Variables|Default|GetEnemyCount)))
    (bind _outactors (Actor|GetAllActorsOfClass "/Game/Blueprints/SpawnPosition_BP.SpawnPosition_BP_C"))
    (if (< (Variables|Default|GetsniperCount) 2)
      (if (Math|Random|RandomBoolwithWeight 0.8)
        (Game|SpawnActorfromClass "/Game/Blueprints/Enemys/Enemy_Standard.Enemy_Standard_C" (Transformation|GetActorTransform (Utilities|Array|Get(acopy) _outactors (Math|Random|RandomInteger (Utilities|Array|Length _outactors)))) "AdjustIfPossibleButAlwaysSpawn" 0 0 :!label _label)
        (else
          (Game|SpawnActorfromClass "/Game/Blueprints/Enemys/Enemy_Sniper.Enemy_Sniper_C" (Transformation|GetActorTransform (Utilities|Array|Get(acopy) _outactors (Math|Random|RandomInteger (Utilities|Array|Length _outactors)))) "AdjustIfPossibleButAlwaysSpawn" 0 0)
          (Math|Integer|IncrementInt (Variables|Default|GetsniperCount)
            (:%20%20
              _))))
      (else
        (goto _label)))
    (Math|Integer|IncrementInt (Variables|Default|Getcounter)
      (:%20%20
        (Utilities|FlowControl|Delay 8.0)
        (CallFunction|SpawnEnemy)))))

(event Custom|SniperKillled
  (Math|Integer|DecrementInt (Variables|Default|GetsniperCount)
    (:%20%20
      (CallFunction|EnemyKilled))))

(event Custom|EndWave
  (bind _player (Variables|Default|Getplayer))
  (bind _purchasedweapon (Variables|/Game/VRTemplate/Blueprints/VRPawn.VRPawn_C|GetpurchasedWeapon _player))
  (Default|StartMenuInteraction (Variables|Default|Getplayer))
  (Variables|Default|SetWaveOver true)
  (bind _returnvalue (Actor|GetActorOfClass "/Game/Blueprints/UI/SpawnUIElement.SpawnUIElement_C"))
  (Default|ShowUi _returnvalue)
  (Utilities|IsValid _purchasedweapon
    (:Is%20Valid
      (Actor|DestroyActor _purchasedweapon)
      (Development|SetHiddeninGame (Variables|Default|GetLeftHand) false false)
      (Development|SetHiddeninGame (Variables|Default|GetRightHand) false false))))

(event Custom|StartWave
  (Variables|Default|SetEnemyCount (+ (Variables|Default|GetEnemyCount) 2))
  (Default|StopMenuInteraction (Variables|Default|Getplayer))
  (Variables|Default|SetWaveOver false)
  (Default|HideUi (Variables|Default|GetuiSpawner))
  (Variables|Default|Setcounter 0)
  (Variables|Default|SetdeathCount 0)
  (Audio|PlaySound2D "/Game/Sounds/Ambience/whistle.whistle" 1.0 1.0 0.0 0 0)
  (Utilities|FlowControl|Delay 5.0)
  (CallFunction|SpawnEnemy))

(event Custom|EnemyKilled
  (Variables|Default|Setcoins (+ (Variables|Default|Getcoins) 10))
  (bind _result (Math|Integer|IncrementInt (Variables|Default|GetdeathCount))
    (:%20%20
      (if (== _result (Variables|Default|GetEnemyCount))
        (CallFunction|EndWave)))))

(event EventBeginPlay
  (bind _returnvalue (Game|Player|GetPlayerPawn 0))
  (bind _returnvalue_2 (Actor|GetActorOfClass "/Game/VRTemplate/Blueprints/VRPawn.VRPawn_C"))
  (Variables|Default|Setplayer _returnvalue_2)
  (Audio|PlaySound2D "/Game/Sounds/Ambience/Background/Background.Background" 1.0 1.0 0.0 0 0)
  (bind _returnvalue_3 (Actor|GetActorOfClass "/Game/Blueprints/UI/SpawnUIElement.SpawnUIElement_C"))
  (Variables|Default|SetuiSpawner _returnvalue_3)
  (Variables|Default|SetLeftHand (Utilities|Array|Get(acopy) (Actor|GetComponentsbyTag _returnvalue "/Script/Engine.SkeletalMeshComponent" "HandLeft")))
  (Variables|Default|SetRightHand (Utilities|Array|Get(acopy) (Actor|GetComponentsbyTag _returnvalue "/Script/Engine.SkeletalMeshComponent" "HandRight")))
  (Utilities|FlowControl|Delay 7.0)
  (CallFunction|StartWave))

(fn ConstructionScript)

(fn BuyItem
  (params (Price :type Integer) (Class :type Actor%20Class%20Reference) (Selection :type String))
  (if (> (Variables|Default|Getcoins) Price)
    (Variables|Default|Setcoins (- (Variables|Default|Getcoins) Price))
    (bind _returnvalue (Actor|GetActorOfClass "/Game/Blueprints/ItemSpawner.ItemSpawner_C"))
    (if (Utilities|Enum|Equal(Enum) Selection "Weapon")
      (Default|SpawnWeapon _returnvalue Class)
      (else
        (Default|SpawnItem _returnvalue Class)))
    (else
      (Audio|PlaySound2D "/Engine/EditorSounds/Notifications/CompileFailed.CompileFailed" 1.0 1.0 0.0 0 0))))